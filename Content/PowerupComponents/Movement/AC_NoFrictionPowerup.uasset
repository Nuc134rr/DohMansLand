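; No-friction movement powerup component that makes every tank slide when it is applied.
; On BeginPlay it zeroes walking braking deceleration and ground friction on all BP_BaseTank actors.
; Inside that loop it checks the owner's projectile powerup components for AC_JuggernautPowerup to set a combo flag.
; With the combo, it gives some grip back to the first actor found of player one's pawn class.
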(event EventBeginPlay
  ;[0.2 0.2 0.2] Sets the braking deceleration and ground friction to 0
  (|CallParentFunction)
  (bind _outactors (Actor|GetAllActorsOfClass "/Game/Blueprints/Player/BP_BaseTank.BP_BaseTank_C"))
  (for _array_element _outactors
    (Variables|/Script/Engine.CharacterMovementComponent|SetBrakingDecelerationWalking (Variables|/Script/Engine.Character|GetCharacterMovement _array_element) 0.0)
    (Variables|/Script/Engine.CharacterMovementComponent|SetGroundFriction (Variables|/Script/Engine.Character|GetCharacterMovement _array_element) 0.0)
    ;[0.2 0.2 0.2] Combo check
    (bind _array_element_2 (Utilities|Array|ForEachLoopwithBreak (Actor|GetComponentsByClass (Components|GetOwner) "/Game/PowerupComponents/AC_BaseProjectilePowerup.AC_BaseProjectilePowerup_C") :!label _label)
      (:LoopBody
        (Utilities|Casting|CastToAC_JuggernautPowerup _array_element_2)
        (Variables|Default|SetbShouldCombo true)
        (goto _label Break))
      (:Completed
        ;[0.2 0.2 0.2] Combo
        (if (Variables|Default|GetbShouldCombo)
          (bind _returnvalue (Actor|GetActorOfClass (Utilities|GetClass (CallFunction|GetPlayerOnePawn))))
          (for _array_element_3 (Utilities|Array|MakeArray _returnvalue)
            (Variables|/Script/Engine.CharacterMovementComponent|SetBrakingDecelerationWalking (Variables|/Script/Engine.Character|GetCharacterMovement _array_element_3) 5.0)
            (Variables|/Script/Engine.CharacterMovementComponent|SetGroundFriction (Variables|/Script/Engine.Character|GetCharacterMovement _array_element_3) 5.0)))))))