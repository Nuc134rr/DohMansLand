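; Juggernaut powerup component that gives the owning tank's controller three lives and shows the remaining lives on the tank's material.
; BeginPlay sets the lives and plays a pickup sound at the controller's spawn point.
; Tick, throttled by a one-second Delay, recreates dynamic material instances on the base and turret, setting the JugBump scalar from lives over three and reapplying the tank colour.
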(event EventBeginPlay
  (bind _ownerref (Variables|Default|GetOwnerRef))
  (bind _controllerreference (Variables|/Game/Blueprints/Player/BP_NewBaseTank.BP_NewBaseTank_C|GetControllerReference _ownerref))
  (|CallParentFunction)
  (Variables|/Game/Blueprints/Player/BP_Player.BP_Player_C|SetLives _controllerreference 3)
  (Audio|PlaySoundatLocation "/Game/Assets/SFX/misc_outside_noises/Powerup_sounds/jug_pickup_Cue.jug_pickup_Cue" (Transformation|GetWorldLocation (Variables|/Game/Blueprints/Player/BP_Player.BP_Player_C|GetSpawnPoint _controllerreference)) "0, 0, 0" 1.0 1.0 0.0 0 0 0 0))

(event EventTick
  (params (DeltaSeconds :type Float%20%28single-precision%29))
  (bind _ownerref (Variables|Default|GetOwnerRef))
  (bind _ownerref_2 (Variables|Default|GetOwnerRef))
  (bind _controllerreference (Variables|/Game/Blueprints/Player/BP_NewBaseTank.BP_NewBaseTank_C|GetControllerReference _ownerref_2))
  (bind _tankvariables (Variables|/Game/Blueprints/Player/BP_NewBaseTank.BP_NewBaseTank_C|GetTankVariables _ownerref_2))
  (bind _lives (Variables|/Game/Blueprints/Player/BP_Player.BP_Player_C|GetLives _controllerreference))
  (bind _returnvalue (Math|Conversions|ToFloat(Integer) _lives))
  (bind _returnvalue_2 (/ _returnvalue 3.0))
  (|CallParentFunction DeltaSeconds)
  (Utilities|FlowControl|Delay 1.0)
  (Utilities|FlowControl|Sequence
    (:then_0
      (for _index (range 0 4)
        (bind _returnvalue_3 (Rendering|Material|CreateDynamicMaterialInstance (Variables|/Game/Blueprints/Player/BP_NewBaseTank.BP_NewBaseTank_C|GetTankBase _ownerref) _index "/Game/Assets/Materials/Doh/M_Doh.M_Doh" "None" :!class /Script/Engine.PrimitiveComponent))
        (Rendering|Material|SetScalarParameterValue _returnvalue_3 "JugBump" _returnvalue_2 :!class /Script/Engine.MaterialInstanceDynamic)
        (Rendering|Material|SetVectorParameterValue _returnvalue_3 "Color0" (.tankcolor _tankvariables) :!class /Script/Engine.MaterialInstanceDynamic))
      (bind _returnvalue_4 (Rendering|Material|CreateDynamicMaterialInstance (Variables|/Game/Blueprints/Player/BP_NewBaseTank.BP_NewBaseTank_C|GetTurret _ownerref) 0 "/Game/Assets/Materials/Doh/M_Doh.M_Doh" "None" :!class /Script/Engine.PrimitiveComponent))
      (Rendering|Material|SetScalarParameterValue _returnvalue_4 "JugBump" _returnvalue_2 :!class /Script/Engine.MaterialInstanceDynamic)
      (Rendering|Material|SetVectorParameterValue _returnvalue_4 "Color0" (.tankcolor _tankvariables) :!class /Script/Engine.MaterialInstanceDynamic))))