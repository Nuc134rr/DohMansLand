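; Movement powerup component that doubles the owning tank's movement and turn speed.
; On BeginPlay it plays an engine rev sound at the controller's spawn point, waits half a second, then doubles the floating pawn movement's max speed and the owner's turn speed.
; Disconnected leftover nodes hold unused logic for juggernaut scaling, removing the no-friction powerup and doubling MoveSpeed.
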(event EventBeginPlay
  (bind _ownerref (Variables|Default|GetOwnerRef))
  (bind _floatingpawnmovement (Variables|/Game/Blueprints/Player/BP_BaseTank.BP_BaseTank_C|GetFloatingPawnMovement _ownerref))
  (|CallParentFunction)
  (Audio|PlaySoundatLocation "/Game/Assets/SFX/misc_outside_noises/Powerup_sounds/speed_rev/engine_rev_Cue.engine_rev_Cue" (Transformation|GetWorldLocation (Variables|/Game/Blueprints/Player/BP_Player.BP_Player_C|GetSpawnPoint (Variables|/Game/Blueprints/Player/BP_BaseTank.BP_BaseTank_C|GetControllerReference (Variables|Default|GetOwnerRef)))) "0, 0, 0" 1.0 1.0 0.0 0 0 0 0)
  (Utilities|FlowControl|Delay 0.5)
  (Variables|/Script/Engine.FloatingPawnMovement|SetMaxSpeed _floatingpawnmovement (* (Class|MovementComponent|GetMaxSpeed _floatingpawnmovement) 2.0))
  (Variables|/Game/Blueprints/Player/BP_BaseTank.BP_BaseTank_C|SetTurnSpeed _ownerref (* (Variables|/Game/Blueprints/Player/BP_BaseTank.BP_BaseTank_C|GetTurnSpeed _ownerref) 2.0)))