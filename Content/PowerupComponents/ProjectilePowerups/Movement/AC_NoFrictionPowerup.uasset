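; AC_NoFrictionPowerup is a powerup component that temporarily removes walking braking friction from every tank in the level.
; On BeginPlay it caches the owner's braking deceleration, then zeroes that value on every BP_BaseTank actor.
; After the Lifespan delay it queries the tanks again, applies the owner's cached value to all of them, and destroys itself.
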(event EventBeginPlay
  ;[0.2 0.2 0.2] Sets the braking deceleration to 0 (no friction) for the duration of the variable "Lifespan"
  (|CallParentFunction)
  (Variables|Default|SetDefaultBrakingDeceleration (Variables|/Script/Engine.CharacterMovementComponent|GetBrakingDecelerationWalking (Variables|/Script/Engine.Character|GetCharacterMovement (Variables|Default|GetOwnerRef))))
  (bind _outactors (Actor|GetAllActorsOfClass "/Game/Blueprints/Player/BP_BaseTank.BP_BaseTank_C"))
  (for _array_element _outactors
    (Variables|/Script/Engine.CharacterMovementComponent|SetBrakingDecelerationWalking (Variables|/Script/Engine.Character|GetCharacterMovement _array_element) 0.0))
  (Utilities|FlowControl|Delay (Variables|Default|GetLifespan))
  (bind _outactors_2 (Actor|GetAllActorsOfClass "/Game/Blueprints/Player/BP_BaseTank.BP_BaseTank_C"))
  (for _array_element_2 _outactors_2
    (Variables|/Script/Engine.CharacterMovementComponent|SetBrakingDecelerationWalking (Variables|/Script/Engine.Character|GetCharacterMovement _array_element_2) (Variables|Default|GetDefaultBrakingDeceleration)))
  (Components|DestroyComponent))