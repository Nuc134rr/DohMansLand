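; Weapon powerup component that lets its owner have more projectiles by raising the max projectile count on BeginPlay.
; Every tick it loops over the owner's active projectiles and turns off bouncing.
; An unconnected combo branch looks for a fast-projectiles powerup to grant a far higher cap and switch to fire projectiles as a "Gattling" combo, but it never runs.
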(event EventBeginPlay
  ;[1 1 1] More Bullet code
  (|CallParentFunction)
  (Utilities|FlowControl|Sequence
    (:then_0
      (Variables|/Game/Blueprints/Player/BP_NewBaseTank.BP_NewBaseTank_C|SetMaxProjectiles (Variables|Default|GetOwnerRef) 10))))

(event EventTick
  (params (DeltaSeconds :type Float%20%28single-precision%29))
  (|CallParentFunction DeltaSeconds)
  (for _array_element (Variables|/Game/Blueprints/Player/BP_NewBaseTank.BP_NewBaseTank_C|GetActiveProjectiles (Variables|Default|GetOwnerRef))
    (Variables|/Game/Projectiles/BP_BaseProjectile.BP_BaseProjectile_C|SetbCanBounce _array_element false)))