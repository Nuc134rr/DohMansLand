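; Greybox tank pawn for Player 1 that moves along fixed world axes and gets a random color.
; The Up and Right input axes feed AddMovementInput on world Y and X, independent of the tank's facing.
; The Construction Script creates a dynamic M_Doh material on the Cube and randomly sets its BaseColor from eight hard-coded cases, with one blue repeated.
; The color re-rolls whenever construction reruns.
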(event Input|AxisEvents|InputAxisRightPlayer1
  (params (AxisValue :type Float%20%28single-precision%29))
  (Pawn|Input|AddMovementInput self "1.000000,0.000000,0.000000" AxisValue false))

(event Input|AxisEvents|InputAxisUpPlayer1
  (params (AxisValue :type Float%20%28single-precision%29))
  (Pawn|Input|AddMovementInput self "0.000000,1.000000, 0" AxisValue false))

(fn ConstructionScript
  ;[1 1 1] Random BaseColor Assignment
  (bind _returnvalue (Rendering|Material|CreateDynamicMaterialInstance (Variables|Default|GetCube) 0 "/Game/Assets/Materials/M_Doh.M_Doh" "None" :!class /Script/Engine.PrimitiveComponent))
  (switch int (Math|Random|RandomInteger 8)
    (:0
      (Rendering|Material|SetVectorParameterValue _returnvalue "BaseColor" "(R=0.973445,G=0.042311,B=0.038204,A=1.000000)" :!class /Script/Engine.MaterialInstanceDynamic))
    (:1
      (Rendering|Material|SetVectorParameterValue _returnvalue "BaseColor" "(R=0.830770,G=0.291771,B=0.000000,A=1.000000)" :!class /Script/Engine.MaterialInstanceDynamic))
    (:2
      (Rendering|Material|SetVectorParameterValue _returnvalue "BaseColor" "(R=0.701102,G=0.658375,B=0.019382,A=1.000000)" :!class /Script/Engine.MaterialInstanceDynamic))
    (:3
      (Rendering|Material|SetVectorParameterValue _returnvalue "BaseColor" "(R=0.318547,G=0.665387,B=0.309469,A=1.000000)" :!class /Script/Engine.MaterialInstanceDynamic))
    (:4
      (Rendering|Material|SetVectorParameterValue _returnvalue "BaseColor" "(R=0.000911,G=0.035601,B=0.514918,A=1.000000)" :!class /Script/Engine.MaterialInstanceDynamic))
    (:5
      (Rendering|Material|SetVectorParameterValue _returnvalue "BaseColor" "(R=0.346704,G=0.029557,B=0.341914,A=1.000000)" :!class /Script/Engine.MaterialInstanceDynamic))
    (:6
      (Rendering|Material|SetVectorParameterValue _returnvalue "BaseColor" "(R=0.000911,G=0.035601,B=0.514918,A=1.000000)" :!class /Script/Engine.MaterialInstanceDynamic))
    (:7
      (Rendering|Material|SetVectorParameterValue _returnvalue "BaseColor" "(R=0.693872,G=0.693872,B=0.768151,A=1.000000)" :!class /Script/Engine.MaterialInstanceDynamic))))