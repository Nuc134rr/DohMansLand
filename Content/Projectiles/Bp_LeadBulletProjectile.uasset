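; Lead bullet projectile Blueprint fired by a tank, extending a parent projectile class.
; Each tick it runs the parent tick, then checks whether its owning BP_BaseTank is unstoppable.
; If so, it removes and destroys itself once its remaining wall-destruction count reaches zero or below.
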(event EventTick
  (params (DeltaSeconds :type Float%20%28single-precision%29))
  (|CallParentFunction DeltaSeconds)
  (if (Variables|/Game/Blueprints/Player/BP_BaseTank.BP_BaseTank_C|GetbIsUnstoppable (.AsBP%20Base%20Tank (Utilities|Casting|CastToBP_BaseTank (Components|GetOwner))))
    (if (<= (Variables|Default|GetMax%20number%20of%20walls%20destoyed%20) 0)
      (CallFunction|RemoveandDestroy))))

(fn ConstructionScript
  (|CallParentFunction))