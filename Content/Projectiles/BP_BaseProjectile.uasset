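; Base tank-fired projectile that ricochets off surfaces, damages tanks and destroys other projectiles, with special rules for BP_BigProjectile.
; Tick moves it manually and sphere-traces for hits; bouncing shots mirror their heading on a forward trace's normal until their bounce limit, others die on walls.
; It initially ignores its firing tank, resetting that list after bouncing.
; Removal updates the owning tank's projectile array; tank kills trigger the GameMode's end check.
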(event EventBeginPlay
  ;[0.2 0.2 0.2] Sets the initial speed of the projectile
  (bind _asbp_base_tank (Utilities|Casting|CastToBP_BaseTank (Variables|Default|GetTankRef)))
  (CallFunction|SetVelocity)
  (Variables|Default|SetActorsToIgnore (Utilities|Array|MakeArray _asbp_base_tank 0)))

(event EventTick
  (params (DeltaSeconds :type Float%20%28single-precision%29))
  (bind _returnvalue (Transformation|GetActorForwardVector))
  (bind _returnvalue_2 (Transformation|GetActorLocation))
  (bind _returnvalue_3 (Transformation|GetActorLocation))
  (bind _actorstoignore (Variables|Default|GetActorsToIgnore))
  (bind _draw_debug_type (Variables|Debugging|GetDraw%20Debug%20Type))
  (bind _draw_time (Variables|Debugging|GetDraw%20Time))
  (bind (_start _end) (CallFunction|GetStartandEndforLineTrace _returnvalue_3 _returnvalue 1e+20))
  ;[0.2 0.2 0.2] Movement for projectile
  (Transformation|SetActorLocation (+ (* DeltaSeconds (Variables|Default|GetVelocity)) (Transformation|GetActorLocation)) true false)
  (Transformation|AddLocalRotation (Variables|Default|GetStaticMesh) "0, 0,1.000000" false false)
  ;[0.2 0.2 0.2] trace forward vector
  (bind _outhit (Collision|LineTraceByChannel _start _end "TraceTypeQuery1" false (Variables|Default|GetActorsToIgnore) (Variables|Debugging|GetDraw%20Debug%20Type) true "(R=1.000000,G=0.000000,B=0.000000,A=1.000000)" "(R=0.000000,G=1.000000,B=0.000000,A=1.000000)" (Variables|Debugging|GetDraw%20Time)))
  ;[0.2 0.2 0.2] trace normal of hit and mirrored projectile motion
  (bind (_outhit_2 _returnvalue_4) (Collision|SphereTraceByChannel _returnvalue_2 _returnvalue_2 (+ (.SphereRadius (Collision|GetComponentBounds (Variables|Default|GetStaticMesh))) 0.1) "TraceTypeQuery1" false (Variables|Default|GetActorsToIgnore) "None"))
  (if _returnvalue_4
    (Collision|CheckforHitProjectile _outhit_2)
    (Collision|CheckforHitTank _outhit_2)
    (if (Variables|Default|GetbCanBounce)
      (Utilities|FlowControl|Sequence
        (:then_0
          (Collision|LineTraceByChannel (.Start (CallFunction|GetStartandEndforLineTrace (.location _outhit) (.normal _outhit) 1e+20)) (.End (CallFunction|GetStartandEndforLineTrace (.location _outhit) (.normal _outhit) 1e+20)) "TraceTypeQuery1" false _actorstoignore _draw_debug_type true "(R=1.000000,G=0.000000,B=0.000000,A=1.000000)" "(R=0.000000,G=1.000000,B=0.000000,A=1.000000)" _draw_time) ; noramal of the hit object
        )
        (:then_1
          (bind _outhit_3 (Collision|LineTraceByChannel (.Start (CallFunction|GetStartandEndforLineTrace (Transformation|GetActorLocation) (Math|Vector|MirrorVectorbyNormal (Transformation|GetActorForwardVector) (.normal _outhit)) 1e+20)) (.End (CallFunction|GetStartandEndforLineTrace (Transformation|GetActorLocation) (Math|Vector|MirrorVectorbyNormal (Transformation|GetActorForwardVector) (.normal _outhit)) 1e+20)) "TraceTypeQuery1" false _actorstoignore _draw_debug_type true "(R=1.000000,G=0.000000,B=0.000000,A=1.000000)" "(R=0.000000,G=1.000000,B=0.000000,A=1.000000)" _draw_time)) ; mirrored vector on normal
          (Collision|Bounce (.location _outhit_3)))
        (:then_2
          (CallFunction|Die)))
      (else
        (Collision|CheckforWall _outhit_2)))))

(fn ConstructionScript
  (CallFunction|SetRandomColors (Variables|Default|GetStaticMesh)))

(fn GetStartandEndforLineTrace
  (params (V1 :type Vector) (V2 :type Vector) (Scaling :type Float%20%28double-precision%29))
  (return V1 (+ V1 (* V2 Scaling))))

(fn SetVelocity
  (Variables|Default|SetVelocity (Math|Conversions|ToVector2D(Vector) (* (Variables|Default|GetSpeed) (Transformation|GetActorForwardVector)))))

(fn SetHitObjectName
  (params (OutHit :type Hit%20Result%20Structure))
  ;[0.2 0.2 0.2] debugging function
  (Development|PrintString (Utilities|String|Append "Hit Object Name: " (Utilities|GetObjectName (.HitActor (Collision|BreakHitResult OutHit)))) true true "(R=0.000000,G=0.660000,B=1.000000,A=1.000000)" 1e+01))

(fn Bounce
  (params (OutHitLocation :type Vector%20%28by%20ref%29))
  ;[0.2 0.2 0.2] find new point from line trace, look towards, and rotate
  (Transformation|SetActorRotation (Math|Rotator|MakeRotator 0.0 0.0 (.yaw (Math|Rotator|FindLookatRotation (Transformation|GetActorLocation) OutHitLocation))))
  (CallFunction|SetVelocity)
  (Audio|PlaySound2D "/Game/Assets/SFX/Bullet/Bullet_Bouncig_1_Cue.Bullet_Bouncig_1_Cue" 1.0 1.0 0.0 0 0)
  (bind _result (Math|Integer|IncrementInt (Variables|Default|GetBounces))
    (:%20%20
      (if (== _result 1)
        (Variables|Default|SetActorsToIgnore (Utilities|Array|MakeArray 0))))))

(fn CheckforHitProjectile
  (params (OutHit :type Hit%20Result%20Structure))
  (bind _hitactor (Collision|BreakHitResult OutHit))
  ;[0.2 0.2 0.2] if projectile hits projectile, kill them both. If the projectile is big, destroy only the smaller projectile
  (bind _asbp_base_projectile (Utilities|Casting|CastToBP_BaseProjectile _hitactor))
  (Utilities|Casting|CastToBP_BigProjectileClass (Utilities|GetClass _hitactor)
    (:then
      (CallFunction|RemoveandDestroy _asbp_base_projectile))
    (:CastFailed
      (bind _asbp_base_tank (Utilities|Casting|CastToBP_BaseTank (Variables|BP_BaseProjectile_C|GetTankRef _asbp_base_projectile)))
      (Default|RemoveProjectile _asbp_base_tank _asbp_base_projectile)
      (Actor|DestroyActor _asbp_base_projectile)
      (CallFunction|RemoveandDestroy))))

(fn Die
  ;[0.2 0.2 0.2] bounce x times and then die
  (if (> (Variables|Default|GetBounces) (Variables|Default|GetBouncesBeforeDeath))
    (CallFunction|RemoveandDestroy)))

(fn CheckforWall
  (params (OutHit :type Hit%20Result%20Structure))
  (bind _hitactor (Collision|BreakHitResult OutHit))
  ;[0.2 0.2 0.2] if the projectile cannot bounce, only destroy when it hits a wall
  (Utilities|IsValid _hitactor
    (:Is%20Valid
      (Utilities|Casting|CastToBP_BaseProjectileClass (Utilities|GetClass _hitactor)
        (:CastFailed
          (CallFunction|RemoveandDestroy))))))

(fn CheckforHitTank
  (params (OutHit :type Hit%20Result%20Structure))
  (bind _hitactor (Collision|BreakHitResult OutHit))
  (bind _asbp_base_tank (Utilities|Casting|CastToBP_BaseTank _hitactor))
  (Utilities|Casting|CastToBP_BigProjectile self
    (:then
      (Variables|/Game/Blueprints/Player/BP_BaseTank.BP_BaseTank_C|SetPlayerLives _asbp_base_tank (- (Variables|/Game/Blueprints/Player/BP_BaseTank.BP_BaseTank_C|GetPlayerLives _asbp_base_tank) 3)))
    (:CastFailed
      (Variables|/Game/Blueprints/Player/BP_BaseTank.BP_BaseTank_C|SetPlayerLives _asbp_base_tank (- (Variables|/Game/Blueprints/Player/BP_BaseTank.BP_BaseTank_C|GetPlayerLives _asbp_base_tank) 1))))
  (if (<= (Variables|/Game/Blueprints/Player/BP_BaseTank.BP_BaseTank_C|GetPlayerLives _asbp_base_tank) 0)
    (Actor|DestroyActor _hitactor)
    (Audio|PlaySound2D "/Game/Assets/SFX/Dead/Tank_Expolding_4_Cue.Tank_Expolding_4_Cue" 1.0 1.0 0.0 0 0)
    (Camera|PlayWorldCameraShake "/Game/Blueprints/Player/Bp_CameraShake.Bp_CameraShake_C" (Camera|GetCameraLocation (Game|GetPlayerCameraManager 0)) 0.0 5e+08)
    (CallFunction|RemoveandDestroy)
    (Default|CheckforEnd (.AsBP%20Doh%20Mans%20Land%20Game%20Mode (Utilities|Casting|CastToBP_DohMansLand_GameMode (Game|GetGameMode))))
    (else
      (CallFunction|RemoveandDestroy))))

(fn RemoveandDestroy
  ;[0.2 0.2 0.2] Remove Projectile from array in BP_BaseTank and then die
  (bind _asbp_base_tank (Utilities|Casting|CastToBP_BaseTank (Variables|Default|GetTankRef)))
  (Default|RemoveProjectile _asbp_base_tank self)
  (Actor|DestroyActor))