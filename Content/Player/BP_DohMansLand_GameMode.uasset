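; Game mode for two-player DohMansLand that scores player deaths, then clears projectiles and reloads the level until the winning score.
; GlobalScan, behind a retriggerable delay, line-traces a grid over every Chunk to record clay blocks and empty spots.
; It adds half-scale BlockSpawns between blocks adjacent in +X or +Y, with materials interpolated from neighbouring colours.
; The AI tank spawn on empty spots is disconnected.
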(event Custom|PlayerOneDeath
  (bind _result (Math|Integer|IncrementInt (Variables|/Game/Player/BP_DohMansLand_GameInstance.BP_DohMansLand_GameInstance_C|GetPlayerTwoScore (CallFunction|GetDohMansLandGameInstance)))
    (:%20%20
      (if (not (== _result (Variables|Score|GetScoreToWin)))
        (CallFunction|RemoveAllProjectiles)
        (Utilities|FlowControl|Delay 1.0)
        (CallFunction|OpenNewLevel "L_GBGenTest_Joysticks")))))

(event Custom|PlayerTwoDeath
  (bind _result (Math|Integer|IncrementInt (Variables|/Game/Player/BP_DohMansLand_GameInstance.BP_DohMansLand_GameInstance_C|GetPlayerOneScore (CallFunction|GetDohMansLandGameInstance)))
    (:%20%20
      (if (not (== _result (Variables|Score|GetScoreToWin)))
        (CallFunction|RemoveAllProjectiles)
        (Utilities|FlowControl|Delay 1.0)
        (CallFunction|OpenNewLevel "L_GBGenTest_Joysticks")))))

(event Custom|GlobalScan
  (bind _locatedblocks (Variables|Default|GetLocatedBlocks))
  (bind _locatedblockpositions (Variables|Default|GetLocatedBlockPositions))
  (Utilities|FlowControl|RetriggerableDelay 0.1)
  (bind _outactors (Actor|GetAllActorsOfClass "/Game/Blueprints/Generation/Chunk.Chunk_C"))
  (for _array_element _outactors
    (for _index (range 0 24)
      (Variables|Default|SetX (+ 5e+02 (Variables|Default|GetX)))
      (if (== (Variables|Default|GetX) 2.5e+03)
        (Variables|Default|SetY (+ (Variables|Default|GetY) 5e+02))
        (Variables|Default|SetX 0.0))
      (bind _outhit (Collision|LineTraceForObjects (Math|Vector|MakeVector (+ (.x (- (Transformation|GetActorLocation _array_element) (Math|Vector|MakeVector 1e+03 1e+03 0.0))) (Variables|Default|GetX)) (+ (.y (- (Transformation|GetActorLocation _array_element) (Math|Vector|MakeVector 1e+03 1e+03 0.0))) (Variables|Default|GetY)) (+ (.z (- (Transformation|GetActorLocation _array_element) (Math|Vector|MakeVector 1e+03 1e+03 0.0))) 1e+03)) (Math|Vector|MakeVector (+ (.x (- (Transformation|GetActorLocation _array_element) (Math|Vector|MakeVector 1e+03 1e+03 0.0))) (Variables|Default|GetX)) (+ (.y (- (Transformation|GetActorLocation _array_element) (Math|Vector|MakeVector 1e+03 1e+03 0.0))) (Variables|Default|GetY)) (- (.z (- (Transformation|GetActorLocation _array_element) (Math|Vector|MakeVector 1e+03 1e+03 0.0))) 1e+03)) (Variables|Default|GetObject%20Types) false 0 "None"))
      (bind _asblock_spawn (Utilities|Casting|CastToBlockSpawn (.HitActor (Collision|BreakHitResult _outhit))))
      (if (== (Variables|/Script/Engine.StaticMeshComponent|GetStaticMesh (Variables|/Game/Blueprints/Generation/BlockSpawn.BlockSpawn_C|GetCube _asblock_spawn)) "/Game/Assets/Meshes/clayCube_lo.clayCube_lo")
        (Utilities|Array|Add (Variables|Default|GetLocatedBlockPositions) (Transformation|GetActorLocation (.HitActor (Collision|BreakHitResult _outhit))))
        (Utilities|Array|Add _locatedblocks _asblock_spawn)
        (else
          (Utilities|Array|Add (Variables|Default|GetLocatedEmpty) (.Location (Collision|BreakHitResult _outhit))))))
    (Variables|Default|SetX -5e+02)
    (Variables|Default|SetY 0.0))
  (Utilities|FlowControl|Sequence
    (:then_0
      (for _array_element_2 _locatedblocks
        (for _index_2 (range 0 1)
          (if (Utilities|Array|ContainsItem _locatedblockpositions (Utilities|Select :Index _index_2 :Option%200 (Math|Vector|MakeVector (+ (.X (Math|Vector|BreakVector (Transformation|GetActorLocation _array_element_2))) 5e+02) (.Y (Math|Vector|BreakVector (Transformation|GetActorLocation _array_element_2))) (.Z (Math|Vector|BreakVector (Transformation|GetActorLocation _array_element_2)))) :Option%201 (Math|Vector|MakeVector (.X (Math|Vector|BreakVector (Transformation|GetActorLocation _array_element_2))) (+ (.Y (Math|Vector|BreakVector (Transformation|GetActorLocation _array_element_2))) 5e+02) (.Z (Math|Vector|BreakVector (Transformation|GetActorLocation _array_element_2)))) :Option%202 "0, 0, 0" :Option%203 "0, 0, 0"))
            (bind _aschunk (Utilities|Casting|CastToChunk (Actor|GetParentActor (Utilities|Array|Get(acopy) (Variables|Default|GetLocatedBlocks) (Utilities|Array|FindItem _locatedblockpositions (Utilities|Select :Index _index_2 :Option%200 (Math|Vector|MakeVector (+ (.X (Math|Vector|BreakVector (Transformation|GetActorLocation _array_element_2))) 5e+02) (.Y (Math|Vector|BreakVector (Transformation|GetActorLocation _array_element_2))) (.Z (Math|Vector|BreakVector (Transformation|GetActorLocation _array_element_2)))) :Option%201 (Math|Vector|MakeVector (.X (Math|Vector|BreakVector (Transformation|GetActorLocation _array_element_2))) (+ (.Y (Math|Vector|BreakVector (Transformation|GetActorLocation _array_element_2))) 5e+02) (.Z (Math|Vector|BreakVector (Transformation|GetActorLocation _array_element_2)))) :Option%202 "0, 0, 0" :Option%203 "0, 0, 0"))))))
            (bind _returnvalue (Game|AddComponentbyClass _aschunk "/Script/Engine.ChildActorComponent" false (Math|Transform|MakeTransform (- (Utilities|Select :Index _index_2 :Option%200 (Math|Vector|MakeVector (- (.X (Math|Vector|BreakVector (Utilities|Select :Index _index_2 :Option%200 (Math|Vector|MakeVector (+ (.X (Math|Vector|BreakVector (Transformation|GetActorLocation _array_element_2))) 5e+02) (.Y (Math|Vector|BreakVector (Transformation|GetActorLocation _array_element_2))) (.Z (Math|Vector|BreakVector (Transformation|GetActorLocation _array_element_2)))) :Option%201 (Math|Vector|MakeVector (.X (Math|Vector|BreakVector (Transformation|GetActorLocation _array_element_2))) (+ (.Y (Math|Vector|BreakVector (Transformation|GetActorLocation _array_element_2))) 5e+02) (.Z (Math|Vector|BreakVector (Transformation|GetActorLocation _array_element_2)))) :Option%202 "0, 0, 0" :Option%203 "0, 0, 0"))) 2.5e+02) (.Y (Math|Vector|BreakVector (Utilities|Select :Index _index_2 :Option%200 (Math|Vector|MakeVector (+ (.X (Math|Vector|BreakVector (Transformation|GetActorLocation _array_element_2))) 5e+02) (.Y (Math|Vector|BreakVector (Transformation|GetActorLocation _array_element_2))) (.Z (Math|Vector|BreakVector (Transformation|GetActorLocation _array_element_2)))) :Option%201 (Math|Vector|MakeVector (.X (Math|Vector|BreakVector (Transformation|GetActorLocation _array_element_2))) (+ (.Y (Math|Vector|BreakVector (Transformation|GetActorLocation _array_element_2))) 5e+02) (.Z (Math|Vector|BreakVector (Transformation|GetActorLocation _array_element_2)))) :Option%202 "0, 0, 0" :Option%203 "0, 0, 0"))) (.Z (Math|Vector|BreakVector (Utilities|Select :Index _index_2 :Option%200 (Math|Vector|MakeVector (+ (.X (Math|Vector|BreakVector (Transformation|GetActorLocation _array_element_2))) 5e+02) (.Y (Math|Vector|BreakVector (Transformation|GetActorLocation _array_element_2))) (.Z (Math|Vector|BreakVector (Transformation|GetActorLocation _array_element_2)))) :Option%201 (Math|Vector|MakeVector (.X (Math|Vector|BreakVector (Transformation|GetActorLocation _array_element_2))) (+ (.Y (Math|Vector|BreakVector (Transformation|GetActorLocation _array_element_2))) 5e+02) (.Z (Math|Vector|BreakVector (Transformation|GetActorLocation _array_element_2)))) :Option%202 "0, 0, 0" :Option%203 "0, 0, 0")))) :Option%201 (Math|Vector|MakeVector (.X (Math|Vector|BreakVector (Utilities|Select :Index _index_2 :Option%200 (Math|Vector|MakeVector (+ (.X (Math|Vector|BreakVector (Transformation|GetActorLocation _array_element_2))) 5e+02) (.Y (Math|Vector|BreakVector (Transformation|GetActorLocation _array_element_2))) (.Z (Math|Vector|BreakVector (Transformation|GetActorLocation _array_element_2)))) :Option%201 (Math|Vector|MakeVector (.X (Math|Vector|BreakVector (Transformation|GetActorLocation _array_element_2))) (+ (.Y (Math|Vector|BreakVector (Transformation|GetActorLocation _array_element_2))) 5e+02) (.Z (Math|Vector|BreakVector (Transformation|GetActorLocation _array_element_2)))) :Option%202 "0, 0, 0" :Option%203 "0, 0, 0"))) (- (.Y (Math|Vector|BreakVector (Utilities|Select :Index _index_2 :Option%200 (Math|Vector|MakeVector (+ (.X (Math|Vector|BreakVector (Transformation|GetActorLocation _array_element_2))) 5e+02) (.Y (Math|Vector|BreakVector (Transformation|GetActorLocation _array_element_2))) (.Z (Math|Vector|BreakVector (Transformation|GetActorLocation _array_element_2)))) :Option%201 (Math|Vector|MakeVector (.X (Math|Vector|BreakVector (Transformation|GetActorLocation _array_element_2))) (+ (.Y (Math|Vector|BreakVector (Transformation|GetActorLocation _array_element_2))) 5e+02) (.Z (Math|Vector|BreakVector (Transformation|GetActorLocation _array_element_2)))) :Option%202 "0, 0, 0" :Option%203 "0, 0, 0"))) 2.5e+02) (.Z (Math|Vector|BreakVector (Utilities|Select :Index _index_2 :Option%200 (Math|Vector|MakeVector (+ (.X (Math|Vector|BreakVector (Transformation|GetActorLocation _array_element_2))) 5e+02) (.Y (Math|Vector|BreakVector (Transformation|GetActorLocation _array_element_2))) (.Z (Math|Vector|BreakVector (Transformation|GetActorLocation _array_element_2)))) :Option%201 (Math|Vector|MakeVector (.X (Math|Vector|BreakVector (Transformation|GetActorLocation _array_element_2))) (+ (.Y (Math|Vector|BreakVector (Transformation|GetActorLocation _array_element_2))) 5e+02) (.Z (Math|Vector|BreakVector (Transformation|GetActorLocation _array_element_2)))) :Option%202 "0, 0, 0" :Option%203 "0, 0, 0"))))) (Transformation|GetActorLocation _aschunk)) "0, 0, 0" "0.500000,0.500000,0.500000")))
            (ChildActorComponent|SetChildActorClass _returnvalue "/Game/Blueprints/Generation/BlockSpawn.BlockSpawn_C")
            (bind _asblock_spawn_2 (Utilities|Casting|CastToBlockSpawn (Variables|/Script/Engine.ChildActorComponent|GetChildActor _returnvalue)))
            (Default|AddSolid _asblock_spawn_2)
            (bind _returnvalue_2 (Rendering|Material|CreateDynamicMaterialInstance (Variables|/Game/Blueprints/Generation/BlockSpawn.BlockSpawn_C|GetCube _asblock_spawn_2) 0 (Rendering|Material|GetMaterial (Variables|/Game/Blueprints/Generation/BlockSpawn.BlockSpawn_C|GetCube _asblock_spawn_2) 0) "None" :!class /Script/Engine.PrimitiveComponent))
            (bind _returnvalue_3 (Rendering|Material|CreateDynamicMaterialInstance (Variables|/Game/Blueprints/Generation/BlockSpawn.BlockSpawn_C|GetCube (Utilities|Array|Get(acopy) (Variables|Default|GetLocatedBlocks) (Utilities|Array|FindItem _locatedblockpositions (Utilities|Select :Index _index_2 :Option%200 (Math|Vector|MakeVector (+ (.X (Math|Vector|BreakVector (Transformation|GetActorLocation _array_element_2))) 5e+02) (.Y (Math|Vector|BreakVector (Transformation|GetActorLocation _array_element_2))) (.Z (Math|Vector|BreakVector (Transformation|GetActorLocation _array_element_2)))) :Option%201 (Math|Vector|MakeVector (.X (Math|Vector|BreakVector (Transformation|GetActorLocation _array_element_2))) (+ (.Y (Math|Vector|BreakVector (Transformation|GetActorLocation _array_element_2))) 5e+02) (.Z (Math|Vector|BreakVector (Transformation|GetActorLocation _array_element_2)))) :Option%202 "0, 0, 0" :Option%203 "0, 0, 0")))) 0 (Rendering|Material|GetMaterial (Variables|/Game/Blueprints/Generation/BlockSpawn.BlockSpawn_C|GetCube (Utilities|Array|Get(acopy) (Variables|Default|GetLocatedBlocks) (Utilities|Array|FindItem _locatedblockpositions (Utilities|Select :Index _index_2 :Option%200 (Math|Vector|MakeVector (+ (.X (Math|Vector|BreakVector (Transformation|GetActorLocation _array_element_2))) 5e+02) (.Y (Math|Vector|BreakVector (Transformation|GetActorLocation _array_element_2))) (.Z (Math|Vector|BreakVector (Transformation|GetActorLocation _array_element_2)))) :Option%201 (Math|Vector|MakeVector (.X (Math|Vector|BreakVector (Transformation|GetActorLocation _array_element_2))) (+ (.Y (Math|Vector|BreakVector (Transformation|GetActorLocation _array_element_2))) 5e+02) (.Z (Math|Vector|BreakVector (Transformation|GetActorLocation _array_element_2)))) :Option%202 "0, 0, 0" :Option%203 "0, 0, 0")))) 0) "None" :!class /Script/Engine.PrimitiveComponent))
            (bind _returnvalue_4 (Rendering|Material|GetVectorParameterValue _returnvalue_3 "Color0" :!class /Script/Engine.MaterialInstanceDynamic))
            (bind _returnvalue_5 (Rendering|Material|GetVectorParameterValue _returnvalue_3 "Color1" :!class /Script/Engine.MaterialInstanceDynamic))
            (bind _returnvalue_6 (Rendering|Material|GetVectorParameterValue _returnvalue_3 "Color3" :!class /Script/Engine.MaterialInstanceDynamic))
            (bind _returnvalue_7 (Rendering|Material|GetScalarParameterValue _returnvalue_3 "NumberOfColors" :!class /Script/Engine.MaterialInstanceDynamic))
            (bind _returnvalue_8 (Rendering|Material|CreateDynamicMaterialInstance (Variables|/Game/Blueprints/Generation/BlockSpawn.BlockSpawn_C|GetCube _array_element_2) 0 (Rendering|Material|GetMaterial (Variables|/Game/Blueprints/Generation/BlockSpawn.BlockSpawn_C|GetCube _array_element_2) 0) "None" :!class /Script/Engine.PrimitiveComponent))
            (Rendering|Material|SetVectorParameterValue _returnvalue_8 "Mat1Color0" _returnvalue_4 :!class /Script/Engine.MaterialInstanceDynamic)
            (Rendering|Material|SetVectorParameterValue _returnvalue_8 "Mat1Color1" _returnvalue_5 :!class /Script/Engine.MaterialInstanceDynamic)
            (Rendering|Material|SetVectorParameterValue _returnvalue_8 "Mat1Color2" _returnvalue_6 :!class /Script/Engine.MaterialInstanceDynamic)
            (Rendering|Material|SetScalarParameterValue _returnvalue_8 "Blend" 0.5 :!class /Script/Engine.MaterialInstanceDynamic)
            (Rendering|Material|SetScalarParameterValue _returnvalue_8 "Colors" _returnvalue_7 :!class /Script/Engine.MaterialInstanceDynamic)
            (Class|MaterialInstanceDynamic|InterpolateMaterialInstanceParams _returnvalue_2 _returnvalue_8 _returnvalue_3 0.5)))))))

(event Custom|RemoveAllProjectiles
  (bind _outactors (Actor|GetAllActorsOfClass "/Game/Projectiles/BP_BaseProjectile.BP_BaseProjectile_C"))
  (for _array_element _outactors
    (Actor|DestroyActor _array_element)
    (Default|RemoveProjectile (CallFunction|GetPlayerOnePawn) _array_element)))

(event EventBeginPlay
  (EventDispatchers|BindEventtoKillPlayerOne (delegate Custom|PlayerOneDeath))
  (EventDispatchers|BindEventtoKillPlayerTwo (delegate Custom|PlayerTwoDeath)))

(fn ConstructionScript)