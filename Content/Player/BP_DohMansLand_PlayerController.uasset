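; Player controller for a two-player tank game that handles both players' input in one Blueprint.
; Separate P1 and P2 fire, move, rotate and turret-aim inputs are forwarded to the player one and player two pawns.
; SpawnPlayerEvent spawns a BP_BaseTank at the start transform plus a new controller to possess it.
; Death handling is an empty stub, and several spawn, respawn and kill-binding experiments are left disconnected.
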(event Custom|PlayerDeath)

(event Custom|SpawnPlayerEvent
  ;[1 1 1] this works on one pawn, but not p2
  (bind _returnvalue (Game|SpawnActorfromClass "/Game/Blueprints/Player/BP_BaseTank.BP_BaseTank_C" (Math|Transform|MakeTransform (Variables|Default|GetPlayerStartLocation) (Variables|Default|GetPlayerStartRotation)) "Undefined" 0 1 0))
  (Variables|Default|SetTank2Ref _returnvalue)
  (bind _returnvalue_2 (Game|SpawnActorfromClass "BP_DohMansLand_PlayerController_C" (Variables|Default|GetEmptyTransform) "Undefined" 0 0))
  (Pawn|Possess _returnvalue_2 (Variables|Default|GetTank2Ref)))

(event EventBeginPlay
  (Class|PlayerController|SetDeprecatedInputYawScale (Variables|Default|GetYawScaling))
  (if (< (Variables|/Game/Player/BP_DohMansLand_GameInstance.BP_DohMansLand_GameInstance_C|GetLevelNumber (CallFunction|GetDohMansLandGameInstance)) 1)
    _))

(event Input|ActionEvents|InputActionFireP1
  (params (Key :type Key%20Structure :default "None"))
  ;[0.2 0.2 0.2] Player One Input
  (:Pressed
    (Default|Fire (CallFunction|GetPlayerOnePawn))))

(event Input|ActionEvents|InputActionFireP2
  (params (Key :type Key%20Structure :default "None"))
  ;[0.2 0.2 0.2] Player Two Input
  (:Pressed
    (Default|Fire (CallFunction|GetPlayerTwoPawn))))

(event Input|AxisEvents|InputAxisAimRightP1
  (params (AxisValue :type Float%20%28single-precision%29))
  ;[0.2 0.2 0.2] Player One Input
  (Default|RotateTurret (CallFunction|GetPlayerOnePawn) AxisValue))

(event Input|AxisEvents|InputAxisRightP1
  (params (AxisValue :type Float%20%28single-precision%29))
  ;[0.2 0.2 0.2] Player One Input
  (Default|RotateBody (CallFunction|GetPlayerOnePawn) AxisValue))

(event Input|AxisEvents|InputAxisUpP1
  (params (AxisValue :type Float%20%28single-precision%29))
  ;[0.2 0.2 0.2] Player One Input
  (Default|MoveForward (CallFunction|GetPlayerOnePawn) AxisValue))

(event Input|AxisEvents|InputAxisUpP2
  (params (AxisValue :type Float%20%28single-precision%29))
  ;[0.2 0.2 0.2] Player Two Input
  (Default|MoveForward (CallFunction|GetPlayerTwoPawn) AxisValue))

(event Input|AxisEvents|InputAxisRightP2
  (params (AxisValue :type Float%20%28single-precision%29))
  ;[0.2 0.2 0.2] Player Two Input
  (Default|RotateBody (CallFunction|GetPlayerTwoPawn) AxisValue))

(event Input|AxisEvents|InputAxisAimRightP2
  (params (AxisValue :type Float%20%28single-precision%29))
  ;[0.2 0.2 0.2] Player Two Input
  (Default|RotateTurret (CallFunction|GetPlayerTwoPawn) AxisValue))

(fn ConstructionScript)