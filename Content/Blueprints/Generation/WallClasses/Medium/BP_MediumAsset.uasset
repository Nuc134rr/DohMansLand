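; BP_MediumAsset is a medium-sized asset in the wall classes used by generation, adding random material variation to specific meshes.
; After the parent construction script runs, it checks which static mesh is assigned.
; A 2x4 Lego brick gets a dynamic material with a random color from LegoBrickColors.
; A tank deck gets one with a random texture from TankDeckTextures.
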(fn ConstructionScript
  (bind _mesh (Variables|Character|GetMesh))
  (bind _staticmesh (Variables|/Script/Engine.StaticMeshComponent|GetStaticMesh _mesh))
  ;[0.2 0.2 0.2] Dynamic material setup for certain meshes
  (|CallParentFunction)
  (Utilities|FlowControl|Sequence
    (:then_0
      (if (== _staticmesh "/Game/Assets/Meshes/LevelProps/Medium/SM_Lego2x4.SM_Lego2x4")
        (bind _returnvalue (Rendering|Material|CreateDynamicMaterialInstance (Variables|Character|GetMesh) 0 "/Game/Assets/Materials/Lego/M_LegobrickRed.M_LegobrickRed" "None" :!class /Script/Engine.PrimitiveComponent))
        (Rendering|Material|SetVectorParameterValue _returnvalue "Color" (.OutItem (Utilities|Array|Random (LocalVariables|GetLegoBrickColors))) :!class /Script/Engine.MaterialInstanceDynamic)))
    (:then_1
      (if (== _staticmesh "/Game/Assets/Meshes/LevelProps/Small/SM_TankDeck.SM_TankDeck")
        (bind _returnvalue_2 (Rendering|Material|CreateDynamicMaterialInstance (Variables|Character|GetMesh) 0 "/Game/Assets/Materials/Techdeck/M_TankDeck.M_TankDeck" "None" :!class /Script/Engine.PrimitiveComponent))
        (Rendering|Material|SetTextureParameterValue _returnvalue_2 "DeckTex" (.OutItem (Utilities|Array|Random (LocalVariables|GetTankDeckTextures))))))))