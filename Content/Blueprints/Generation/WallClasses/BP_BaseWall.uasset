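; Base wall actor for level generation that sizes itself and picks a random mesh for that size in its construction script.
; It measures the mesh's X-Y bounds in 500x500 blocks and classifies it as Small, Medium or Large.
; The size class sets a mass override, with physics simulation off, and selects which DohMansLand game mode mesh list to draw from.
; The block-break Niagara effect in the event graph is unconnected.
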(event EventTick
  (params (DeltaSeconds :type Float%20%28single-precision%29)))

(event EventDestroyed)

(fn ConstructionScript
  (bind _returnvalue (CallFunction|GetDohMansLandGameMode))
  (bind _mesh (Variables|Default|GetMesh))
  (bind _boxextent (Collision|GetComponentBounds _mesh))
  (bind _returnvalue_2 (* _boxextent 2.0))
  ;[0.2 0.2 0.2] Determines the size of the asset for meshes
  (Physics|SetSimulatePhysics (Variables|Default|GetMesh) false)
  (Utilities|FlowControl|Sequence
    (:then_0
      (bind _output_get (Variables|Default|SetMeshArea (/ (* (.x _returnvalue_2) (.y _returnvalue_2)) 2.5e+05)))
      (if (> _output_get (Variables|Area|GetMaxSmallArea)) ; true= med/large\nfalse=small
        (if (> (Variables|Default|GetMeshArea) (Variables|Area|GetMaxMediumArea)) ; true=large\nfalse=med
          (Variables|Default|SetSizeEnum "NewEnumerator0")
          (else
            (Variables|Default|SetSizeEnum "NewEnumerator1")))
        (else
          (Variables|Default|SetSizeEnum "NewEnumerator2")))
      (Class|PrimitiveComponent|SetMassOverrideinKg (Variables|Default|GetMesh) "None" (Utilities|Select :Index (Variables|Default|GetSizeEnum) :NewEnumerator0 1e+03 :NewEnumerator1 1e+02 :NewEnumerator2 1e+01) true))
    (:then_1
      ;[0.2 0.2 0.2] Chooses a mesh
      (Components|StaticMesh|SetStaticMesh (Variables|Default|GetMesh) (.OutItem (Utilities|Array|Random (Utilities|Select :Index (Variables|Default|GetSizeEnum) :NewEnumerator0 (Variables|/Game/Blueprints/Player/BP_DohMansLand_GameMode.BP_DohMansLand_GameMode_C|GetLargeMeshes _returnvalue) :NewEnumerator1 (Variables|/Game/Blueprints/Player/BP_DohMansLand_GameMode.BP_DohMansLand_GameMode_C|GetMediumMeshes _returnvalue) :NewEnumerator2 (Variables|/Game/Blueprints/Player/BP_DohMansLand_GameMode.BP_DohMansLand_GameMode_C|GetSmallMeshes _returnvalue))))))))