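; BP_SmallAsset is a small-prop actor in the generation wall classes that multiplies itself when it carries the Jax mesh.
; On BeginPlay, a mesh check triggers spawning of a few more BP_SmallAsset actors at random navigable points nearby, with random yaw.
; Each copy is flagged moveable and non-destructible and receives the same mesh after spawning, followed by a placeholder debug print.
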(event EventBeginPlay
  (|CallParentFunction)
  (if (== (Variables|/Script/Engine.StaticMeshComponent|GetStaticMesh (Variables|Character|GetMesh)) "/Game/Assets/Meshes/SM_Jax_Jax1.SM_Jax_Jax1")
    (for _index (range 0 (Math|Random|RandomIntegerinRange 2 4))
      (bind _returnvalue (Game|SpawnActorfromClass "BP_SmallAsset_C" (Math|Transform|MakeTransform (.RandomLocation (Class|NavigationSystemV1|GetRandomPointinNavigableRadius (Transformation|GetActorLocation) 5e+02 0 0)) (Math|Rotator|MakeRotator 0.0 0.0 (.yaw (Math|Random|RandomRotator false))) "1.000000,1.000000,1.000000") "Undefined" 0 0 true false 0))
      (Components|StaticMesh|SetStaticMesh (Variables|/Game/Blueprints/Generation/WallClasses/BP_BaseWall.BP_BaseWall_C|GetMesh _returnvalue) (Variables|/Script/Engine.StaticMeshComponent|GetStaticMesh (Variables|Character|GetMesh)))
      (Development|PrintString "asdfasfasdf"))))

(fn ConstructionScript
  (|CallParentFunction))