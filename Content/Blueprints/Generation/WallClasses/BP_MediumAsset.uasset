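; BP_MediumAsset is a generation wall-class Blueprint for a medium asset, extending its parent's construction and BeginPlay logic.
; After the parent construction script runs, it checks whether its mesh is the 2x4 Lego brick.
; If so, it creates a dynamic instance of the red brick material and sets its Color parameter to a random entry from LegoBrickColors.
; BeginPlay only calls the parent implementation.
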(event EventBeginPlay
  (|CallParentFunction))

(fn ConstructionScript
  (|CallParentFunction)
  (if (== (Variables|/Script/Engine.StaticMeshComponent|GetStaticMesh (Variables|Character|GetMesh)) "/Game/Assets/Meshes/LevelProps/Medium/SM_Lego2x4.SM_Lego2x4")
    (bind _returnvalue (Rendering|Material|CreateDynamicMaterialInstance (Variables|Character|GetMesh) 0 "/Game/Assets/Materials/M_LegobrickRed.M_LegobrickRed" "None" :!class /Script/Engine.PrimitiveComponent))
    (Rendering|Material|SetVectorParameterValue _returnvalue "Color" (.OutItem (Utilities|Array|Random (LocalVariables|GetLegoBrickColors))) :!class /Script/Engine.MaterialInstanceDynamic)))