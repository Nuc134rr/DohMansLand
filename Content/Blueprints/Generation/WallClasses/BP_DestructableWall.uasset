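; Destructible wall Blueprint that breaks when hit by projectiles.
; DecrementLives destroys it instantly for a BP_BigProjectile, while any other projectile removes one life and destroys it at zero, intended as three hits.
; On Destroyed, it spawns the FX_BlockBreak effect at its transform and prints that location and rotation as debug output.
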(event Custom|DecrementLives
  (params (Projectile :type BP%20Base%20Projectile%20Object%20Reference))
  ;[0.2 0.2 0.2] Checks to see if it was hit by a projectile
  ; -If the projectile is big, destory the actor in one hit
  ; -If not, it will take 3 hits to destroy
  (Utilities|Casting|CastToBP_BigProjectile Projectile ; fail means regular proj\nsuccess means big proj
    (:then
      (Actor|DestroyActor :!label _label))
    (:CastFailed
      (bind _result (Math|Integer|DecrementInt (Variables|Default|GetLives))
        (:%20%20
          (if (== _result 0)
            (goto _label)))))))

(event EventBeginPlay
  (|CallParentFunction))

(event EventDestroyed
  (bind _self_ref (Variables|Default|GetSelf%20ref))
  (bind _returnvalue (Transformation|GetActorLocation _self_ref))
  (bind _returnvalue_2 (Transformation|GetActorRotation _self_ref))
  (Niagara|SpawnSystematLocation "/Game/Assets/FX/FX_BlockBreak.FX_BlockBreak" _returnvalue _returnvalue_2)
  (Development|PrintString (Utilities|String|ToString(Vector) _returnvalue))
  (Development|PrintString (Utilities|String|ToString(Rotator) _returnvalue_2) true true "(R=0.516587,G=0.112235,B=1.000000,A=1.000000)"))

(fn ConstructionScript
  (|CallParentFunction))