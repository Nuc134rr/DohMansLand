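; BP_SorryPawn is a small wall-class prop for level generation that takes on a random tank color.
; Its construction script runs the parent's, creates a dynamic material instance on the mesh's first slot and sets the PawnColor parameter.
; The color comes from the DohMansLand game mode's TankVariables, using a random pick from a fixed index list that skips index 1.
; The event graph holds no active logic.
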(event EventBeginPlay
  (|CallParentFunction) ; This node is disabled and will not be called.\nDrag off pins to build functionality.
)

(event Collision|EventActorBeginOverlap
  (params (OtherActor :type Actor%20Object%20Reference)))

(event EventTick
  (params (DeltaSeconds :type Float%20%28single-precision%29)))

(fn ConstructionScript
  (bind _mesh (Variables|Character|GetMesh))
  (|CallParentFunction)
  (bind _returnvalue (Rendering|Material|CreateDynamicMaterialInstance _mesh 0 (Rendering|Material|GetMaterial _mesh 0) "None" :!class /Script/Engine.PrimitiveComponent))
  (Rendering|Material|SetVectorParameterValue _returnvalue "PawnColor" (.tankcolor (Utilities|Array|Get(acopy) (Variables|/Game/Blueprints/Player/BP_DohMansLand_GameMode.BP_DohMansLand_GameMode_C|GetTank%20Variables (CallFunction|GetDohMansLandGameMode)) (.OutItem (Utilities|Array|Random (Utilities|Array|MakeArray 0 2 3 4))))) :!class /Script/Engine.MaterialInstanceDynamic))