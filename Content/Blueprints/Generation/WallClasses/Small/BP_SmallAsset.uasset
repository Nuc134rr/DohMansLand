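; BP_SmallAsset is a small-asset Blueprint among the generation wall classes, adding random color variation to Lego bricks.
; Its construction script runs the parent's, then checks whether the mesh is the 2x2 Lego brick.
; If so, it creates a dynamic instance of the red brick material on element 1 and sets its Color parameter to a random pick from LegoBrickColors.
; BeginPlay only calls the parent.
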(event EventBeginPlay
  (|CallParentFunction))

(fn ConstructionScript
  ;[0.2 0.2 0.2] Dynamic material for the lego bricks
  (|CallParentFunction)
  (if (== (Variables|/Script/Engine.StaticMeshComponent|GetStaticMesh (Variables|Character|GetMesh)) "/Game/Assets/Meshes/LevelProps/Small/SM_Lego2x2.SM_Lego2x2")
    (bind _returnvalue (Rendering|Material|CreateDynamicMaterialInstance (Variables|Character|GetMesh) 1 "/Game/Assets/Materials/Lego/M_LegobrickRed.M_LegobrickRed" "None" :!class /Script/Engine.PrimitiveComponent))
    (Rendering|Material|SetVectorParameterValue _returnvalue "Color" (.OutItem (Utilities|Array|Random (LocalVariables|GetLegoBrickColors))) :!class /Script/Engine.MaterialInstanceDynamic)))