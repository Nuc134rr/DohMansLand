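; BP_FloorWithTreads is a floor that accumulates tread marks and can fade its material to an ice look for no friction.
; BeginPlay feeds a render target, proportioned to the mesh bounds, into a dynamic material and blocks a custom trace channel for tread detection.
; Treads queued through AddToTreadArray are batch-drawn on Tick at bounds-normalized positions, then cleared.
; SetNoFrictionMaterial plays or reverses a timeline driving the NoFriction parameter.
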(event Custom|AddToTreadArray
  (params (Added%20Variable :type Tank%20Color%20Trans%20Structure))
  ;[1 1 1] Run on component to add new treads
  (Utilities|Array|Add (Variables|Default|GetNew%20Treads) Added%20Variable))

(event Custom|SetNoFrictionMaterial
  (params (bInitialSet :type Boolean))
  ;[1 1 1] Changes the material to ice when no friction is picked up
  (if bInitialSet
    (bind _alpha (Timeline|NoFrictionLerp Play)
      (:Update
        (bind _output_get (Variables|Default|SetAlpha _alpha))
        (Rendering|Material|SetScalarParameterValue (Variables|Default|GetMaterial%20Instance) "NoFriction" _output_get :!class /Script/Engine.MaterialInstanceDynamic)))
    (else
      (Timeline|NoFrictionLerp Reverse))))

(event EventBeginPlay
  (bind _staticmeshcomponent (Variables|Debug|GetStaticMeshComponent))
  (bind _boxextent (Collision|GetComponentBounds _staticmeshcomponent))
  (bind _returnvalue (/ (.y _boxextent) (.x _boxextent)))
  (bind _returnvalue_2 (* (Math|Vector|MakeVector 1.0 _returnvalue 0.0) "2048.000000,2048.000000,0"))
  ;[1 1 1] Creating default thingies
  (bind _returnvalue_3 (Rendering|Material|CreateDynamicMaterialInstance (Variables|Debug|GetStaticMeshComponent) 0 (Variables|Default|GetSource%20Material) "None" :!class /Script/Engine.PrimitiveComponent)) ; Makes variable material
  (Variables|Default|SetMaterial%20Instance _returnvalue_3)
  (bind _returnvalue_4 (Rendering|CreateRenderTarget2D (Math|Float|Truncate (.x _returnvalue_2)) (Math|Float|Truncate (.y _returnvalue_2)) "RTF_RGBA16f" "(R=0.000000,G=0.000000,B=0.000000,A=0.076000)"))
  (bind _output_get (Variables|Default|SetRender%20Texture _returnvalue_4))
  (Rendering|Material|SetTextureParameterValue (Variables|Default|GetMaterial%20Instance) "Treads" _output_get) ; Sets material reference to our render target
  (Collision|SetCollisionResponsetoChannel (Variables|Debug|GetStaticMeshComponent) "ECC_GameTraceChannel4" "ECR_Block") ; Customchannel only tread component uses.\nMakes sure we don't get blocked by other objects
)

(event EventTick
  (params (DeltaSeconds :type Float%20%28single-precision%29))
  (if (> (Utilities|Array|Length (Variables|Default|GetNew%20Treads)) 0) ; hopefully helps with performance
    ;[1 1 1] Drawing to texture
    (bind (_canvas _size _context) (Rendering|BeginDrawCanvastoRenderTarget (Variables|Default|GetRender%20Texture))) ; Starts the drawing process and ends after loop finishes
    (for _array_element (Variables|Default|GetNew%20Treads)
      (Canvas|DrawTexture :self _canvas :RenderTexture "/Game/Assets/Textures/Train/treads.treads" :ScreenPosition (- (* _size (Math|Vector2D|MakeVector2D (.ReturnValue_X (|MathsBruv (.location (.transform _array_element)))) (.ReturnValue_Y (|MathsBruv (.location (.transform _array_element)))))) (/ (Variables|Default|GetTread%20Size) "(X=2.000000,Y=2.000000)")) :ScreenSize (Variables|Default|GetTread%20Size) :CoordinateSize "(X=1.000000,Y=1.000000)" :RenderColor (.color _array_element) :BlendMode "BLEND_AlphaComposite" :Rotation (+ (.Yaw (Math|Rotator|BreakRotator (.rotation (.transform _array_element)))) 9e+01) :PivotPoint "(X=0.500000,Y=0.500000)") ; finally draws to the texture on material
    )
    (Rendering|EndDrawCanvastoRenderTarget _context)
    (Utilities|Array|Clear (Variables|Default|GetNew%20Treads)) ; Remove old drawing treads
  ))

(fn ConstructionScript)