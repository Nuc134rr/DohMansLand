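; Foam block tower prop (20x20) built from toy-like mesh pieces such as ramps, cylinders, arches and cubes, which play impact sounds when a tank hits them.
; Each piece has its own hit event that ignores anything other than a BP_BaseTank and passes the impulse to FoamSounds.
; A separate DoOnce per piece, reset after a short delay, throttles repeated sounds from that block.
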(event OnComponentHit(SM_FoamRamp1)
  (params (HitComponent :type Primitive%20Component%20Object%20Reference) (OtherActor :type Actor%20Object%20Reference) (OtherComp :type Primitive%20Component%20Object%20Reference) (NormalImpulse :type Vector :default "0, 0, 0") (Hit :type Hit%20Result%20Structure%20%28by%20ref%29))
  (Utilities|Casting|CastToBP_BaseTank)
  (Utilities|FlowControl|DoOnce false :!label _label
    (:Completed
      (CallFunction|FoamSounds NormalImpulse)
      (Utilities|FlowControl|Delay 1.2)
      (goto _label Reset))))

(event OnComponentHit(SM_FoamCylinder)
  (params (HitComponent :type Primitive%20Component%20Object%20Reference) (OtherActor :type Actor%20Object%20Reference) (OtherComp :type Primitive%20Component%20Object%20Reference) (NormalImpulse :type Vector :default "0, 0, 0") (Hit :type Hit%20Result%20Structure%20%28by%20ref%29))
  (Utilities|Casting|CastToBP_BaseTank)
  (Utilities|FlowControl|DoOnce false :!label _label
    (:Completed
      (CallFunction|FoamSounds NormalImpulse)
      (Utilities|FlowControl|Delay 1.2)
      (goto _label Reset))))

(event OnComponentHit(SM_FoamRectangle2)
  (params (HitComponent :type Primitive%20Component%20Object%20Reference) (OtherActor :type Actor%20Object%20Reference) (OtherComp :type Primitive%20Component%20Object%20Reference) (NormalImpulse :type Vector :default "0, 0, 0") (Hit :type Hit%20Result%20Structure%20%28by%20ref%29))
  (Utilities|Casting|CastToBP_BaseTank)
  (Utilities|FlowControl|DoOnce false :!label _label
    (:Completed
      (CallFunction|FoamSounds NormalImpulse)
      (Utilities|FlowControl|Delay 1.2)
      (goto _label Reset))))

(event OnComponentHit(SM_FoamRectangle1)
  (params (HitComponent :type Primitive%20Component%20Object%20Reference) (OtherActor :type Actor%20Object%20Reference) (OtherComp :type Primitive%20Component%20Object%20Reference) (NormalImpulse :type Vector :default "0, 0, 0") (Hit :type Hit%20Result%20Structure%20%28by%20ref%29))
  (Utilities|Casting|CastToBP_BaseTank)
  (Utilities|FlowControl|DoOnce false :!label _label
    (:Completed
      (CallFunction|FoamSounds NormalImpulse)
      (Utilities|FlowControl|Delay 1.2)
      (goto _label Reset))))

(event OnComponentHit(SM_FoamArch)
  (params (HitComponent :type Primitive%20Component%20Object%20Reference) (OtherActor :type Actor%20Object%20Reference) (OtherComp :type Primitive%20Component%20Object%20Reference) (NormalImpulse :type Vector :default "0, 0, 0") (Hit :type Hit%20Result%20Structure%20%28by%20ref%29))
  (Utilities|Casting|CastToBP_BaseTank)
  (Utilities|FlowControl|DoOnce false :!label _label
    (:Completed
      (CallFunction|FoamSounds NormalImpulse)
      (Utilities|FlowControl|Delay 1.2)
      (goto _label Reset))))

(event OnComponentHit(SM_FoamArch1)
  (params (HitComponent :type Primitive%20Component%20Object%20Reference) (OtherActor :type Actor%20Object%20Reference) (OtherComp :type Primitive%20Component%20Object%20Reference) (NormalImpulse :type Vector :default "0, 0, 0") (Hit :type Hit%20Result%20Structure%20%28by%20ref%29))
  (Utilities|Casting|CastToBP_BaseTank)
  (Utilities|FlowControl|DoOnce false :!label _label
    (:Completed
      (CallFunction|FoamSounds NormalImpulse)
      (Utilities|FlowControl|Delay 1.2)
      (goto _label Reset))))

(event OnComponentHit(SM_FoamArch2)
  (params (HitComponent :type Primitive%20Component%20Object%20Reference) (OtherActor :type Actor%20Object%20Reference) (OtherComp :type Primitive%20Component%20Object%20Reference) (NormalImpulse :type Vector :default "0, 0, 0") (Hit :type Hit%20Result%20Structure%20%28by%20ref%29))
  (Utilities|Casting|CastToBP_BaseTank)
  (Utilities|FlowControl|DoOnce false :!label _label
    (:Completed
      (CallFunction|FoamSounds NormalImpulse)
      (Utilities|FlowControl|Delay 1.2)
      (goto _label Reset))))

(event OnComponentHit(SM_FoamArch3)
  (params (HitComponent :type Primitive%20Component%20Object%20Reference) (OtherActor :type Actor%20Object%20Reference) (OtherComp :type Primitive%20Component%20Object%20Reference) (NormalImpulse :type Vector :default "0, 0, 0") (Hit :type Hit%20Result%20Structure%20%28by%20ref%29))
  (Utilities|Casting|CastToBP_BaseTank)
  (Utilities|FlowControl|DoOnce false :!label _label
    (:Completed
      (CallFunction|FoamSounds NormalImpulse)
      (Utilities|FlowControl|Delay 1.2)
      (goto _label Reset))))

(event OnComponentHit(SM_FoamRamp)
  (params (HitComponent :type Primitive%20Component%20Object%20Reference) (OtherActor :type Actor%20Object%20Reference) (OtherComp :type Primitive%20Component%20Object%20Reference) (NormalImpulse :type Vector :default "0, 0, 0") (Hit :type Hit%20Result%20Structure%20%28by%20ref%29))
  (Utilities|Casting|CastToBP_BaseTank)
  (Utilities|FlowControl|DoOnce false :!label _label
    (:Completed
      (CallFunction|FoamSounds NormalImpulse)
      (Utilities|FlowControl|Delay 1.2)
      (goto _label Reset))))

(event OnComponentHit(SM_FoamRectangle)
  (params (HitComponent :type Primitive%20Component%20Object%20Reference) (OtherActor :type Actor%20Object%20Reference) (OtherComp :type Primitive%20Component%20Object%20Reference) (NormalImpulse :type Vector :default "0, 0, 0") (Hit :type Hit%20Result%20Structure%20%28by%20ref%29))
  (Utilities|Casting|CastToBP_BaseTank)
  (Utilities|FlowControl|DoOnce false :!label _label
    (:Completed
      (CallFunction|FoamSounds NormalImpulse)
      (Utilities|FlowControl|Delay 1.2)
      (goto _label Reset))))

(event OnComponentHit(SM_FoamHolePiece)
  (params (HitComponent :type Primitive%20Component%20Object%20Reference) (OtherActor :type Actor%20Object%20Reference) (OtherComp :type Primitive%20Component%20Object%20Reference) (NormalImpulse :type Vector :default "0, 0, 0") (Hit :type Hit%20Result%20Structure%20%28by%20ref%29))
  (Utilities|Casting|CastToBP_BaseTank)
  (Utilities|FlowControl|DoOnce false :!label _label
    (:Completed
      (CallFunction|FoamSounds NormalImpulse)
      (Utilities|FlowControl|Delay 1.2)
      (goto _label Reset))))

(event OnComponentHit(SM_FoamRectangle3)
  (params (HitComponent :type Primitive%20Component%20Object%20Reference) (OtherActor :type Actor%20Object%20Reference) (OtherComp :type Primitive%20Component%20Object%20Reference) (NormalImpulse :type Vector :default "0, 0, 0") (Hit :type Hit%20Result%20Structure%20%28by%20ref%29))
  (Utilities|Casting|CastToBP_BaseTank)
  (Utilities|FlowControl|DoOnce false :!label _label
    (:Completed
      (CallFunction|FoamSounds NormalImpulse)
      (Utilities|FlowControl|Delay 1.2)
      (goto _label Reset))))

(event OnComponentHit(SM_FoamSemiCircle)
  (params (HitComponent :type Primitive%20Component%20Object%20Reference) (OtherActor :type Actor%20Object%20Reference) (OtherComp :type Primitive%20Component%20Object%20Reference) (NormalImpulse :type Vector :default "0, 0, 0") (Hit :type Hit%20Result%20Structure%20%28by%20ref%29))
  (Utilities|Casting|CastToBP_BaseTank)
  (Utilities|FlowControl|DoOnce false :!label _label
    (:Completed
      (CallFunction|FoamSounds NormalImpulse)
      (Utilities|FlowControl|Delay 1.2)
      (goto _label Reset))))

(event OnComponentHit(SM_FoamSemiCircle2)
  (params (HitComponent :type Primitive%20Component%20Object%20Reference) (OtherActor :type Actor%20Object%20Reference) (OtherComp :type Primitive%20Component%20Object%20Reference) (NormalImpulse :type Vector :default "0, 0, 0") (Hit :type Hit%20Result%20Structure%20%28by%20ref%29))
  (Utilities|Casting|CastToBP_BaseTank)
  (Utilities|FlowControl|DoOnce false :!label _label
    (:Completed
      (CallFunction|FoamSounds NormalImpulse)
      (Utilities|FlowControl|Delay 1.2)
      (goto _label Reset))))

(event OnComponentHit(SM_FoamSemiCircle1)
  (params (HitComponent :type Primitive%20Component%20Object%20Reference) (OtherActor :type Actor%20Object%20Reference) (OtherComp :type Primitive%20Component%20Object%20Reference) (NormalImpulse :type Vector :default "0, 0, 0") (Hit :type Hit%20Result%20Structure%20%28by%20ref%29))
  (Utilities|Casting|CastToBP_BaseTank)
  (Utilities|FlowControl|DoOnce false :!label _label
    (:Completed
      (CallFunction|FoamSounds NormalImpulse)
      (Utilities|FlowControl|Delay 1.2)
      (goto _label Reset))))

(event OnComponentHit(SM_FoamSemiCircle3)
  (params (HitComponent :type Primitive%20Component%20Object%20Reference) (OtherActor :type Actor%20Object%20Reference) (OtherComp :type Primitive%20Component%20Object%20Reference) (NormalImpulse :type Vector :default "0, 0, 0") (Hit :type Hit%20Result%20Structure%20%28by%20ref%29))
  (Utilities|Casting|CastToBP_BaseTank)
  (Utilities|FlowControl|DoOnce false :!label _label
    (:Completed
      (CallFunction|FoamSounds NormalImpulse)
      (Utilities|FlowControl|Delay 1.2)
      (goto _label Reset))))

(event OnComponentHit(SM_FoamCube)
  (params (HitComponent :type Primitive%20Component%20Object%20Reference) (OtherActor :type Actor%20Object%20Reference) (OtherComp :type Primitive%20Component%20Object%20Reference) (NormalImpulse :type Vector :default "0, 0, 0") (Hit :type Hit%20Result%20Structure%20%28by%20ref%29))
  (Utilities|Casting|CastToBP_BaseTank)
  (Utilities|FlowControl|DoOnce false :!label _label
    (:Completed
      (CallFunction|FoamSounds NormalImpulse)
      (Utilities|FlowControl|Delay 1.2)
      (goto _label Reset))))

(event OnComponentHit(SM_FoamCylinder1)
  (params (HitComponent :type Primitive%20Component%20Object%20Reference) (OtherActor :type Actor%20Object%20Reference) (OtherComp :type Primitive%20Component%20Object%20Reference) (NormalImpulse :type Vector :default "0, 0, 0") (Hit :type Hit%20Result%20Structure%20%28by%20ref%29))
  (Utilities|Casting|CastToBP_BaseTank)
  (Utilities|FlowControl|DoOnce false :!label _label
    (:Completed
      (CallFunction|FoamSounds NormalImpulse)
      (Utilities|FlowControl|Delay 1.2)
      (goto _label Reset))))

(event OnComponentHit(SM_FoamTriangle1)
  (params (HitComponent :type Primitive%20Component%20Object%20Reference) (OtherActor :type Actor%20Object%20Reference) (OtherComp :type Primitive%20Component%20Object%20Reference) (NormalImpulse :type Vector :default "0, 0, 0") (Hit :type Hit%20Result%20Structure%20%28by%20ref%29))
  (Utilities|Casting|CastToBP_BaseTank)
  (Utilities|FlowControl|DoOnce false :!label _label
    (:Completed
      (CallFunction|FoamSounds NormalImpulse)
      (Utilities|FlowControl|Delay 1.2)
      (goto _label Reset))))

(fn ConstructionScript)