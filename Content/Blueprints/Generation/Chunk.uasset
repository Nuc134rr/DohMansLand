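; Map chunk that randomly generates a 5x5 grid of BlockSpawn child actors on BeginPlay, occasionally leaving it entirely empty.
; Otherwise it randomly fills blocks, then uses vertical line traces at four neighbor positions to detect blocks and add more solids.
; An anti-softlock pass checks detected tagged map walls, clearing the chunk's border for multiple walls or cutting one straight path for one.
; Non-empty chunks then call GlobalScan on the game mode.
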(event EventBeginPlay
  (bind _returnvalue (Math|Random|RandomIntegerinRange 1 7))
  (bind _0 (Variables|Default|Get0))
  (bind _1 (Variables|Default|Get1))
  (bind _2 (Variables|Default|Get2))
  (bind _3 (Variables|Default|Get3))
  (bind _4 (Variables|Default|Get4))
  (bind _0_2 (Variables|Default|Get0))
  (bind _5 (Variables|Default|Get5))
  (bind _10 (Variables|Default|Get10))
  (bind _15 (Variables|Default|Get15))
  (bind _20 (Variables|Default|Get20))
  (bind _array (Utilities|Array|MakeArray _0 _1 _2 _3 _4))
  (bind _array_2 (Utilities|Array|MakeArray _0_2 _5 _10 _15 _20))
  (Utilities|FlowControl|Sequence
    (:then_0
      ;[1 1 1] Adding Walls of map
      (bind _outactors (Actor|GetAllActorsOfClass "/Game/Blueprints/Generation/BlockSpawn.BlockSpawn_C"))
      (for _array_element _outactors
        (if (Math|Boolean|ORBoolean (Components|ComponentHasTag (Variables|/Script/Engine.Actor|GetRootComponent _array_element) "Wall1") (Components|ComponentHasTag (Variables|/Script/Engine.Actor|GetRootComponent _array_element) "Wall2") (Components|ComponentHasTag (Variables|/Script/Engine.Actor|GetRootComponent _array_element) "Wall3") (Components|ComponentHasTag (Variables|/Script/Engine.Actor|GetRootComponent _array_element) "Wall4"))
          (Utilities|Array|Add (Variables|Default|GetWalls) _array_element)
          (Development|PrintString (Utilities|String|ToString(Boolean) (Math|Boolean|ORBoolean (Components|ComponentHasTag (Variables|/Script/Engine.Actor|GetRootComponent _array_element) "Wall1") (Components|ComponentHasTag (Variables|/Script/Engine.Actor|GetRootComponent _array_element) "Wall2") (Components|ComponentHasTag (Variables|/Script/Engine.Actor|GetRootComponent _array_element) "Wall3") (Components|ComponentHasTag (Variables|/Script/Engine.Actor|GetRootComponent _array_element) "Wall4"))) true true "(R=0.001000,G=1.000000,B=0.000000,A=1.000000)" 1e+01))))
    (:then_1
      ;[1 1 1] Setup blocks in chunk
      (Variables|Default|SetBlocks (Utilities|Array|MakeArray (Variables|Default|Get0) (Variables|Default|Get1) (Variables|Default|Get2) (Variables|Default|Get3) (Variables|Default|Get4) (Variables|Default|Get5) (Variables|Default|Get6) (Variables|Default|Get7) (Variables|Default|Get8) (Variables|Default|Get9) (Variables|Default|Get10) (Variables|Default|Get11) (Variables|Default|Get12) (Variables|Default|Get13) (Variables|Default|Get14) (Variables|Default|Get15) (Variables|Default|Get16) (Variables|Default|Get17) (Variables|Default|Get18) (Variables|Default|Get19) (Variables|Default|Get20) (Variables|Default|Get21) (Variables|Default|Get22) (Variables|Default|Get23) (Variables|Default|Get24)))
      ;[1 1 1] EmptyChunk Generation
      (if (> (Math|Random|RandomIntegerinRange 1 7) 1)
        ;[1 1 1] RandomBlockGen
        (for _array_element_2 (Variables|Default|GetBlocks)
          (bind _asblock_spawn (Utilities|Casting|CastToBlockSpawn (Variables|/Script/Engine.ChildActorComponent|GetChildActor _array_element_2)))
          (switch int (select (< _returnvalue 4) (/ _returnvalue _returnvalue) 0)
            (:0
              (Default|EmptyBlock _asblock_spawn))
            (:1
              (Default|AddSolid _asblock_spawn))))
        (for _array_element_3 (Variables|Default|GetBlocks)
          (bind _asblock_spawn_2 (Utilities|Casting|CastToBlockSpawn (Variables|/Script/Engine.ChildActorComponent|GetChildActor _array_element_3)))
          ;[1 1 1] Find Neighboring Blocks
          (for _index (range 0 3)
            (bind _outhit (Collision|LineTraceForObjects (Math|Vector|MakeVector (.x (Utilities|Select :Index _index :Option%200 (Math|Vector|MakeVector (+ (.x (Transformation|GetActorLocation _asblock_spawn_2)) 5e+02) (.y (Transformation|GetActorLocation _asblock_spawn_2)) (.z (Transformation|GetActorLocation _asblock_spawn_2))) :Option%201 (Math|Vector|MakeVector (.x (Transformation|GetActorLocation _asblock_spawn_2)) (+ (.y (Transformation|GetActorLocation _asblock_spawn_2)) 5e+02) (.z (Transformation|GetActorLocation _asblock_spawn_2))) :Option%202 (Math|Vector|MakeVector (- (.x (Transformation|GetActorLocation _asblock_spawn_2)) 5e+02) (.y (Transformation|GetActorLocation _asblock_spawn_2)) (.z (Transformation|GetActorLocation _asblock_spawn_2))) :Option%203 (Math|Vector|MakeVector (.x (Transformation|GetActorLocation _asblock_spawn_2)) (- (.y (Transformation|GetActorLocation _asblock_spawn_2)) 5e+02) (.z (Transformation|GetActorLocation _asblock_spawn_2))))) (.y (Utilities|Select :Index _index :Option%200 (Math|Vector|MakeVector (+ (.x (Transformation|GetActorLocation _asblock_spawn_2)) 5e+02) (.y (Transformation|GetActorLocation _asblock_spawn_2)) (.z (Transformation|GetActorLocation _asblock_spawn_2))) :Option%201 (Math|Vector|MakeVector (.x (Transformation|GetActorLocation _asblock_spawn_2)) (+ (.y (Transformation|GetActorLocation _asblock_spawn_2)) 5e+02) (.z (Transformation|GetActorLocation _asblock_spawn_2))) :Option%202 (Math|Vector|MakeVector (- (.x (Transformation|GetActorLocation _asblock_spawn_2)) 5e+02) (.y (Transformation|GetActorLocation _asblock_spawn_2)) (.z (Transformation|GetActorLocation _asblock_spawn_2))) :Option%203 (Math|Vector|MakeVector (.x (Transformation|GetActorLocation _asblock_spawn_2)) (- (.y (Transformation|GetActorLocation _asblock_spawn_2)) 5e+02) (.z (Transformation|GetActorLocation _asblock_spawn_2))))) (+ (.z (Utilities|Select :Index _index :Option%200 (Math|Vector|MakeVector (+ (.x (Transformation|GetActorLocation _asblock_spawn_2)) 5e+02) (.y (Transformation|GetActorLocation _asblock_spawn_2)) (.z (Transformation|GetActorLocation _asblock_spawn_2))) :Option%201 (Math|Vector|MakeVector (.x (Transformation|GetActorLocation _asblock_spawn_2)) (+ (.y (Transformation|GetActorLocation _asblock_spawn_2)) 5e+02) (.z (Transformation|GetActorLocation _asblock_spawn_2))) :Option%202 (Math|Vector|MakeVector (- (.x (Transformation|GetActorLocation _asblock_spawn_2)) 5e+02) (.y (Transformation|GetActorLocation _asblock_spawn_2)) (.z (Transformation|GetActorLocation _asblock_spawn_2))) :Option%203 (Math|Vector|MakeVector (.x (Transformation|GetActorLocation _asblock_spawn_2)) (- (.y (Transformation|GetActorLocation _asblock_spawn_2)) 5e+02) (.z (Transformation|GetActorLocation _asblock_spawn_2))))) 1e+03)) (Math|Vector|MakeVector (.x (Utilities|Select :Index _index :Option%200 (Math|Vector|MakeVector (+ (.x (Transformation|GetActorLocation _asblock_spawn_2)) 5e+02) (.y (Transformation|GetActorLocation _asblock_spawn_2)) (.z (Transformation|GetActorLocation _asblock_spawn_2))) :Option%201 (Math|Vector|MakeVector (.x (Transformation|GetActorLocation _asblock_spawn_2)) (+ (.y (Transformation|GetActorLocation _asblock_spawn_2)) 5e+02) (.z (Transformation|GetActorLocation _asblock_spawn_2))) :Option%202 (Math|Vector|MakeVector (- (.x (Transformation|GetActorLocation _asblock_spawn_2)) 5e+02) (.y (Transformation|GetActorLocation _asblock_spawn_2)) (.z (Transformation|GetActorLocation _asblock_spawn_2))) :Option%203 (Math|Vector|MakeVector (.x (Transformation|GetActorLocation _asblock_spawn_2)) (- (.y (Transformation|GetActorLocation _asblock_spawn_2)) 5e+02) (.z (Transformation|GetActorLocation _asblock_spawn_2))))) (.y (Utilities|Select :Index _index :Option%200 (Math|Vector|MakeVector (+ (.x (Transformation|GetActorLocation _asblock_spawn_2)) 5e+02) (.y (Transformation|GetActorLocation _asblock_spawn_2)) (.z (Transformation|GetActorLocation _asblock_spawn_2))) :Option%201 (Math|Vector|MakeVector (.x (Transformation|GetActorLocation _asblock_spawn_2)) (+ (.y (Transformation|GetActorLocation _asblock_spawn_2)) 5e+02) (.z (Transformation|GetActorLocation _asblock_spawn_2))) :Option%202 (Math|Vector|MakeVector (- (.x (Transformation|GetActorLocation _asblock_spawn_2)) 5e+02) (.y (Transformation|GetActorLocation _asblock_spawn_2)) (.z (Transformation|GetActorLocation _asblock_spawn_2))) :Option%203 (Math|Vector|MakeVector (.x (Transformation|GetActorLocation _asblock_spawn_2)) (- (.y (Transformation|GetActorLocation _asblock_spawn_2)) 5e+02) (.z (Transformation|GetActorLocation _asblock_spawn_2))))) (- (.z (Utilities|Select :Index _index :Option%200 (Math|Vector|MakeVector (+ (.x (Transformation|GetActorLocation _asblock_spawn_2)) 5e+02) (.y (Transformation|GetActorLocation _asblock_spawn_2)) (.z (Transformation|GetActorLocation _asblock_spawn_2))) :Option%201 (Math|Vector|MakeVector (.x (Transformation|GetActorLocation _asblock_spawn_2)) (+ (.y (Transformation|GetActorLocation _asblock_spawn_2)) 5e+02) (.z (Transformation|GetActorLocation _asblock_spawn_2))) :Option%202 (Math|Vector|MakeVector (- (.x (Transformation|GetActorLocation _asblock_spawn_2)) 5e+02) (.y (Transformation|GetActorLocation _asblock_spawn_2)) (.z (Transformation|GetActorLocation _asblock_spawn_2))) :Option%203 (Math|Vector|MakeVector (.x (Transformation|GetActorLocation _asblock_spawn_2)) (- (.y (Transformation|GetActorLocation _asblock_spawn_2)) 5e+02) (.z (Transformation|GetActorLocation _asblock_spawn_2))))) 1e+03)) (Variables|Default|GetObject%20Types) false 0 "None"))
            (bind _asblock_spawn_3 (Utilities|Casting|CastToBlockSpawn (.HitActor (Collision|BreakHitResult _outhit))))
            (Utilities|Array|AddUnique (Variables|Default|GetDetectedBlocks) _asblock_spawn_3)
            (bind _returnvalue_2 (Utilities|Array|Add (Variables|Default|GetDirections) (Math|Vector|MakeVector (.x (Utilities|Select :Index _index :Option%200 (Math|Vector|MakeVector (+ (.x (Transformation|GetActorLocation _asblock_spawn_2)) 5e+02) (.y (Transformation|GetActorLocation _asblock_spawn_2)) (.z (Transformation|GetActorLocation _asblock_spawn_2))) :Option%201 (Math|Vector|MakeVector (.x (Transformation|GetActorLocation _asblock_spawn_2)) (+ (.y (Transformation|GetActorLocation _asblock_spawn_2)) 5e+02) (.z (Transformation|GetActorLocation _asblock_spawn_2))) :Option%202 (Math|Vector|MakeVector (- (.x (Transformation|GetActorLocation _asblock_spawn_2)) 5e+02) (.y (Transformation|GetActorLocation _asblock_spawn_2)) (.z (Transformation|GetActorLocation _asblock_spawn_2))) :Option%203 (Math|Vector|MakeVector (.x (Transformation|GetActorLocation _asblock_spawn_2)) (- (.y (Transformation|GetActorLocation _asblock_spawn_2)) 5e+02) (.z (Transformation|GetActorLocation _asblock_spawn_2))))) (.y (Utilities|Select :Index _index :Option%200 (Math|Vector|MakeVector (+ (.x (Transformation|GetActorLocation _asblock_spawn_2)) 5e+02) (.y (Transformation|GetActorLocation _asblock_spawn_2)) (.z (Transformation|GetActorLocation _asblock_spawn_2))) :Option%201 (Math|Vector|MakeVector (.x (Transformation|GetActorLocation _asblock_spawn_2)) (+ (.y (Transformation|GetActorLocation _asblock_spawn_2)) 5e+02) (.z (Transformation|GetActorLocation _asblock_spawn_2))) :Option%202 (Math|Vector|MakeVector (- (.x (Transformation|GetActorLocation _asblock_spawn_2)) 5e+02) (.y (Transformation|GetActorLocation _asblock_spawn_2)) (.z (Transformation|GetActorLocation _asblock_spawn_2))) :Option%203 (Math|Vector|MakeVector (.x (Transformation|GetActorLocation _asblock_spawn_2)) (- (.y (Transformation|GetActorLocation _asblock_spawn_2)) 5e+02) (.z (Transformation|GetActorLocation _asblock_spawn_2))))) (.z (Utilities|Select :Index _index :Option%200 (Math|Vector|MakeVector (+ (.x (Transformation|GetActorLocation _asblock_spawn_2)) 5e+02) (.y (Transformation|GetActorLocation _asblock_spawn_2)) (.z (Transformation|GetActorLocation _asblock_spawn_2))) :Option%201 (Math|Vector|MakeVector (.x (Transformation|GetActorLocation _asblock_spawn_2)) (+ (.y (Transformation|GetActorLocation _asblock_spawn_2)) 5e+02) (.z (Transformation|GetActorLocation _asblock_spawn_2))) :Option%202 (Math|Vector|MakeVector (- (.x (Transformation|GetActorLocation _asblock_spawn_2)) 5e+02) (.y (Transformation|GetActorLocation _asblock_spawn_2)) (.z (Transformation|GetActorLocation _asblock_spawn_2))) :Option%203 (Math|Vector|MakeVector (.x (Transformation|GetActorLocation _asblock_spawn_2)) (- (.y (Transformation|GetActorLocation _asblock_spawn_2)) 5e+02) (.z (Transformation|GetActorLocation _asblock_spawn_2)))))))))
          (Utilities|FlowControl|Sequence
            (:then_0
              ;[1 1 1] Add direction to total
              (for _array_element_4 (Variables|Default|GetDirections)
                (Utilities|Array|AddUnique (Variables|Default|GetNextToWall) _array_element_4)
                (Utilities|Array|Clear (Variables|Default|GetDirections))))
            (:then_1
              ;[1 1 1] Generate more walls
              (if (Math|Boolean|ANDBoolean (< (Math|Random|RandomIntegerinRange 1 8) 3) (Utilities|Array|ContainsItem (Variables|Default|GetNextToWall) (Transformation|GetActorLocation _asblock_spawn_2)) (Variables|/Game/Blueprints/Generation/BlockSpawn.BlockSpawn_C|GetWasEmpty _asblock_spawn_2))
                (Default|AddSolid _asblock_spawn_2)))
            (:then_2
              ;[1 1 1] Add Missing Cubes
              (if (and (> _returnvalue_2 1) (Variables|/Game/Blueprints/Generation/BlockSpawn.BlockSpawn_C|GetWasEmpty _asblock_spawn_2))
                (Default|AddSolid _asblock_spawn_2)))))
        (Utilities|FlowControl|Sequence
          (:then_0
            ;[1 1 1] AntiSoftLock Mechanism
            (for _array_element_5 (Variables|Default|GetWalls)
              (if (Utilities|Array|ContainsItem (Variables|Default|GetDetectedBlocks) _array_element_5)
                (Variables|Default|SetDetectedWall _array_element_5)
                (bind _output_get (Variables|Default|SetDetectedWallAmount (+ (Variables|Default|GetDetectedWallAmount) 1)))
                (if (> _output_get 1)
                  (Utilities|FlowControl|Sequence
                    (:then_0
                      (for _array_element_6 _array
                        (bind _asblock_spawn_4 (Utilities|Casting|CastToBlockSpawn (Variables|/Script/Engine.ChildActorComponent|GetChildActor _array_element_6)))
                        (Default|EmptyBlock _asblock_spawn_4)))
                    (:then_1
                      (for _array_element_7 _array_2
                        (bind _asblock_spawn_5 (Utilities|Casting|CastToBlockSpawn (Variables|/Script/Engine.ChildActorComponent|GetChildActor _array_element_7)))
                        (Default|EmptyBlock _asblock_spawn_5)))
                    (:then_2
                      (for _array_element_8 (Utilities|Array|MakeArray (Variables|Default|Get20) (Variables|Default|Get21) (Variables|Default|Get22) (Variables|Default|Get23) (Variables|Default|Get24))
                        (bind _asblock_spawn_6 (Utilities|Casting|CastToBlockSpawn (Variables|/Script/Engine.ChildActorComponent|GetChildActor _array_element_8)))
                        (Default|EmptyBlock _asblock_spawn_6)))
                    (:then_3
                      (for _array_element_9 (Utilities|Array|MakeArray (Variables|Default|Get4) (Variables|Default|Get9) (Variables|Default|Get14) (Variables|Default|Get19) (Variables|Default|Get24))
                        (bind _asblock_spawn_7 (Utilities|Casting|CastToBlockSpawn (Variables|/Script/Engine.ChildActorComponent|GetChildActor _array_element_9)))
                        (Default|EmptyBlock _asblock_spawn_7)))))))
            (if (== _output_get 1)
              ;[1 1 1] Cut Paths in Blocks
              (Variables|Default|SetRandom0-5 (Math|Random|RandomIntegerinRange 0 4))
              (if (or (Components|ComponentHasTag (Variables|/Script/Engine.Actor|GetRootComponent (Variables|Default|GetDetectedWall)) "Wall2") (Components|ComponentHasTag (Variables|/Script/Engine.Actor|GetRootComponent (Variables|Default|GetDetectedWall)) "Wall1"))
                (for (_array_element_10 _array_index) _array
                  (if (== (Variables|Default|GetRandom0-5) _array_index)
                    (for _index_2 (range 0 4)
                      (bind _asblock_spawn_8 (Utilities|Casting|CastToBlockSpawn (Variables|/Script/Engine.ChildActorComponent|GetChildActor (Utilities|Array|Get(acopy) (Variables|Default|GetBlocks) (+ (Utilities|Array|FindItem (Variables|Default|GetBlocks) _array_element_10) (* _index_2 5))))))
                      (Default|EmptyBlock _asblock_spawn_8))))
                (else
                  (for (_array_element_11 _array_index_2) _array_2
                    (if (== (Variables|Default|GetRandom0-5) _array_index_2)
                      (for _index_3 (range 0 4)
                        (bind _asblock_spawn_9 (Utilities|Casting|CastToBlockSpawn (Variables|/Script/Engine.ChildActorComponent|GetChildActor (Utilities|Array|Get(acopy) (Variables|Default|GetBlocks) (+ (Utilities|Array|FindItem (Variables|Default|GetBlocks) _array_element_11) _index_3)))))
                        (Default|EmptyBlock _asblock_spawn_9))))))))
          (:then_1
            (Default|GlobalScan (.AsBP%20Doh%20Mans%20Land%20Game%20Mode (Utilities|Casting|CastToBP_DohMansLand_GameMode (Game|GetGameMode))))))
        (else
          (for _array_element_12 (Variables|Default|GetBlocks)
            (bind _asblock_spawn_10 (Utilities|Casting|CastToBlockSpawn (Variables|/Script/Engine.ChildActorComponent|GetChildActor _array_element_12)))
            (Default|EmptyBlock _asblock_spawn_10)))))))

(event Collision|EventActorBeginOverlap
  (params (OtherActor :type Actor%20Object%20Reference)))

(event EventTick
  (params (DeltaSeconds :type Float%20%28single-precision%29)))

(fn ConstructionScript)