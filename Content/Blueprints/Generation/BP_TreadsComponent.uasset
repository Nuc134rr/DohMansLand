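; Tank component that leaves tread marks in the tank's color on BP_FloorWithTreads floors as the tank moves.
; UpdateSpeeds enables one pair of four local spawn points based on forward or reverse motion, and none when forward speed is zero.
; Tick traces down from each active point after enough 2D travel.
; Hits queue the collision UV, yaw and color in the floor's NewTreads array.
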(event Custom|UpdateSpeeds
  (params (NewLeftRight :type Float%20%28double-precision%29) (NewForward :type Float%20%28double-precision%29))
  (bind _spawntreads (Variables|Default|GetSpawnTreads))
  (bind _spawntreads_2 (Variables|Default|GetSpawnTreads))
  (Variables|Default|SetLeftRightSpeed NewLeftRight)
  (bind _output_get (Variables|Default|SetForwardSpeed NewForward))
  (if (> _output_get 0.0)
    (Utilities|SetTwoArrayElements false _spawntreads 0 1
      (:%20%20
        (Utilities|SetTwoArrayElements true _spawntreads 2 3)))
    (elif (< (Variables|Default|GetForwardSpeed) 0.0)
      (Utilities|SetTwoArrayElements true _spawntreads_2 0 1
        (:%20%20
          (Utilities|SetTwoArrayElements false _spawntreads_2 2 3)))
      (else
        (Utilities|SetTwoArrayElements false _spawntreads_2 0 1
          (:%20%20
            (Utilities|SetTwoArrayElements false _spawntreads_2 2 3)))))))

(event EventBeginPlay
  (Variables|Default|SetOwner (Components|GetOwner))
  (Utilities|ResetPoint
    (:%20%20
      (Utilities|ResetPoint 1
        (:%20%20
          (Utilities|ResetPoint 2
            (:%20%20
              (Utilities|ResetPoint 3
                (:%20%20
                  (bind _asbp_base_tank (Utilities|Casting|CastToBP_BaseTank (Components|GetOwner)))
                  (Variables|Default|SetColor (.tankcolor (Utilities|Array|Get(acopy) (Variables|/Game/Blueprints/Player/BP_DohMansLand_GameMode.BP_DohMansLand_GameMode_C|GetTank%20Variables (CallFunction|GetDohMansLandGameMode)) (Variables|/Game/Blueprints/Player/BP_BaseTank.BP_BaseTank_C|GetPlayerID _asbp_base_tank)))))))))))))

(event EventTick
  (params (DeltaSeconds :type Float%20%28single-precision%29))
  (for (_array_element _array_index) (Variables|Default|GetSpawnTreads)
    (if _array_element
      (if (> (Math|Vector|Distance2D(Vector) (Math|Vector2D|MakeVector2D (.x (Math|Transform|TransformLocation (Transformation|GetActorTransform (Variables|Default|GetOwner)) (Utilities|Array|Get(acopy) (Variables|Default|GetSpawnPoints) _array_index))) (.y (Math|Transform|TransformLocation (Transformation|GetActorTransform (Variables|Default|GetOwner)) (Utilities|Array|Get(acopy) (Variables|Default|GetSpawnPoints) _array_index)))) (Math|Vector2D|MakeVector2D (.x (Utilities|Array|Get(acopy) (Variables|Default|GetLast%20Points) _array_index)) (.y (Utilities|Array|Get(acopy) (Variables|Default|GetLast%20Points) _array_index)))) (Variables|Default|GetTread%20Spawn%20Distance))
        (Utilities|ResetPoint _array_index
          (:%20%20
            (Utilities|TraceandSet _array_index)))))))