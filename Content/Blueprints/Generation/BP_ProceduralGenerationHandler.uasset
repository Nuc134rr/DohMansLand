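; Procedural generation handler that, when enabled, spawns a grid of wall blocks from a bottom-left corner on BeginPlay.
; Grid spacing comes from the mesh bounds of a temporarily spawned first map class plus BlockSpacing.
; Each cell picks randomly among WallClassMap classes whose weight exceeds a random roll up to the weight total.
; SpawnSingularBlock lets BP_BaseWall request extra blocks; the asset-count limit passed to SpawnBlocks is unused.
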(event Custom|SpawnBlocks
  (params (MaxNumberOfAssets :type Integer))
  (bind _bottomleftcorner (Variables|Default|GetBottomLeftCorner))
  (bind _blocksize (Variables|Grid|GetBlockSize))
  ;[0.2 0.2 0.2] Spawn a grid of X rows and Y columns of walls, where the class is decided through the map
  (for _index (range 0 (- (Variables|Grid|GetNumberOfRows) 1))
    (Variables|Grid|SetCurrentRow _index)
    (for _index_2 (range 0 (- (Variables|Grid|GetNumberOfColumns) 1))
      (Variables|Grid|SetCurrentColumn _index_2)
      (bind _percentagesum (CallFunction|GetPercentageSum))
      (bind _classtospawn (CallFunction|PickWallMesh _percentagesum))
      (Game|SpawnActorfromClass _classtospawn (Math|Transform|MakeTransform (Math|Vector|MakeVector (+ (* (Variables|Grid|GetCurrentRow) _blocksize) (.x _bottomleftcorner)) (+ (* _blocksize (Variables|Grid|GetCurrentColumn)) (.y _bottomleftcorner)) 0.0) "0, 0, 0" "1.000000,1.000000,1.000000") "Undefined" self false 0)))
  (Math|Integer|IncrementInt (Variables|Default|GetSpawnIndex)))

(event Custom|SetBlockSize
  ;[0.2 0.2 0.2] Sets the size of each block within the map
  (bind _keys (Utilities|Map|Keys (Variables|Maps|GetWallClassMap)))
  (bind _returnvalue (Game|SpawnActorfromClass (Utilities|Array|Get(acopy) _keys) (Math|Transform|MakeTransform "0, 0, 0" "0, 0, 0" "1.000000,1.000000,1.000000") "Undefined" 0 false 0))
  (Utilities|IsValid _returnvalue
    (:Is%20Valid
      (Variables|Grid|SetBlockSize (+ (* (.x (.boxextent (StaticMesh|GetBounds (Variables|/Script/Engine.StaticMeshComponent|GetStaticMesh (Variables|/Game/Blueprints/Generation/WallClasses/BP_BaseWall.BP_BaseWall_C|GetMesh _returnvalue))))) 2.0) (Variables|Grid|GetBlockSpacing)))
      (Actor|DestroyActor _returnvalue))))

(event Custom|SpawnSingularBlock
  (params (BlockClass :type BP%20Base%20Wall%20Class%20Reference) (SpawnTransform :type Transform))
  ;[0.2 0.2 0.2] Spawns a singluar block (called from BP_BaseWall)
  (Game|SpawnActorfromClass BlockClass SpawnTransform "Undefined" self true 0))

(event Collision|EventActorBeginOverlap
  (params (OtherActor :type Actor%20Object%20Reference)))

(event EventTick
  (params (DeltaSeconds :type Float%20%28single-precision%29)))

(event EventBeginPlay
  ;[0.2 0.2 0.2] Call events
  (if (Variables|Default|GetbEnableGeneration)
    (Utilities|FlowControl|Sequence
      (:then_0
        (CallFunction|SetBlockSize))
      (:then_1
        (CallFunction|SpawnBlocks (Utilities|Select :Index (Variables|Default|GetSpawnIndex) :Option%200 (Variables|MaxAssetNumbers|GetMaxLargeAssets) :Option%201 (Variables|MaxAssetNumbers|GetMaxMediumAssets) :Option%202 (Variables|MaxAssetNumbers|GetMaxSmallAssets)))))))

(fn ConstructionScript)

(fn GetPercentageSum
  (bind _values (Utilities|Map|Values (Variables|Maps|GetWallClassMap)))
  (for _array_element _values
    (LocalVariables|SetTotalSum (+ _array_element (LocalVariables|GetTotalSum))))
  (return (LocalVariables|GetTotalSum)))

(fn PickWallMesh
  (params (PercentageSum :type Float%20%28double-precision%29))
  (LocalVariables|SetRandomFloat (Math|Random|RandomFloatinRange 0.0 PercentageSum))
  (bind _keys (Utilities|Map|Keys (Variables|Maps|GetWallClassMap)))
  (for _array_element _keys
    (if (> (.Value (Utilities|Map|Find (Variables|Maps|GetWallClassMap) _array_element)) (LocalVariables|GetRandomFloat))
      (Utilities|Array|Add (LocalVariables|GetPossibleMeshes) _array_element)))
  (return (.OutItem (Utilities|Array|Random (LocalVariables|GetPossibleMeshes)))))