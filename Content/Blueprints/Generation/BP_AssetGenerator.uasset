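; Level generator actor that spawns large, medium and small assets on BeginPlay, using separate wall and asset classes up to per-size limits.
; Each spawn takes its transform from RandomTransformInNavMesh, whose random navmesh-point and yaw nodes are marked unused.
; An overlap pass in Test, meant to reposition walls or destroy them after limited retries, is disconnected and never runs.
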(event Custom|GenerateAssets
  (for _index (range 0 2)
    (switch int _index
      (:0
        (for _index_2 (range 0 (Variables|NumberOfAssets|GetMaxLargeAssets))
          (Game|SpawnActorfromClass "/Game/Blueprints/Generation/WallClasses/BP_LargeAsset.BP_LargeAsset_C" (Utilities|RandomTransforminNavMesh) "Undefined" self false _index_2 0)))
      (:1
        (for _index_3 (range 0 (Variables|NumberOfAssets|GetMaxMediumAssets))
          (Game|SpawnActorfromClass "/Game/Blueprints/Generation/WallClasses/BP_1x2Wall.BP_1x2Wall_C" (Utilities|RandomTransforminNavMesh) "Undefined" self false _index_3 0)))
      (:2
        (for _index_4 (range 0 (Variables|NumberOfAssets|GetMaxSmallAssets))
          (Game|SpawnActorfromClass "/Game/Blueprints/Generation/WallClasses/BP_DefaultWall.BP_DefaultWall_C" (Utilities|RandomTransforminNavMesh) "Undefined" self false _index_4 0))))))

(event EventBeginPlay
  (CallFunction|GenerateAssets))

(fn ConstructionScript)

(fn Test
  (params (Input :type BP%20Base%20Wall%20Object%20Reference)))

(fn UpdateLocation
  (params (Input :type BP%20Base%20Wall%20Object%20Reference))
  (Transformation|SetActorTransform Input (Utilities|RandomTransforminNavMesh) true true))