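; Airdrop actor whose physics-driven AirDrop component tumbles randomly during play.
; On BeginPlay, Spawned starts a looping sub-second timer that calls Impulse, applying a small random angular velocity kick on all three axes.
; A sequence that would spawn a BP_Powerup at the actor's transform after a delay and then destroy the actor is unconnected, so it never runs.
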(event Custom|Spawned
  (Utilities|Time|SetTimerbyFunctionName 0 "Impulse" 0.6 true))

(event EventBeginPlay
  (CallFunction|Spawned))

(fn ConstructionScript)

(fn Impulse
  (bind _returnvalue (Math|Random|RandomFloatinRange -15.0 15.0))
  (Class|PrimitiveComponent|AddAngularImpulseinDegrees (Variables|Default|GetAirDrop) (Math|Vector|MakeVector _returnvalue _returnvalue _returnvalue) "None" true))