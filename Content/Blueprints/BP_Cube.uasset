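; BP_Cube is a cube actor that gets a randomized dough-style look from the M_Doh material; its event graph is empty.
; The Construction Script creates a dynamic material instance on the Cube and sets a random seed.
; It randomly picks one or two colors, drawing each independently from the same seven-color palette, so both can match.
; Because randomization runs at construction, the look re-rolls whenever the script reruns.
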(event EventBeginPlay)

(event Collision|EventActorBeginOverlap
  (params (OtherActor :type Actor%20Object%20Reference)))

(event EventTick
  (params (DeltaSeconds :type Float%20%28single-precision%29)))

(fn ConstructionScript
  (bind _returnvalue (Rendering|Material|CreateDynamicMaterialInstance (Variables|Default|GetCube) 0 "/Game/Assets/Materials/M_Doh.M_Doh" "None" :!class /Script/Engine.PrimitiveComponent))
  ;[1 1 1] Random Seed
  (Rendering|Material|SetScalarParameterValue _returnvalue "RandomSeed" (Math|Random|RandomFloatinRange 0.0 1e+03) :!class /Script/Engine.MaterialInstanceDynamic)
  ;[1 1 1] Number of Doh Colors
  (switch int (Math|Random|RandomInteger 2)
    (:0
      ;[1 1 1] Random Color0 Assignment
      (Rendering|Material|SetScalarParameterValue _returnvalue "NumberOfColors" 1.0 :!class /Script/Engine.MaterialInstanceDynamic :!label _label)
      (switch int (Math|Random|RandomInteger 7)
        (:0
          (Rendering|Material|SetVectorParameterValue _returnvalue "Color0" "(R=0.973445,G=0.042311,B=0.038204,A=1.000000)" :!class /Script/Engine.MaterialInstanceDynamic))
        (:1
          (Rendering|Material|SetVectorParameterValue _returnvalue "Color0" "(R=0.830770,G=0.291771,B=0.000000,A=1.000000)" :!class /Script/Engine.MaterialInstanceDynamic))
        (:2
          (Rendering|Material|SetVectorParameterValue _returnvalue "Color0" "(R=0.701102,G=0.658375,B=0.019382,A=1.000000)" :!class /Script/Engine.MaterialInstanceDynamic))
        (:3
          (Rendering|Material|SetVectorParameterValue _returnvalue "Color0" "(R=0.318547,G=0.665387,B=0.309469,A=1.000000)" :!class /Script/Engine.MaterialInstanceDynamic))
        (:4
          (Rendering|Material|SetVectorParameterValue _returnvalue "Color0" "(R=0.000911,G=0.035601,B=0.514918,A=1.000000)" :!class /Script/Engine.MaterialInstanceDynamic))
        (:5
          (Rendering|Material|SetVectorParameterValue _returnvalue "Color0" "(R=0.346704,G=0.029557,B=0.341914,A=1.000000)" :!class /Script/Engine.MaterialInstanceDynamic))
        (:6
          (Rendering|Material|SetVectorParameterValue _returnvalue "Color0" "(R=0.693872,G=0.693872,B=0.768151,A=1.000000)" :!class /Script/Engine.MaterialInstanceDynamic))))
    (:1
      (Utilities|FlowControl|Sequence
        (:then_0
          (goto _label))
        (:then_1
          ;[1 1 1] Random Color1 Assignment
          (Rendering|Material|SetScalarParameterValue _returnvalue "NumberOfColors" 2.0 :!class /Script/Engine.MaterialInstanceDynamic)
          (switch int (Math|Random|RandomInteger 7)
            (:0
              (Rendering|Material|SetVectorParameterValue _returnvalue "Color1" "(R=0.972549,G=0.043137,B=0.039216,A=1.000000)" :!class /Script/Engine.MaterialInstanceDynamic))
            (:1
              (Rendering|Material|SetVectorParameterValue _returnvalue "Color1" "(R=0.830770,G=0.291771,B=0.000000,A=1.000000)" :!class /Script/Engine.MaterialInstanceDynamic))
            (:2
              (Rendering|Material|SetVectorParameterValue _returnvalue "Color1" "(R=0.701102,G=0.658375,B=0.019382,A=1.000000)" :!class /Script/Engine.MaterialInstanceDynamic))
            (:3
              (Rendering|Material|SetVectorParameterValue _returnvalue "Color1" "(R=0.318547,G=0.665387,B=0.309469,A=1.000000)" :!class /Script/Engine.MaterialInstanceDynamic))
            (:4
              (Rendering|Material|SetVectorParameterValue _returnvalue "Color1" "(R=0.000911,G=0.035601,B=0.514918,A=1.000000)" :!class /Script/Engine.MaterialInstanceDynamic))
            (:5
              (Rendering|Material|SetVectorParameterValue _returnvalue "Color1" "(R=0.346704,G=0.029557,B=0.341914,A=1.000000)" :!class /Script/Engine.MaterialInstanceDynamic))
            (:6
              (Rendering|Material|SetVectorParameterValue _returnvalue "Color1" "(R=0.693872,G=0.693872,B=0.768151,A=1.000000)" :!class /Script/Engine.MaterialInstanceDynamic))))))))