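; BP_AirdropButton is a touchable button that spawns BP_Airdrop actors and then recharges.
; Reset, run on BeginPlay and after each use, steps the cylinder's material from red through yellow to green over AirdropTimerTimeDelay, then sets Ready.
; Touching the cylinder when Ready spawns NumOfPowerups airdrops at a fixed height, taking X and Y from separate random navigable-point queries around Origin.
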(event OnInputTouchBegin(Cylinder)
  (params (FingerIndex :type ETouchIndex%20Enum :default "Touch1") (TouchedComponent :type Primitive%20Component%20Object%20Reference))
  (bind _origin (Variables|Default|GetOrigin))
  (bind _nav_data (Variables|Default|GetNav%20Data))
  (bind _randomlocation (Class|NavigationSystemV1|GetRandomPointinNavigableRadius _origin 5e+03 _nav_data 0))
  ;[1 1 1] Spawning Airdrop
  (if (Variables|Default|Getready)
    (for _index (range 0 (- (Variables|Default|GetNumOfPowerups) 1))
      (Game|SpawnActorfromClass "/Game/Blueprints/BP_Airdrop.BP_Airdrop_C" (Math|Transform|MakeTransform (Math|Vector|MakeVector (.x _randomlocation) (.y _randomlocation) 2e+03) "0, 0, 0" "3.000000,3.000000,3.000000") "Undefined" 0 0))
    (Variables|Default|Setready false)
    (CallFunction|Reset)))

(event Custom|Reset
  (bind _cylinder (Variables|Default|GetCylinder))
  ;[1 1 1] Color Stuff
  (Rendering|Material|SetMaterial _cylinder 0 "/Game/Assets/Materials/M_RedButton.M_RedButton")
  (Utilities|FlowControl|Delay (/ (Variables|Default|GetAirdropTimerTimeDelay) 2.0))
  (Rendering|Material|SetMaterial _cylinder 0 "/Game/Assets/Materials/M_YellowButton.M_YellowButton")
  (Utilities|FlowControl|Delay (/ (Variables|Default|GetAirdropTimerTimeDelay) 2.0))
  (Rendering|Material|SetMaterial (Variables|Default|GetCylinder) 0 "/Game/Assets/Materials/M_GreenButton.M_GreenButton")
  (Variables|Default|Setready true))

(event EventBeginPlay
  ;[1 1 1] Color Stuff
  (CallFunction|Reset))

(fn ConstructionScript)