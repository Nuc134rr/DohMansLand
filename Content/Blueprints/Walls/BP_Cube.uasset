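; BP_Cube is a breakable wall cube that projectiles destroy on overlapping its Box component.
; A big projectile destroys it immediately, while other BP_BaseProjectile types increment a hit counter and are removed on impact.
; When the counter reaches MaxHits, the cube destroys itself after a very short delay.
; The construction script applies random colors to its static mesh, and the Hit event is empty.
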(event OnComponentBeginOverlap(Box)
  (params (OverlappedComponent :type Primitive%20Component%20Object%20Reference) (OtherActor :type Actor%20Object%20Reference) (OtherComp :type Primitive%20Component%20Object%20Reference) (OtherBodyIndex :type Integer) (bFromSweep :type Boolean) (SweepResult :type Hit%20Result%20Structure%20%28by%20ref%29))
  ;[0.2 0.2 0.2] the wall will break from 3 normal projectile hits/1 big projectile hit
  (bind _asbp_base_projectile (Utilities|Casting|CastToBP_BaseProjectileClass (Utilities|GetClass OtherActor)))
  (Utilities|Casting|CastToBP_BigProjectileClass _asbp_base_projectile
    (:then
      (Actor|DestroyActor))
    (:CastFailed
      (bind _result (Math|Integer|IncrementInt (Variables|Default|GetCurrentHits))
        (:%20%20
          (if (== _result (Variables|Default|GetMaxHits))
            (Utilities|FlowControl|Delay 0.01)
            (Actor|DestroyActor))
          (Default|RemoveandDestroy (.AsBP%20Base%20Projectile (Utilities|Casting|CastToBP_BaseProjectile OtherActor))))))))

(event Collision|EventHit
  (params (MyComp :type Primitive%20Component%20Object%20Reference) (Other :type Actor%20Object%20Reference) (OtherComp :type Primitive%20Component%20Object%20Reference) (bSelfMoved :type Boolean) (HitLocation :type Vector :default "0, 0, 0") (HitNormal :type Vector :default "0, 0, 0") (NormalImpulse :type Vector :default "0, 0, 0") (Hit :type Hit%20Result%20Structure%20%28by%20ref%29))
  ;[0.2 0.2 0.2] long node lol
)

(fn ConstructionScript
  (CallFunction|SetRandomColors (Variables|Default|GetStaticMesh)))