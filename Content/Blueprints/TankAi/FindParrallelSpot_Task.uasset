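; Behavior tree task for the AI tank that picks a position in line with its Target along a world axis and writes it to TargetPosition.
; It takes the tank-minus-target offset and compares its signed X and Y, without absolute values.
; If X is smaller, the spot uses the tank's X with the target's Y and Z.
; Otherwise it shifts the target's Y by the offset's Z, not its Y, then always finishes successfully.
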(event EventReceiveExecute
  (params (OwnerActor :type Actor%20Object%20Reference))
  (bind _returnvalue (AI|GetBlackboard OwnerActor))
  (bind _returnvalue_2 (Utilities|Name|MakeLiteralName "Target"))
  (bind _returnvalue_3 (Utilities|Name|MakeLiteralName "SelfActor"))
  (bind _returnvalue_4 (AI|Components|Blackboard|GetValueasObject _returnvalue _returnvalue_2))
  (bind _returnvalue_5 (AI|Components|Blackboard|GetValueasObject _returnvalue _returnvalue_3))
  (bind _asbp_ai_tank (Utilities|Casting|CastToBP_AiTank _returnvalue_5))
  (bind _asactor (Utilities|Casting|CastToActor _returnvalue_4))
  (bind _returnvalue_6 (Transformation|GetActorLocation _asactor))
  (bind _returnvalue_7 (Transformation|GetActorLocation _asbp_ai_tank))
  (bind (_x _y _z) (Math|Vector|BreakVector _returnvalue_6))
  (bind _returnvalue_8 (- _returnvalue_7 _returnvalue_6))
  (AI|Components|Blackboard|SetValueasVector _returnvalue (Utilities|Name|MakeLiteralName "TargetPosition") (select (< (.x _returnvalue_8) (.y _returnvalue_8)) (Math|Vector|MakeVector (+ (.x _returnvalue_8) _x) _y _z) (Math|Vector|MakeVector _x (+ _y (.z _returnvalue_8)) _z)))
  (AI|BehaviorTree|FinishExecute true))