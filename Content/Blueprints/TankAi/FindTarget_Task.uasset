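; Behavior tree task for tank AI that picks the nearest BP_BaseTank as the blackboard Target.
; On execute it loops over all BP_BaseTank actors, comparing squared distances to the SelfActor BP_AiTank against LowestNumber to track the closest index.
; The graph applies no self or team filter and never resets LowestNumber or LowestIndex before the loop.
; It writes the selected actor to Target and finishes successfully.
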(event EventReceiveExecute
  (params (OwnerActor :type Actor%20Object%20Reference))
  (bind _returnvalue (AI|GetBlackboard OwnerActor))
  (bind _outactors (Actor|GetAllActorsOfClass "/Game/Blueprints/Player/BP_BaseTank.BP_BaseTank_C"))
  (for (_array_element _array_index) _outactors
    (if (< (Class|KismetMathLibrary|VectorDistanceSquared (Transformation|GetActorLocation _array_element) (Transformation|GetActorLocation (.AsBP%20Ai%20Tank (Utilities|Casting|CastToBP_AiTank (AI|Components|Blackboard|GetValueasObject _returnvalue (Utilities|Name|MakeLiteralName "SelfActor")))))) (Variables|Default|GetLowestNumber))
      (Variables|Default|SetLowestNumber (Class|KismetMathLibrary|VectorDistanceSquared (Transformation|GetActorLocation _array_element) (Transformation|GetActorLocation (.AsBP%20Ai%20Tank (Utilities|Casting|CastToBP_AiTank (AI|Components|Blackboard|GetValueasObject _returnvalue (Utilities|Name|MakeLiteralName "SelfActor")))))))
      (Variables|Default|SetLowestIndex _array_index)))
  (AI|Components|Blackboard|SetValueasObject _returnvalue (Utilities|Name|MakeLiteralName "Target") (Utilities|Array|Get(acopy) _outactors (Variables|Default|GetLowestIndex)))
  (AI|BehaviorTree|FinishExecute true))