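; AI-controlled tank that steers its body toward its velocity, aims its turret at sighted tanks and fires projectiles.
; Tick sets the FoundActor blackboard key from sight perception of BP_BaseTank actors.
; Fire spawns a projectile at the barrel, rate-limited by that projectile's FireRate; the projectile cap check is disconnected.
; Construction derives PlayerID from the BP_BaseTank count and tints body and turret with randomly seeded M_Doh dynamic materials.
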(event Custom|Fire
  (bind _barrel (Variables|Default|GetBarrel))
  ;[0.7982 0.2142 1] Projectile Logic
  ;;[0.2 0.2 0.2] Fire Projectile (LShift OR RShift) IF this tank has less than 3 projectiles already spawned
  (Utilities|FlowControl|DoOnce false :!label _label
    (:Completed
      (bind _returnvalue (Game|SpawnActorfromClass (Variables|Default|GetProjectileClass) (Math|Transform|MakeTransform (Transformation|GetWorldLocation _barrel) (Transformation|GetWorldRotation _barrel) "1.000000,1.000000,1.000000") "AdjustIfPossibleButAlwaysSpawn" 0 0 0))
      (Utilities|FlowControl|Delay (Variables|/Game/Projectiles/BP_BaseProjectile.BP_BaseProjectile_C|GetFireRate _returnvalue))
      (goto _label Reset))))

(event Custom|RemoveProjectile
  (params (ProjectileToRemove :type BP%20Base%20Projectile%20Object%20Reference))
  ;[0.7982 0.2142 1] Projectile Logic
  ;;[0.2 0.2 0.2] Remove Projectile from array when it dies
  (Utilities|Array|RemoveItem (Variables|Default|GetCurrentProjectiles) ProjectileToRemove))

(event EventTick
  (params (DeltaSeconds :type Float%20%28single-precision%29))
  (Transformation|SetActorRotation (Math|Interpolation|RInterpTo (Transformation|GetActorRotation) (Math|Conversions|RotationFromXVector (Transformation|GetVelocity)) (Utilities|Time|GetWorldDeltaSeconds) 1.0))
  (AI|Components|Blackboard|SetValueasBool (AI|GetBlackboard 0) (Utilities|Name|MakeLiteralName "FoundActor") false)
  (for _array_element (Class|AIPerceptionComponent|GetPerceivedActors (Variables|Default|GetAIPerception) "/Script/AIModule.AISense_Sight")
    (bind _asbp_base_tank (Utilities|Casting|CastToBP_BaseTank _array_element))
    (Transformation|SetWorldRotation (Variables|Default|GetTurret) (Math|Rotator|FindLookatRotation (Transformation|GetActorLocation) (Transformation|GetActorLocation _asbp_base_tank)) false false)
    (AI|Components|Blackboard|SetValueasBool (AI|GetBlackboard 0) (Utilities|Name|MakeLiteralName "FoundActor") true)))

(fn ConstructionScript
  (bind _playerid (CallFunction|SetPlayerID))
  (CallFunction|SetPlayerTankDoh (Variables|Character|GetMesh) _playerid)
  (CallFunction|SetPlayerTankDoh (Variables|Default|GetTurret) _playerid))

(fn SetPlayerTankDoh
  (params (InputPin :type Skeletal%20Mesh%20Component%20Object%20Reference) (PlayerID :type Integer))
  (bind _returnvalue (Rendering|Material|CreateDynamicMaterialInstance InputPin 0 "/Game/Assets/Materials/M_Doh.M_Doh" "None" :!class /Script/Engine.PrimitiveComponent))
  ;[1 1 1] Random Seed
  (Rendering|Material|SetScalarParameterValue _returnvalue "RandomSeed" (Math|Random|RandomFloatinRange 0.0 1e+03) :!class /Script/Engine.MaterialInstanceDynamic)
  ;[1 1 1] Random Color0 Assignment
  (Rendering|Material|SetScalarParameterValue _returnvalue "NumberOfColors" 1.0 :!class /Script/Engine.MaterialInstanceDynamic)
  (switch int PlayerID
    (:0
      (Rendering|Material|SetVectorParameterValue _returnvalue "Color0" "(R=0.973445,G=0.042311,B=0.038204,A=1.000000)" :!class /Script/Engine.MaterialInstanceDynamic))
    (:1
      (Rendering|Material|SetVectorParameterValue _returnvalue "Color0" "(R=0.000911,G=0.035601,B=0.514918,A=1.000000)" :!class /Script/Engine.MaterialInstanceDynamic))
    (:2
      (Rendering|Material|SetVectorParameterValue _returnvalue "Color0" "(R=0.000000,G=1.000000,B=0.000000,A=1.000000)" :!class /Script/Engine.MaterialInstanceDynamic))))

(fn SetPlayerID
  (bind _outactors (Actor|GetAllActorsOfClass "/Game/Blueprints/Player/BP_BaseTank.BP_BaseTank_C"))
  (bind _result (Math|Integer|DecrementInt (Utilities|Array|Length _outactors))
    (:%20%20
      (bind _output_get (Variables|Default|SetPlayerID _result))
      (return _output_get))))