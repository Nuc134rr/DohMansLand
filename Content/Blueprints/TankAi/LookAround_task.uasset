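; Behavior tree task that nudges an AI tank's turret in yaw, apparently to make it look around.
; On execute it gets the BP_TankAi pawn from Bp_AiController and takes one constant-speed interpolation step toward a yaw 45 degrees ahead.
; The completion check compares the current yaw to itself plus 45, so it never passes.
; The task therefore prints "fail" and never calls FinishExecute, as do failed casts.
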(event EventReceiveExecute
  (params (OwnerActor :type Actor%20Object%20Reference))
  (bind _asbp_ai_controller (Utilities|Casting|CastToBp_AiController OwnerActor)
    (:then
      (bind _asbp_tank_ai (Utilities|Casting|CastToBP_TankAi (Pawn|GetControlledPawn _asbp_ai_controller))
        (:then
          (Transformation|SetWorldRotation (Variables|/Game/Blueprints/TankAi/BP_TankAi.BP_TankAi_C|GetTurret _asbp_tank_ai) (Class|KismetMathLibrary|RInterptoConstant (Transformation|GetWorldRotation (Variables|/Game/Blueprints/TankAi/BP_TankAi.BP_TankAi_C|GetTurret _asbp_tank_ai)) (Math|Rotator|MakeRotator (.Roll (Math|Rotator|BreakRotator (Transformation|GetWorldRotation (Variables|/Game/Blueprints/TankAi/BP_TankAi.BP_TankAi_C|GetTurret _asbp_tank_ai)))) (.Pitch (Math|Rotator|BreakRotator (Transformation|GetWorldRotation (Variables|/Game/Blueprints/TankAi/BP_TankAi.BP_TankAi_C|GetTurret _asbp_tank_ai)))) (+ (.Yaw (Math|Rotator|BreakRotator (Transformation|GetWorldRotation (Variables|/Game/Blueprints/TankAi/BP_TankAi.BP_TankAi_C|GetTurret _asbp_tank_ai)))) 45.0)) (Utilities|Time|GetWorldDeltaSeconds) 3.0) false false)
          (if (> (.Yaw (Math|Rotator|BreakRotator (Transformation|GetWorldRotation (Variables|/Game/Blueprints/TankAi/BP_TankAi.BP_TankAi_C|GetTurret _asbp_tank_ai)))) (+ (.Yaw (Math|Rotator|BreakRotator (Transformation|GetWorldRotation (Variables|/Game/Blueprints/TankAi/BP_TankAi.BP_TankAi_C|GetTurret _asbp_tank_ai)))) 45.0))
            (AI|BehaviorTree|FinishExecute true)
            (else
              (Development|PrintString "fail" :!label _label))))
        (:CastFailed
          (goto _label))))
    (:CastFailed
      (goto _label))))