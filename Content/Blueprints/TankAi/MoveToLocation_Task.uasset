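; Behavior tree task for tank AI that sends the pawn toward the TargetPosition blackboard location.
; It starts an AI move, then applies one interpolated rotation step toward a look-at angle derived from LastLocation, with a 90-degree offset.
; It clears LastLocation and reports success right after the move starts, without waiting for arrival, or failure if the request fails.
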(event EventReceiveExecuteAI
  (params (OwnerController :type AI%20Controller%20Object%20Reference) (ControlledPawn :type Pawn%20Object%20Reference))
  (bind _returnvalue (Transformation|GetActorLocation ControlledPawn))
  (AI|AIMoveTo OwnerController (AI|Components|Blackboard|GetValueasVector (AI|GetBlackboard ControlledPawn) (Utilities|Name|MakeLiteralName "TargetPosition")) 0 -1.0 "Default" "Default" true true
    (:then
      (Transformation|SetActorRotation ControlledPawn (Math|Interpolation|RInterpTo (Transformation|GetActorRotation ControlledPawn) (Math|Rotator|CombineRotators (Math|Rotator|FindLookatRotation _returnvalue (- (Variables|Default|GetLastLocation) _returnvalue)) "0,-90.000000, 0") (Utilities|Time|GetWorldDeltaSeconds) 1e+01))
      (Variables|Default|SetLastLocation "0, 0, 0")
      (AI|BehaviorTree|FinishExecute true))
    (:OnRequestFailed
      (AI|BehaviorTree|FinishExecute false))))