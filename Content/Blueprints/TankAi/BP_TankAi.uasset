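; AI-controlled tank that turns its body toward its velocity, aims its turret at sighted tanks and can fire projectiles from the barrel.
; Each Tick scans sight perception and points the turret at any BP_BaseTank, setting the blackboard FoundActor flag.
; The loop's completion also clears that flag, so it ends every Tick false.
; A Fire event spawns the projectile; leftover manual movement nodes are disconnected.
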(event Custom|Fire
  (bind _barrel (Variables|Default|GetBarrel))
  ;[0.2 0.2 0.2] Shoot (LShift)
  (Game|SpawnActorfromClass (Variables|Default|GetProjectileClass) (Math|Transform|MakeTransform (Transformation|GetWorldLocation _barrel) (Transformation|GetWorldRotation _barrel) "1.000000,1.000000,1.000000") "Undefined" self 0 0))

(event EventTick
  (params (DeltaSeconds :type Float%20%28single-precision%29))
  (Transformation|SetActorRotation (Math|Interpolation|RInterpTo (Transformation|GetActorRotation) (Math|Conversions|RotationFromXVector (Transformation|GetVelocity)) (Utilities|Time|GetWorldDeltaSeconds) 1.0))
  (for _array_element (Class|AIPerceptionComponent|GetPerceivedActors (Variables|Default|GetAIPerception) "/Script/AIModule.AISense_Sight")
    (bind _asbp_base_tank (Utilities|Casting|CastToBP_BaseTank _array_element)
      (:then
        ;[0.145 0.6838 1] Movement/Rotation
        ;;[0.2 0.2 0.2] Rotate the Turret of the tank (Q and E)
        (Transformation|SetWorldRotation (Variables|Default|GetTurret) (Math|Rotator|FindLookatRotation (Transformation|GetActorLocation) (Transformation|GetActorLocation _asbp_base_tank)) false false)
        (AI|Components|Blackboard|SetValueasBool (AI|GetBlackboard 0) (Utilities|Name|MakeLiteralName "FoundActor") true))
      (:CastFailed
        (AI|Components|Blackboard|SetValueasBool (AI|GetBlackboard 0) (Utilities|Name|MakeLiteralName "FoundActor") false))))
  (AI|Components|Blackboard|SetValueasBool (AI|GetBlackboard 0) (Utilities|Name|MakeLiteralName "FoundActor") false))

(fn ConstructionScript)