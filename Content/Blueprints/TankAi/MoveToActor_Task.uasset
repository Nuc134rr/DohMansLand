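; Behavior tree task for tank AI that moves the controlled pawn to the actor stored in the "Target" blackboard key.
; It starts AIMoveTo, then immediately applies a single interpolated rotation built from the pawn's own forward vector.
; The task finishes only when the move succeeds; a failed cast or failed move never calls FinishExecute.
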(event EventReceiveExecuteAI
  (params (OwnerController :type AI%20Controller%20Object%20Reference) (ControlledPawn :type Pawn%20Object%20Reference))
  (bind _returnvalue (Transformation|GetActorForwardVector ControlledPawn))
  (bind _asactor (Utilities|Casting|CastToActor (AI|Components|Blackboard|GetValueasObject (AI|GetBlackboard ControlledPawn) (Utilities|Name|MakeLiteralName "Target"))))
  (AI|AIMoveTo ControlledPawn "0, 0, 0" _asactor 5.0 false
    (:then
      (Transformation|SetActorRotation ControlledPawn (Math|Interpolation|RInterpTo (Transformation|GetActorRotation ControlledPawn) (Math|Rotator|MakeRotfromXY _returnvalue _returnvalue) 0.0 0.0)))
    (:OnSuccess
      (AI|BehaviorTree|FinishExecute true))))