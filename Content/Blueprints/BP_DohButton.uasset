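; Dough button that squishes when clicked, touched or triggered by the E key, a stand-in for touch input.
; The Squish timeline drives a randomly chosen one of three morph targets, re-rolled every update.
; On finish, or E release, Unsquish zeroes a random target each update rather than easing it.
; Construction calls SetRandomColors on the mesh; an older inline random-color material setup remains unconnected.
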(event OnClicked(DohButton)
  (params (TouchedComponent :type Primitive%20Component%20Object%20Reference) (ButtonPressed :type Key%20Structure :default "None"))
  (bind _returnvalue (Math|Random|RandomInteger 3))
  (bind _dohbutton (Variables|Default|GetDohButton))
  (bind _dohbutton_2 (Variables|Default|GetDohButton))
  (Development|PrintString "ButtonPress")
  (bind _newtrack_0 (Timeline|Squish Play)
    (:Update
      (switch int _returnvalue
        (:0
          (Components|SkeletalMesh|SetMorphTarget _dohbutton_2 "Squish1" _newtrack_0 true))
        (:1
          (Components|SkeletalMesh|SetMorphTarget _dohbutton_2 "Squish2" _newtrack_0 true))
        (:2
          (Components|SkeletalMesh|SetMorphTarget _dohbutton_2 "Squish3" _newtrack_0 true))))
    (:Finished
      (Timeline|Unsquish Play
        (:Update
          (switch int _returnvalue
            (:0
              (Components|SkeletalMesh|SetMorphTarget _dohbutton "Squish1" 0.0 true))
            (:1
              (Components|SkeletalMesh|SetMorphTarget _dohbutton "Squish2" 0.0 true))
            (:2
              (Components|SkeletalMesh|SetMorphTarget _dohbutton "Squish3" 0.0 true))))))))

(event OnInputTouchBegin(DohButton)
  (params (FingerIndex :type ETouchIndex%20Enum :default "Touch1") (TouchedComponent :type Primitive%20Component%20Object%20Reference))
  (bind _returnvalue (Math|Random|RandomInteger 3))
  (bind _dohbutton (Variables|Default|GetDohButton))
  (bind _dohbutton_2 (Variables|Default|GetDohButton))
  (Development|PrintString "ButtonPress")
  (bind _newtrack_0 (Timeline|Squish Play)
    (:Update
      (switch int _returnvalue
        (:0
          (Components|SkeletalMesh|SetMorphTarget _dohbutton_2 "Squish1" _newtrack_0 true))
        (:1
          (Components|SkeletalMesh|SetMorphTarget _dohbutton_2 "Squish2" _newtrack_0 true))
        (:2
          (Components|SkeletalMesh|SetMorphTarget _dohbutton_2 "Squish3" _newtrack_0 true))))
    (:Finished
      (Timeline|Unsquish Play
        (:Update
          (switch int _returnvalue
            (:0
              (Components|SkeletalMesh|SetMorphTarget _dohbutton "Squish1" 0.0 true))
            (:1
              (Components|SkeletalMesh|SetMorphTarget _dohbutton "Squish2" 0.0 true))
            (:2
              (Components|SkeletalMesh|SetMorphTarget _dohbutton "Squish3" 0.0 true))))))))

(event Input|KeyboardEvents|E
  (params (Key :type Key%20Structure :default "None"))
  (bind _returnvalue (Math|Random|RandomInteger 3))
  (bind _dohbutton (Variables|Default|GetDohButton))
  (bind _dohbutton_2 (Variables|Default|GetDohButton))
  (:Pressed
    (Development|PrintString "ButtonPress")
    (bind _newtrack_0 (Timeline|Squish Play)
      (:Update
        (switch int _returnvalue
          (:0
            (Components|SkeletalMesh|SetMorphTarget _dohbutton_2 "Squish1" _newtrack_0 true))
          (:1
            (Components|SkeletalMesh|SetMorphTarget _dohbutton_2 "Squish2" _newtrack_0 true))
          (:2
            (Components|SkeletalMesh|SetMorphTarget _dohbutton_2 "Squish3" _newtrack_0 true))))
      (:Finished
        (Timeline|Unsquish Play
          (:Update
            (switch int _returnvalue
              (:0
                (Components|SkeletalMesh|SetMorphTarget _dohbutton "Squish1" 0.0 true))
              (:1
                (Components|SkeletalMesh|SetMorphTarget _dohbutton "Squish2" 0.0 true))
              (:2
                (Components|SkeletalMesh|SetMorphTarget _dohbutton "Squish3" 0.0 true))))))))
  (:Released
    (Timeline|Unsquish Play)))

(fn ConstructionScript
  (CallFunction|SetRandomColors (Variables|Default|GetDohButton)))