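; Base tank projectile that ricochets a limited number of times, damaging tanks, opening airdrop crates and destroying other projectiles.
; Tick moves it manually by Velocity, and a sphere trace triggers powerup, projectile, tank and wall checks, then bounce and death.
; Bounces mirror a forward line trace's normal, then turn toward the new trace's hit.
; The owning tank supplies colour and sounds and is notified when projectiles are destroyed.
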(event Custom|SetTankVariables
  (bind _tankref (Variables|Default|GetTankRef))
  (bind _tankvariables (Variables|/Game/Blueprints/Player/BP_BaseTank.BP_BaseTank_C|GetTankVariables _tankref))
  ;[0.2 0.2 0.2] Sets the initial speed of the projectile
  (bind _outactors (Actor|GetAllActorsOfClass "/Game/Blueprints/Generation/BP_FloorWithTreads.BP_FloorWithTreads_C"))
  (for _array_element _outactors
    (Variables|Default|SetActorsToIgnore (Utilities|Array|MakeArray _array_element (Variables|Default|GetTankRef))))
  (CallFunction|SetVelocity)
  (Variables|Sound|SetMove%20Sound (.movesound _tankvariables))
  (Variables|Sound|SetBounceSound (.bouncesound _tankvariables))
  (Variables|Sound|SetExplosion%20Sound (.explosionsound _tankvariables))
  (Variables|Sound|SetShoot%20Sound (select (.bSuccess (Utilities|Casting|CastToBP_BigProjectile self)) (.bigbulletssound _tankvariables) (.shootsound _tankvariables))))

(event EventBeginPlay
  ;[0.2 0.2 0.2] Sets the initial speed of the projectile
  (CallFunction|SetTankVariables))

(event EventTick
  (params (DeltaSeconds :type Float%20%28single-precision%29))
  (bind _returnvalue (Transformation|GetActorForwardVector))
  (bind _returnvalue_2 (Transformation|GetActorLocation))
  (bind _returnvalue_3 (Transformation|GetActorLocation))
  (bind _actorstoignore (Variables|Default|GetActorsToIgnore))
  (bind _draw_debug_type (Variables|Debugging|GetDraw%20Debug%20Type))
  (bind _draw_time (Variables|Debugging|GetDraw%20Time))
  (bind (_start _end) (CallFunction|GetStartandEndforLineTrace _returnvalue_3 _returnvalue 1e+20))
  ;[0.2 0.2 0.2] Movement for projectile
  (Transformation|SetActorLocation (+ (* DeltaSeconds (Variables|Speed|GetVelocity)) (Transformation|GetActorLocation)) true true)
  ;[0.2 0.2 0.2] trace forward vector
  (bind _outhit (Collision|LineTraceByChannel _start _end "TraceTypeQuery1" false (Variables|Default|GetActorsToIgnore) (Variables|Debugging|GetDraw%20Debug%20Type) true "(R=1.000000,G=0.000000,B=0.000000,A=1.000000)" "(R=0.000000,G=1.000000,B=0.000000,A=1.000000)" (Variables|Debugging|GetDraw%20Time)))
  ;[0.2 0.2 0.2] trace normal of hit and mirrored projectile motion
  (bind (_outhit_2 _returnvalue_4) (Collision|SphereTraceByChannel _returnvalue_2 _returnvalue_2 (+ (.SphereRadius (Collision|GetComponentBounds (Variables|Default|GetStaticMesh))) 0.1) "TraceTypeQuery1" false (Variables|Default|GetActorsToIgnore) (Variables|Debugging|GetDraw%20Debug%20Type) true "(R=1.000000,G=0.000000,B=0.000000,A=1.000000)" "(R=0.000000,G=1.000000,B=0.000000,A=1.000000)" (Variables|Debugging|GetDraw%20Time)))
  (if _returnvalue_4
    (Utilities|FlowControl|Sequence
      (:then_0
        (Collision|CheckforHitPowerup _outhit_2))
      (:then_1
        (Collision|CheckforHitProjectile _outhit_2))
      (:then_2
        (Collision|CheckforHitTank _outhit_2))
      (:then_3
        (Collision|CheckforWall _outhit_2))
      (:then_4
        (Utilities|FlowControl|Sequence
          (:then_0
            (Collision|LineTraceByChannel (.Start (CallFunction|GetStartandEndforLineTrace (.location _outhit) (.normal _outhit) 1e+20)) (.End (CallFunction|GetStartandEndforLineTrace (.location _outhit) (.normal _outhit) 1e+20)) "TraceTypeQuery1" false _actorstoignore _draw_debug_type true "(R=1.000000,G=0.000000,B=0.000000,A=1.000000)" "(R=0.000000,G=1.000000,B=0.000000,A=1.000000)" _draw_time) ; noramal of the hit object
          )
          (:then_1
            (bind _outhit_3 (Collision|LineTraceByChannel (.Start (CallFunction|GetStartandEndforLineTrace (Transformation|GetActorLocation) (Math|Vector|MirrorVectorbyNormal (Transformation|GetActorForwardVector) (.normal _outhit)) 1e+20)) (.End (CallFunction|GetStartandEndforLineTrace (Transformation|GetActorLocation) (Math|Vector|MirrorVectorbyNormal (Transformation|GetActorForwardVector) (.normal _outhit)) 1e+20)) "TraceTypeQuery1" false _actorstoignore _draw_debug_type true "(R=1.000000,G=0.000000,B=0.000000,A=1.000000)" "(R=0.000000,G=1.000000,B=0.000000,A=1.000000)" _draw_time)) ; mirrored vector on normal
            (Collision|Bounce (.location _outhit_3)))
          (:then_2
            (CallFunction|Die)))))))

(fn ConstructionScript
  (bind _returnvalue (Rendering|Material|CreateDynamicMaterialInstance (Variables|Default|GetStaticMesh) 0 "/Game/Assets/Materials/Doh/M_BulletDoh.M_BulletDoh" "None" :!class /Script/Engine.PrimitiveComponent))
  (Rendering|Material|SetVectorParameterValue _returnvalue "DohColor" (.tankcolor (Variables|/Game/Blueprints/Player/BP_BaseTank.BP_BaseTank_C|GetTankVariables (Variables|Default|GetTankRef))) :!class /Script/Engine.MaterialInstanceDynamic)
  (Rendering|Material|SetScalarParameterValue _returnvalue "Bullet" 1.0 :!class /Script/Engine.MaterialInstanceDynamic))

(fn GetStartandEndforLineTrace
  (params (V1 :type Vector) (V2 :type Vector) (Scaling :type Float%20%28double-precision%29))
  (return V1 (+ V1 (* V2 Scaling))))

(fn SetVelocity
  (Variables|Speed|SetVelocity (Math|Conversions|ToVector2D(Vector) (* (Variables|Speed|GetSpeed) (Transformation|GetActorForwardVector)))))

(fn SetHitObjectName
  (params (OutHit :type Hit%20Result%20Structure))
  ;[0.2 0.2 0.2] debugging function
  (Development|PrintString (Utilities|String|Append "Hit Object Name: " (Utilities|GetObjectName (.HitActor (Collision|BreakHitResult OutHit)))) true true "(R=0.000000,G=0.660000,B=1.000000,A=1.000000)" 1e+01))

(fn Bounce
  (params (OutHitLocation :type Vector%20%28by%20ref%29))
  (bind _bounces (Variables|Bounces|GetBounces))
  ;[0.2 0.2 0.2] find new point from line trace, look towards, and rotate
  (if (Variables|Bounces|GetbCanBounce)
    (Transformation|SetActorRotation (Math|Rotator|MakeRotator 0.0 0.0 (.yaw (Math|Rotator|FindLookatRotation (Transformation|GetActorLocation) OutHitLocation))))
    (CallFunction|SetVelocity)
    (if (== _bounces (Variables|Bounces|GetBouncesBeforeDeath))
      _
      (else
        (Audio|PlaySound2D (Variables|Sound|GetBounceSound) 1.0 1.0 0.0 0 0)
        (Niagara|SpawnSystematLocation "/Game/Assets/FX/Bullet/FX_Bounce_old.FX_Bounce_old" (Transformation|GetActorLocation))))
    (bind _result (Math|Integer|IncrementInt _bounces)
      (:%20%20
        (if (Variables|Default|GetbEnableSuicide)
          (if (== _result 1) ; connect to enable self killing
            (Variables|Default|SetActorsToIgnore (Utilities|Array|MakeArray 0))))))))

(fn CheckforHitProjectile
  (params (OutHit :type Hit%20Result%20Structure))
  (bind _hitactor (Collision|BreakHitResult OutHit))
  ;[0.2 0.2 0.2] if projectile hits projectile, kill them both. If the projectile is big, destroy only the smaller projectile
  (bind _asbp_base_projectile (Utilities|Casting|CastToBP_BaseProjectile _hitactor))
  (LocalVariables|SetProjectile _asbp_base_projectile)
  (Utilities|Casting|CastToBP_BigProjectileClass (Utilities|GetClass _hitactor)
    (:then
      (CallFunction|RemoveandDestroy self))
    (:CastFailed
      (CallFunction|RemoveandDestroy (LocalVariables|GetProjectile) (LocalVariables|GetProjectile))
      (CallFunction|RemoveandDestroy self))))

(fn Die
  (bind _self self)
  ;[0.2 0.2 0.2] bounce x times and then die
  (if (> (Variables|Bounces|GetBounces) (Variables|Bounces|GetBouncesBeforeDeath))
    (CallFunction|RemoveandDestroy _self _self)))

(fn CheckforWall
  (params (OutHit :type Hit%20Result%20Structure))
  (bind (_bblockinghit _binitialoverlap _time _distance _location _impactpoint _normal _impactnormal _physmat _hitactor _hitcomponent) (Collision|BreakHitResult OutHit))
  (bind _self self)
  ;[0.2 0.2 0.2] if the projectile cannot bounce, only destroy when it hits a wall
  (Utilities|FlowControl|Sequence
    (:then_0
      (if (Physics|IsSimulatingPhysics _hitcomponent "None")
        (Physics|AddImpulseatLocation _hitcomponent (* (Transformation|GetActorForwardVector) (* (.SphereRadius (Collision|GetComponentBounds (Variables|Default|GetStaticMesh))) (Variables|Speed|GetSpeed))) _location "None")))
    (:then_1
      (bind _asbp_base_wall (Utilities|Casting|CastToBP_BaseWall _hitactor))
      (Default|PlayHitSound _asbp_base_wall))
    (:then_2
      (if (not (Variables|Bounces|GetbCanBounce))
        (CallFunction|RemoveandDestroy _self _self)))))

(fn CheckforHitTank
  (params (OutHit :type Hit%20Result%20Structure))
  (bind _self self)
  (bind _asbp_base_tank (Utilities|Casting|CastToBP_BaseTank (.HitActor (Collision|BreakHitResult OutHit))))
  (switch Utilities|FlowControl|Switch|SwitchonEPlayerState (Variables|/Game/Blueprints/Player/BP_Player.BP_Player_C|GetEPlayerState (Variables|/Game/Blueprints/Player/BP_BaseTank.BP_BaseTank_C|GetControllerReference _asbp_base_tank))
    (:NewEnumerator1
      (Default|DecrementLives (Variables|/Game/Blueprints/Player/BP_Player.BP_Player_C|GetTankRef (Variables|/Game/Blueprints/Player/BP_BaseTank.BP_BaseTank_C|GetControllerReference _asbp_base_tank)) self OutHit)
      (CallFunction|RemoveandDestroy _self _self))))

(fn RemoveandDestroy
  (params (ProjectileToRemove :type BP%20Base%20Projectile%20Object%20Reference))
  ;[0.2 0.2 0.2] Remove Projectile from array in BP_BaseTank and then die
  (bind _tankref (Variables|Default|GetTankRef)
    (:then
      (Default|RemoveProjectile _tankref ProjectileToRemove))
    (:else
      _))
  (Actor|DestroyActor ProjectileToRemove))

(fn CheckforHitPowerup
  (params (OutHit :type Hit%20Result%20Structure))
  (bind _self self)
  (bind _asbp_airdrop_crate (Utilities|Casting|CastToBP_AirdropCrate (.HitActor (Collision|BreakHitResult OutHit))))
  (Default|OpenCapsule _asbp_airdrop_crate)
  (CallFunction|RemoveandDestroy _self _self))