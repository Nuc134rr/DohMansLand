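; BP_Powerup is a powerup actor that picks a random type at BeginPlay and labels itself with 3D text.
; A random PowerupArray item becomes Powerup, while a switch on the random index sets one of five text values.
; Item and index come from separate Random evaluations, so label and type can differ.
; A looping timer calls ColorChange to cycle the text's front and extrude materials through ColorArray.
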(event EventBeginPlay
  (bind _poweruparray (Variables|Default|GetPowerupArray))
  (bind (_outitem _outindex) (Utilities|Array|Random _poweruparray))
  ;[1 1 1] Text Setter
  (Variables|Default|SetPowerup _outitem)
  (Utilities|Time|SetTimerbyFunctionName 0 "ColorChange" 0.2 true)
  (switch int _outindex
    (:0
      (Class|Text3DComponent|SetText (Variables|Default|GetText3D) (Variables|Default|GetValuePowerup0)))
    (:1
      (Class|Text3DComponent|SetText (Variables|Default|GetText3D) (Variables|Default|GetValuePowerup1)))
    (:2
      (Class|Text3DComponent|SetText (Variables|Default|GetText3D) (Variables|Default|GetValuePowerup2)))
    (:3
      (Class|Text3DComponent|SetText (Variables|Default|GetText3D) (Variables|Default|GetValuePowerup3)))
    (:4
      (Class|Text3DComponent|SetText (Variables|Default|GetText3D) (Variables|Default|GetValuePowerup4)))))

(fn ConstructionScript)

(fn ColorChange
  (bind _text3d (Variables|Default|GetText3D))
  (if (== (Variables|Default|GetColorIndex) 6)
    (Variables|Default|SetColorIndex 0))
  (Class|Text3DComponent|SetExtrudeMaterial _text3d (Utilities|Array|Get(acopy) (Variables|Default|GetColorArray) (Variables|Default|GetColorIndex)))
  (Class|Text3DComponent|SetFrontMaterial _text3d (Utilities|Array|Get(acopy) (Variables|Default|GetColorArray) (Variables|Default|GetColorIndex)))
  (Variables|Default|SetColorIndex (+ (Variables|Default|GetColorIndex) 1)))