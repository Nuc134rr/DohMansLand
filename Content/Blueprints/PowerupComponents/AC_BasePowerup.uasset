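; AC_BasePowerup is the base actor component for powerups attached to tanks in the DohMansLand game mode.
; On BeginPlay it caches its owner as a BP_BaseTank reference for variable editing and registers its Sound with the game mode's music.
; On EndPlay it asks the game mode to remove that music, passing the sound and its own component class.
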(event EventBeginPlay
  ;[0.2 0.2 0.2] Sets a reference to BaseTank for varaible editing
  (Variables|Default|SetOwnerRef (.AsBP%20Base%20Tank (Utilities|Casting|CastToBP_BaseTank (Components|GetOwner))))
  (Default|AddMusic (CallFunction|GetDohMansLandGameMode) (Variables|Default|GetSound)))

(event EventEndPlay
  (params (EndPlayReason :type EEndPlayReason%20Enum :default "Destroyed"))
  (Default|RemoveMusic (CallFunction|GetDohMansLandGameMode) (Variables|Default|GetSound) (Utilities|GetClass self)))