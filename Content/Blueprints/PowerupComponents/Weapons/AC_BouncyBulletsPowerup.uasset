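; Weapon powerup component that makes the owner's projectiles extra bouncy.
; On BeginPlay it runs the parent logic and plays a pickup sound at the controller's spawn point location.
; Every Tick it loops over the owner's active projectiles, enabling bouncing and raising their bounce count before death, rather than modifying projectiles as they spawn.
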(event EventTick
  (params (DeltaSeconds :type Float%20%28single-precision%29))
  ;[0.2 0.2 0.2] Makes all projectiles extra bouncy
  (for _array_element (Variables|/Game/Blueprints/Player/BP_BaseTank.BP_BaseTank_C|GetActiveProjectiles (Variables|Default|GetOwnerRef))
    (Variables|/Game/Blueprints/Projectiles/BP_BaseProjectile.BP_BaseProjectile_C|SetbCanBounce _array_element true)
    (Variables|/Game/Blueprints/Projectiles/BP_BaseProjectile.BP_BaseProjectile_C|SetBouncesBeforeDeath _array_element 10)))

(event EventBeginPlay
  ;[0.2 0.2 0.2] Makes all projectiles extra bouncy
  (|CallParentFunction)
  (Audio|PlaySoundatLocation "/Game/Assets/SFX/misc_outside_noises/Powerup_sounds/bullet_powerups/SFXQ_Bullet_powerup_pickup.SFXQ_Bullet_powerup_pickup" (Transformation|GetWorldLocation (Variables|/Game/Blueprints/Player/BP_Player.BP_Player_C|GetSpawnPoint (Variables|/Game/Blueprints/Player/BP_BaseTank.BP_BaseTank_C|GetControllerReference (Variables|Default|GetOwnerRef)))) "0, 0, 0" 1.0 1.0 0.0 0 0 0 0))