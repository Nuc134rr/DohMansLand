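; Weapon powerup component that switches the owner to fast projectiles when it begins play.
; After the parent BeginPlay, it resets the turret to the default mesh and plays a pickup sound at the controller's spawn point.
; It then sets the owner's projectile class to BP_FireProjectile, which per its comment also removes big bullets.
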(event EventBeginPlay
  (bind _ownerref (Variables|Default|GetOwnerRef))
  ;[0.2 0.2 0.2] Set projectile type to Fast/removes big bullets
  (|CallParentFunction)
  (Components|StaticMesh|SetStaticMesh (Variables|/Game/Blueprints/Player/BP_BaseTank.BP_BaseTank_C|GetTurret _ownerref) (Variables|/Game/Blueprints/Player/BP_BaseTank.BP_BaseTank_C|GetDefaultTurretMesh _ownerref))
  (Audio|PlaySoundatLocation "/Game/Assets/SFX/misc_outside_noises/Powerup_sounds/bullet_powerups/SFXQ_Bullet_powerup_pickup.SFXQ_Bullet_powerup_pickup" (Transformation|GetWorldLocation (Variables|/Game/Blueprints/Player/BP_Player.BP_Player_C|GetSpawnPoint (Variables|/Game/Blueprints/Player/BP_BaseTank.BP_BaseTank_C|GetControllerReference (Variables|Default|GetOwnerRef)))) "0, 0, 0" 1.0 1.0 0.0 0 0 0 0)
  (Variables|/Game/Blueprints/Player/BP_BaseTank.BP_BaseTank_C|SetProjectileClass (Variables|Default|GetOwnerRef) "/Game/Blueprints/Projectiles/BP_FireProjectile.BP_FireProjectile_C"))