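; Powerup component that switches the owning tank's weapon to big projectiles.
; On BeginPlay it plays the pickup sound at the owner's spawn point and sets the owner's projectile class to BP_BigProjectile.
; It also swaps the turret mesh to the monkey barrel and tints a dynamic material instance with the tank's color.
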(event EventBeginPlay
  (bind _ownerref (Variables|Default|GetOwnerRef))
  (bind _turret (Variables|/Game/Blueprints/Player/BP_BaseTank.BP_BaseTank_C|GetTurret _ownerref))
  ;[0.2 0.2 0.2] set projectile type to big
  (|CallParentFunction)
  (Audio|PlaySoundatLocation "/Game/Assets/SFX/misc_outside_noises/Powerup_sounds/bullet_powerups/Bullet_powerup_pickup.Bullet_powerup_pickup" (Transformation|GetWorldLocation (Variables|/Game/Blueprints/Player/BP_Player.BP_Player_C|GetSpawnPoint (Variables|/Game/Blueprints/Player/BP_BaseTank.BP_BaseTank_C|GetControllerReference (Variables|Default|GetOwnerRef)))) "0, 0, 0" 1.0 1.0 0.0 0 0 0 0)
  (Utilities|FlowControl|Sequence
    (:then_0
      (Variables|/Game/Blueprints/Player/BP_BaseTank.BP_BaseTank_C|SetProjectileClass (Variables|Default|GetOwnerRef) "/Game/Blueprints/Projectiles/BP_BigProjectile.BP_BigProjectile_C"))
    (:then_1
      ;[0.2 0.2 0.2] Sets new turret mesh
      (Components|StaticMesh|SetStaticMesh _turret "/Game/Assets/Meshes/MonkeyGun/SM_MonkeyBarrel.SM_MonkeyBarrel")
      (bind _returnvalue (Rendering|Material|CreateDynamicMaterialInstance _turret 0 "/Game/Assets/Materials/Monkies/M_MonkeyBarrel.M_MonkeyBarrel" "None" :!class /Script/Engine.PrimitiveComponent))
      (Rendering|Material|SetVectorParameterValue _returnvalue "BarrelColor" (.tankcolor (Variables|/Game/Blueprints/Player/BP_BaseTank.BP_BaseTank_C|GetTankVariables _ownerref)) :!class /Script/Engine.MaterialInstanceDynamic))))