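; Weapon powerup component that switches the owning tank to big projectiles.
; On BeginPlay it plays a pickup sound, sets the projectile class, and swaps in the monkey barrel mesh with a dynamic material in the tank's color.
; Every Tick it rescales all active projectile meshes by the number of copies of this component on the owner, so stacked pickups enlarge shots up to double scale.
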(event EventBeginPlay
  (bind _ownerref (Variables|Default|GetOwnerRef))
  (bind _turret (Variables|/Game/Blueprints/Player/BP_BaseTank.BP_BaseTank_C|GetTurret _ownerref))
  ;[0.2 0.2 0.2] set projectile type to big
  (|CallParentFunction)
  (Audio|PlaySoundatLocation "/Game/Assets/SFX/misc_outside_noises/Powerup_sounds/bullet_powerups/SFXQ_Bullet_powerup_pickup.SFXQ_Bullet_powerup_pickup" (Transformation|GetWorldLocation (Variables|/Game/Blueprints/Player/BP_Player.BP_Player_C|GetSpawnPoint (Variables|/Game/Blueprints/Player/BP_BaseTank.BP_BaseTank_C|GetControllerReference (Variables|Default|GetOwnerRef)))) "0, 0, 0" 1.0 1.0 0.0 0 0 0 0)
  (Utilities|FlowControl|Sequence
    (:then_0
      (Variables|/Game/Blueprints/Player/BP_BaseTank.BP_BaseTank_C|SetProjectileClass (Variables|Default|GetOwnerRef) "/Game/Blueprints/Projectiles/BP_BigProjectile.BP_BigProjectile_C"))
    (:then_1
      ;[0.2 0.2 0.2] Sets new turret mesh
      (Components|StaticMesh|SetStaticMesh _turret "/Game/Assets/Meshes/MonkeyGun/SM_MonkeyBarrel.SM_MonkeyBarrel")
      (bind _returnvalue (Rendering|Material|CreateDynamicMaterialInstance _turret 0 "/Game/Assets/Materials/Monkies/M_MonkeyBarrel.M_MonkeyBarrel" "None" :!class /Script/Engine.PrimitiveComponent))
      (Rendering|Material|SetVectorParameterValue _returnvalue "BarrelColor" (.tankcolor (Variables|/Game/Blueprints/Player/BP_BaseTank.BP_BaseTank_C|GetTankVariables _ownerref)) :!class /Script/Engine.MaterialInstanceDynamic))))

(event EventTick
  (params (DeltaSeconds :type Float%20%28single-precision%29))
  (bind _ownerref (Variables|Default|GetOwnerRef))
  (bind _returnvalue (Actor|GetComponentsByClass _ownerref "AC_BigProjectilesPowerup_C"))
  (bind _returnvalue_2 (Utilities|Array|Length _returnvalue))
  (bind _returnvalue_3 (Math|Integer|Clamp(Integer) _returnvalue_2 0 2))
  (bind _returnvalue_4 (Math|Conversions|ToFloat(Integer) _returnvalue_3))
  (for _array_element (Variables|/Game/Blueprints/Player/BP_BaseTank.BP_BaseTank_C|GetActiveProjectiles (Variables|Default|GetOwnerRef))
    (Transformation|SetWorldScale3D (Variables|/Game/Blueprints/Projectiles/BP_BaseProjectile.BP_BaseProjectile_C|GetStaticMesh _array_element) (Math|Vector|MakeVector _returnvalue_4 _returnvalue_4 _returnvalue_4))))