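; Powerup component that makes every tank except its owner slide frictionlessly and turns the owner's tank into a Zamboni.
; On BeginPlay it zeroes the other tanks' deceleration, alters their turning boost and switches tread floors to the ice material.
; A game-mode death callback, gated by a never-reset DoOnce, either lowers the last-found floor's ice alpha for an affected tank or clears it and restores movement if the owner died.
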(event Custom|SetNoFrictionAlpha
  (params (Tank :type BP%20Base%20Tank%20Object%20Reference))
  ;[0.2 0.2 0.2] Applies no friction to all tanks EXCEPT the player that picked it up
  (Utilities|FlowControl|DoOnce false
    (:Completed
      (if (Utilities|Array|ContainsItem (Variables|Default|GetAffectedTanks) Tank)
        (Variables|/Game/Blueprints/Generation/BP_FloorWithTreads.BP_FloorWithTreads_C|SetAlpha (Variables|Default|GetFloorRef) (- (Variables|/Game/Blueprints/Generation/BP_FloorWithTreads.BP_FloorWithTreads_C|GetAlpha (Variables|Default|GetFloorRef)) (/ 1.0 (Math|Conversions|ToFloat(Integer) (Variables|Default|GetNumberOfPlayers)))))
        (Default|SetNoFrictionMaterial (Variables|Default|GetFloorRef) false)
        (Utilities|Array|RemoveItem (Variables|Default|GetAffectedTanks) Tank)
        (elif (== Tank (Variables|Default|GetOwnerRef))
          (Variables|/Game/Blueprints/Generation/BP_FloorWithTreads.BP_FloorWithTreads_C|SetAlpha (Variables|Default|GetFloorRef) 0.0)
          (Default|SetNoFrictionMaterial (Variables|Default|GetFloorRef) false)
          (for _array_element (Variables|Default|GetAffectedTanks)
            (Variables|/Script/Engine.FloatingPawnMovement|SetDeceleration (Variables|/Game/Blueprints/Player/BP_BaseTank.BP_BaseTank_C|GetFloatingPawnMovement _array_element) (Variables|Default|GetDefaultDeceleration))
            (Variables|/Script/Engine.FloatingPawnMovement|SetTurningBoost (Variables|/Game/Blueprints/Player/BP_BaseTank.BP_BaseTank_C|GetFloatingPawnMovement _array_element) (Variables|Default|GetDefaultTurningBoost))))))))

(event EventBeginPlay
  (bind _ownerref (Variables|Default|GetOwnerRef))
  (bind _ownerref_2 (Variables|Default|GetOwnerRef))
  (bind _floatingpawnmovement (Variables|/Game/Blueprints/Player/BP_BaseTank.BP_BaseTank_C|GetFloatingPawnMovement _ownerref))
  ;[0.2 0.2 0.2] Applies no friction to all tanks EXCEPT the player that picked it up
  (|CallParentFunction)
  (EventDispatchers|BindEventtoTankDeath (CallFunction|GetDohMansLandGameMode) (delegate Custom|SetNoFrictionAlpha))
  (Audio|PlaySound2D "/Game/Assets/SFX/misc_outside_noises/Powerup_sounds/Ice/SFXQ_ice_sfx.SFXQ_ice_sfx" 1.0 1.0 0.0 0 0)
  (bind _outactors (Actor|GetAllActorsOfClass "/Game/Blueprints/Player/BP_BaseTank.BP_BaseTank_C"))
  (bind _output_get (Variables|Default|SetAffectedTanks _outactors))
  (Utilities|Array|RemoveItem _output_get (Variables|Default|GetOwnerRef))
  (Variables|Default|SetNumberOfPlayers (Utilities|Array|Length (Variables|Default|GetAffectedTanks)))
  (for _array_element (Variables|Default|GetAffectedTanks)
    (Variables|/Script/Engine.FloatingPawnMovement|SetDeceleration (Variables|/Game/Blueprints/Player/BP_BaseTank.BP_BaseTank_C|GetFloatingPawnMovement _array_element) 0.0)
    (Variables|/Script/Engine.FloatingPawnMovement|SetTurningBoost (Variables|/Game/Blueprints/Player/BP_BaseTank.BP_BaseTank_C|GetFloatingPawnMovement _array_element) -16.0))
  (bind _outactors_2 (Actor|GetAllActorsOfClass "/Game/Blueprints/Generation/BP_FloorWithTreads.BP_FloorWithTreads_C"))
  (for _array_element_2 _outactors_2
    (bind _output_get_2 (Variables|Default|SetFloorRef _array_element_2))
    (Default|SetNoFrictionMaterial _output_get_2 true))
  (Variables|/Script/Engine.FloatingPawnMovement|SetDeceleration _floatingpawnmovement (Variables|Default|GetDefaultDeceleration))
  (Variables|/Script/Engine.FloatingPawnMovement|SetTurningBoost _floatingpawnmovement (Variables|Default|GetDefaultTurningBoost))
  (Components|StaticMesh|SetStaticMesh (Variables|/Game/Blueprints/Player/BP_BaseTank.BP_BaseTank_C|GetTankBase _ownerref_2) "/Game/Assets/Meshes/Tank/Zamboni/SM_ZAMBONI.SM_ZAMBONI")
  (Components|StaticMesh|SetStaticMesh (Variables|/Game/Blueprints/Player/BP_BaseTank.BP_BaseTank_C|GetTurret _ownerref_2) "/Game/Assets/Meshes/Tank/Zamboni/SM_ZamboniTop.SM_ZamboniTop"))