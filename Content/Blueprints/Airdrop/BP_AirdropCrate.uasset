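; Airdrop crate actor that rolls a random powerup on spawn and shows it with a decal.
; BeginPlay picks from the powerup array, stores its index and looks up the matching decal material in a map.
; Hits against a Chunk re-apply the root's current transform as a non-sweeping physics teleport.
; An explosion effect and sound chain exists but is not connected to any event.
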(event EventBeginPlay
  (bind _poweruparray (Variables|Powerups|GetPowerupArray))
  (Variables|Powerups|SetPowerup (.OutItem (Utilities|Array|Random _poweruparray)))
  (Variables|Powerups|SetPowerupInt (Utilities|Array|FindItem _poweruparray (Variables|Powerups|GetPowerup)))
  (Rendering|Components|Decal|SetDecalMaterial (Variables|Default|GetDecal) (.Value (Utilities|Map|Find (Variables|Powerups|GetPowerupDecalMap) (Variables|Powerups|GetPowerup)))))

(event Collision|EventHit
  (params (MyComp :type Primitive%20Component%20Object%20Reference) (Other :type Actor%20Object%20Reference) (OtherComp :type Primitive%20Component%20Object%20Reference) (bSelfMoved :type Boolean) (HitLocation :type Vector :default "0, 0, 0") (HitNormal :type Vector :default "0, 0, 0") (NormalImpulse :type Vector :default "0, 0, 0") (Hit :type Hit%20Result%20Structure%20%28by%20ref%29))
  (bind _defaultsceneroot (Variables|Default|GetDefaultSceneRoot))
  ;[0.2 0.2 0.2] long ass node lol
  (Utilities|Casting|CastToChunk Other)
  (Transformation|SetWorldTransform _defaultsceneroot (Transformation|GetWorldTransform _defaultsceneroot) false true))

(fn ConstructionScript)