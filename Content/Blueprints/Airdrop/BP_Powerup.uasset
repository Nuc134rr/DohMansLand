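; BP_Powerup is an airdrop powerup actor that displays a randomly chosen powerup as animated 3D text.
; On BeginPlay it picks a random entry from the powerup array, stores its index and uses that index to select the matching value for the Text3D label.
; A looping timer calls ColorChange, which cycles the text's front and extrude materials through a color array for a flashing effect.
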(event EventBeginPlay
  (bind _poweruparray (Variables|Default|GetPowerupArray))
  ;[1 1 1] Text Setter
  (Variables|Default|SetPowerup (.OutItem (Utilities|Array|Random _poweruparray)))
  (Variables|Default|SetPowerupInt (Utilities|Array|FindItem _poweruparray (Variables|Default|GetPowerup)))
  (Utilities|Time|SetTimerbyFunctionName 0 "ColorChange" 0.2 true)
  (Class|Text3DComponent|SetText (Variables|Default|GetText3D) (Utilities|Select :Index (Variables|Default|GetPowerupInt) :Option%200 (Variables|Default|GetValuePowerup0) :Option%201 (Variables|Default|GetValuePowerup1) :Option%202 (Variables|Default|GetValuePowerup2) :Option%203 (Variables|Default|GetValuePowerup3) :Option%204 (Variables|Default|GetValuePowerup4) :Option%205 (Variables|Default|GetValuePowerup5))))

(fn ConstructionScript)

(fn ColorChange
  (bind _text3d (Variables|Default|GetText3D))
  (if (== (Variables|Default|GetColorIndex) 6)
    (Variables|Default|SetColorIndex 0))
  (Class|Text3DComponent|SetExtrudeMaterial _text3d (Utilities|Array|Get(acopy) (Variables|Default|GetColorArray) (Variables|Default|GetColorIndex)))
  (Class|Text3DComponent|SetFrontMaterial _text3d (Utilities|Array|Get(acopy) (Variables|Default|GetColorArray) (Variables|Default|GetColorIndex)))
  (Variables|Default|SetColorIndex (+ (Variables|Default|GetColorIndex) 1)))