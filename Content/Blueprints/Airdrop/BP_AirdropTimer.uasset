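; Airdrop countdown actor with a rotating dial that periodically drops fresh BP_AirdropCrate actors from high in the sky.
; A looping timer steps TimerDial 6 degrees every sixtieth of a random cooldown.
; When yaw nears zero, it destroys existing crates and spawns MaxSpawnedAirdrops new ones using random navmesh points for X/Y.
; It then stops the timer while the WindTimer timeline rewinds the dial, then restarts with a new cooldown.
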(event Custom|ResetCountdown
  ;[0.2 0.2 0.2] Rewinds timer after airdrop is dropped
  (bind _newrotation (Timeline|WindTimer PlayFromStart)
    (:Update
      (Transformation|SetRelativeRotation (Variables|Default|GetTimerDial) (Math|Rotator|MakeRotator 0.0 0.0 _newrotation) false false))
    (:Finished
      (Variables|Default|SetCooldown (Math|Random|RandomFloatinRange (Variables|Default|GetMinCooldown) (Variables|Default|GetMaxCooldown)))
      (CallFunction|StartTimer))))

(event Custom|TickTimer
  (bind _origin (Variables|Default|GetOrigin))
  (bind _nav_data (Variables|Default|GetNav%20Data))
  (bind _timerdial (Variables|Default|GetTimerDial))
  (bind _randomlocation (Class|NavigationSystemV1|GetRandomPointinNavigableRadius _origin 5e+03 _nav_data 0))
  ;[0.2 0.2 0.2] Ticks the timer depending on the cooldown
  (Transformation|AddRelativeRotation _timerdial (Math|Rotator|MakeRotator 0.0 0.0 -6.0) false false)
  (if (Math|Float|NearlyEqual(Float) (.yaw (Variables|/Script/Engine.SceneComponent|GetRelativeRotation _timerdial)) 0.0 2.0)
    (bind _outactors (Actor|GetAllActorsOfClass "/Game/Blueprints/Airdrop/BP_AirdropCrate.BP_AirdropCrate_C"))
    (for _array_element _outactors
      (Actor|DestroyActor _array_element))
    (for _index (range 0 (- (Variables|Default|GetMaxSpawnedAirdrops) 1))
      (Game|SpawnActorfromClass "/Game/Blueprints/Airdrop/BP_AirdropCrate.BP_AirdropCrate_C" (Math|Transform|MakeTransform (Math|Vector|MakeVector (.x _randomlocation) (.y _randomlocation) (Math|Random|RandomFloatinRange 2e+04 4e+04)) "0, 0, 0" "1.000000,1.000000,1.000000") "Undefined" 0 0)
      (CallFunction|ResetCountdown)
      (Utilities|Time|ClearandInvalidateTimerbyHandle (Variables|Default|GetTimerHandle)))))

(event Custom|StartTimer
  (bind _returnvalue (Utilities|Time|SetTimerbyEvent (delegate Custom|TickTimer) (/ (Variables|Default|GetCooldown) 6e+01) true))
  (Variables|Default|SetTimerHandle _returnvalue))

(event EventBeginPlay
  (Variables|Default|SetCooldown (Math|Random|RandomFloatinRange (Variables|Default|GetMinCooldown) (Variables|Default|GetMaxCooldown)))
  (CallFunction|StartTimer))

(fn ConstructionScript)