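; BP_Airdrop is an airdrop actor that turns into a powerup after it lands on terrain of the Chunk class.
; On a hit with a Chunk, it waits briefly, spawns an enlarged BP_Powerup at its own transform and destroys itself.
; An Impulse function applies random angular tumbling to the AirDrop component, but its looping timer is disconnected, and the Spawned event called at BeginPlay is empty.
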(event Custom|Spawned)

(event Collision|EventHit
  (params (MyComp :type Primitive%20Component%20Object%20Reference) (Other :type Actor%20Object%20Reference) (OtherComp :type Primitive%20Component%20Object%20Reference) (bSelfMoved :type Boolean) (HitLocation :type Vector :default "0, 0, 0") (HitNormal :type Vector :default "0, 0, 0") (NormalImpulse :type Vector :default "0, 0, 0") (Hit :type Hit%20Result%20Structure%20%28by%20ref%29))
  (Utilities|Casting|CastToChunk (.hitactor Hit))
  (Utilities|FlowControl|Delay 1.0)
  (Game|SpawnActorfromClass "/Game/Blueprints/Airdrop/BP_Powerup.BP_Powerup_C" (Math|Transform|MakeTransform (Transformation|GetActorLocation) (Transformation|GetActorRotation) "3.000000,3.000000,3.000000") "Undefined" 0 0)
  (Actor|DestroyActor))

(event EventBeginPlay
  (CallFunction|Spawned))

(fn ConstructionScript)

(fn Impulse
  (bind _returnvalue (Math|Random|RandomFloatinRange -15.0 15.0))
  (Class|PrimitiveComponent|AddAngularImpulseinDegrees (Variables|Default|GetAirDrop) (Math|Vector|MakeVector _returnvalue _returnvalue _returnvalue) "None" true))