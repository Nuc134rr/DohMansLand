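; BP_Bomb is a timed bomb that kills tanks and destroys most other objects in its blast radius, sparing BP_FloorWithTreads.
; A fuse timeline drives the dynamic material's colour, with a delayed beep, then triggers Explode.
; Explode runs two sphere traces: one for destruction, a wider one that impulses the bomb's own Mesh toward physics-simulating hits.
; The bomb then destroys itself, spawning explosion FX and camera shake from Destroyed.
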(event Custom|Explode
  (bind _mesh (Variables|Default|GetMesh))
  (bind _mesh_2 (Variables|Default|GetMesh))
  (bind _returnvalue (Transformation|GetWorldLocation _mesh))
  (bind _returnvalue_2 (Transformation|GetWorldLocation _mesh_2))
  ;[0.2 0.2 0.2] Explode anything within the ExplosionRadius, and Impulse anything in the ImpulseRadius
  (bind _outhits (Collision|MultiSphereTraceByChannel _returnvalue_2 _returnvalue_2 (Variables|Default|GetExplosionRadius) "TraceTypeQuery3" false 0 "None"))
  (for _array_element _outhits
    (Utilities|Casting|CastToBP_FloorWithTreads (.HitActor (Collision|BreakHitResult _array_element))
      (:CastFailed
        (bind _asbp_new_base_tank (Utilities|Casting|CastToBP_NewBaseTank (.HitActor (Collision|BreakHitResult _array_element)))
          (:then
            (Default|TankDeath (Variables|/Game/Blueprints/Player/BP_NewBaseTank.BP_NewBaseTank_C|GetControllerReference _asbp_new_base_tank)))
          (:CastFailed
            (Actor|DestroyActor (.HitActor (Collision|BreakHitResult _array_element)))
            (Components|DestroyComponent (.HitComponent (Collision|BreakHitResult _array_element))))))))
  (bind _outhits_2 (Collision|MultiSphereTraceByChannel _returnvalue _returnvalue (+ (Variables|Default|GetExplosionRadius) (Variables|Default|GetImpulseRadius)) "TraceTypeQuery3" false 0 "None"))
  (for _array_element_2 _outhits_2
    (if (Physics|IsSimulatingPhysics (Variables|/Script/Engine.Actor|GetRootComponent (.HitActor (Collision|BreakHitResult _array_element_2))) "None")
      (Transformation|SetActorRotation (Math|Rotator|FindLookatRotation (Transformation|GetActorLocation) (.Location (Collision|BreakHitResult _array_element_2))))
      (Physics|AddImpulseatLocation (Variables|Default|GetMesh) (* (Transformation|GetActorForwardVector) (Variables|Default|GetImpulseStrength)) (.Location (Collision|BreakHitResult _array_element_2)) "None")))
  (Actor|DestroyActor))

(event EventBeginPlay
  (Utilities|FlowControl|Sequence
    (:then_0
      (bind _fusetimer (Timeline|FuseTimer Play)
        (:Update
          (Rendering|Material|SetScalarParameterValue (Variables|Default|GetBombMaterial) "BombColor" _fusetimer :!class /Script/Engine.MaterialInstanceDynamic))
        (:Finished
          (CallFunction|Explode)
          (Audio|PlaySound2D "/Game/Assets/SFX/misc_outside_noises/Powerup_capsule/Capsule_explosion/powerup_explosion_Cue.powerup_explosion_Cue" 1.0 1.0 0.0 0 0))))
    (:then_1
      (Utilities|FlowControl|Delay 5.0)
      (Audio|PlaySound2D "/Game/Assets/SFX/misc_outside_noises/Powerup_capsule/Powerup_Beeping/beeping_Cue.beeping_Cue" 1.0 1.0 0.0 0 0))))

(event EventDestroyed
  (Niagara|SpawnSystematLocation "/Game/Assets/FX/AirDrops/FX_BombExplosion.FX_BombExplosion" (Transformation|GetActorLocation))
  (CameraShakes|StartCameraShake (Game|GetPlayerCameraManager 0) "/Game/Blueprints/MapItems/Bp_CameraShake.Bp_CameraShake_C" 4.0 "CameraLocal" "0, 0, 0"))

(fn ConstructionScript
  (bind _mesh (Variables|Default|GetMesh))
  (bind _returnvalue (Rendering|Material|CreateDynamicMaterialInstance _mesh 0 (Rendering|Material|GetMaterial _mesh 0) "None" :!class /Script/Engine.PrimitiveComponent))
  (Variables|Default|SetBombMaterial _returnvalue))