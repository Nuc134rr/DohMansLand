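; Touchable airdrop button that, when ready, spawns a batch of BP_AirdropCrate actors high in the sky.
; Crates appear at random navigable X/Y points around an origin, with random height and a dropping sound.
; Its material steps red, yellow, green as a timed cooldown, arming at green and resetting after each drop.
; A timeline drives the press animation through a scalar in the MPC_WorldOffset parameter collection.
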(event OnInputTouchBegin(Button)
  (params (FingerIndex :type ETouchIndex%20Enum :default "Touch1") (TouchedComponent :type Primitive%20Component%20Object%20Reference))
  (bind _origin (Variables|Default|GetOrigin))
  (bind _nav_data (Variables|Default|GetNav%20Data))
  (bind _randomlocation (Class|NavigationSystemV1|GetRandomPointinNavigableRadius _origin 5e+03 _nav_data 0))
  ;[1 1 1] Spawning Airdrop
  (Audio|PlaySound2D "/Game/Assets/SFX/misc_outside_noises/button_click_Cue.button_click_Cue" 1.0 1.0 0.0 0 0)
  (if (Variables|Default|Getready)
    (for _index (range 0 (- (Variables|Default|GetNumOfPowerups) 1))
      (Game|SpawnActorfromClass "/Game/Blueprints/Airdrop/BP_AirdropCrate.BP_AirdropCrate_C" (Math|Transform|MakeTransform (Math|Vector|MakeVector (.x _randomlocation) (.y _randomlocation) (Math|Random|RandomFloatinRange 2e+04 4e+04)) "0, 0, 0" "1.000000,1.000000,1.000000") "Undefined" 0 0)
      (Utilities|FlowControl|Delay 0.5)
      (Audio|PlaySound2D "/Game/Assets/SFX/misc_outside_noises/powerup_dropping_sound_Cue.powerup_dropping_sound_Cue" 1.0 1.0 0.0 0 0))
    (Variables|Default|Setready false)
    (CallFunction|Reset)
    (bind _buttonpushed (Timeline|ButtonPushed PlayFromStart)
      (:Update
        (Rendering|Material|SetScalarParameterValue "/Game/Assets/Materials/MPC_WorldOffset.MPC_WorldOffset" "PushButton" _buttonpushed :!class /Script/Engine.KismetMaterialLibrary)))))

(event Custom|Reset
  (bind _button (Variables|Default|GetButton))
  ;[1 1 1] Color Stuff
  (Rendering|Material|SetMaterial _button 0 "/Game/Assets/Materials/M_RedButton.M_RedButton")
  (Utilities|FlowControl|Delay (/ (Variables|Default|GetAirdropTimerTimeDelay) 2.0))
  (Rendering|Material|SetMaterial _button 0 "/Game/Assets/Materials/M_YellowButton.M_YellowButton")
  (Utilities|FlowControl|Delay (/ (Variables|Default|GetAirdropTimerTimeDelay) 2.0))
  (Rendering|Material|SetMaterial _button 0 "/Game/Assets/Materials/M_GreenButton.M_GreenButton")
  (Variables|Default|Setready true))

(event EventBeginPlay
  ;[1 1 1] Color Stuff
  (CallFunction|Reset))

(fn ConstructionScript)