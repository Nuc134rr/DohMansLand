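; BP_TrainTracks is a map item that builds a train track with station meshes along an editable spline.
; Its construction script adds a spline mesh segment between each pair of Track points, using their local locations and tangents to follow the curve.
; It then places an enlarged static mesh for each Stations entry, treating the value as a constant-velocity time along the spline.
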(fn ConstructionScript
  (bind _track (Variables|Default|GetTrack))
  (Utilities|FlowControl|Sequence
    (:then_0
      (for _index (range 0 (- (Spline|GetNumberOfSplinePoints (Variables|Default|GetTrack)) 2))
        (bind _returnvalue (AddComponent|AddSplineMeshComponent false))
        (SplineMesh|SetStartandEnd _returnvalue (.Location (Spline|GetLocationandTangentatSplinePoint _track _index "Local")) (.Tangent (Spline|GetLocationandTangentatSplinePoint _track _index "Local")) (.Location (Spline|GetLocationandTangentatSplinePoint _track (+ _index 1) "Local")) (.Tangent (Spline|GetLocationandTangentatSplinePoint _track (+ _index 1) "Local")) true :!class /Script/Engine.SplineMeshComponent)
        (Transformation|AttachComponentToComponent _returnvalue (Variables|Default|GetDefaultSceneRoot) "None" "KeepRelative" "KeepRelative" "KeepRelative" true)))
    (:then_1
      (for _array_element (Variables|Default|GetStations)
        (AddComponent|AddStaticMeshComponent false (Math|Transform|MakeTransform (Spline|GetLocationatTime (Variables|Default|GetTrack) _array_element "Local" true) "0, 0, 0" "3.000000,3.000000,3.000000"))))))