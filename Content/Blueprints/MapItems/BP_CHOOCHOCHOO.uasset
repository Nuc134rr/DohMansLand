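; Train actor that drives its carts and spinning wheels around a looping chain of track splines, taken from BP_Craine actors ordered by station number.
; TrainStopped advances the segment and picks one of four speed-profile timelines based on whether the previous or current station is a stop.
; Timeline updates feed MoveTrainCarts, which spaces points backward along the reversed splines, wrapping onto the previous segment and aiming each using its neighbour.
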(event Custom|Move%20Object
  ;[0.6781 0 1] Set the play rate for varibles on how fast the train to move, timeline determines the velocity at the spline, plays the function that calulates the distance between train carts
  (Components|Timeline|SetPlayRate (Variables|Default|GetStopAtStation) (/ 1.0 (Variables|Default|GetTime%20to%20complete%20%28in%20Seconds%29)))
  (CallFunction|TrainStopped))

(event Custom|WheelsRotation
  ;[1 0 0.08366] Handles the rotation of the wheels
  (Transformation|AddLocalRotation (Variables|Default|GetWheels) (Math|Rotator|MakeRotator 0.0 (Variables|Default|GetTime%20To%20Complete%20%28In%20Seconds%29) 0.0) false false))

(event Custom|MoveTrain
  (params (Alpha :type Float%20%28double-precision%29))
  (bind _track_position_these_nuts (Variables|Default|GetTrack%20Position%20these%20nuts))
  (bind _spline_ref (Variables|Default|GetSpline%20REF))
  (bind _output (Utilities|Array|Get(acopy) _spline_ref _track_position_these_nuts))
  ;[0 1 0.328] Gets spline length and spline ID
  (CallFunction|MoveTrainCarts (Math|Float|Lerp 0.0 (Spline|GetSplineLength (Variables|/Game/Blueprints/MapItems/BP_Craine.BP_Craine_C|GetTraintracks _output)) Alpha) (Variables|/Game/Blueprints/MapItems/BP_Craine.BP_Craine_C|GetTraintracks _output))
  (CallFunction|WheelsRotation))

(event Custom|Train%20Stopped
  ;[0.04493 0 1] Deciding what timeline to use
  (bind _output_get (Variables|Default|SetSpeedUp (!= (Utilities|Array|FindItem (Variables|Default|GetStopAtStations) (Variables|Default|GetTrack%20Position%20these%20nuts)) -1)))
  (if _output_get
    (Utilities|Array|RemoveIndex (Variables|Default|GetStopAtStations) (Variables|Default|GetTrack%20Position%20these%20nuts)))
  (if (< (Variables|Default|GetTrack%20Position%20these%20nuts) (- (Utilities|Array|Length (Variables|Default|GetSpline%20REF)) 1)) ; Add or Loop To Next INT
    (Math|Integer|IncrementInt (Variables|Default|GetTrack%20Position%20these%20nuts)
      (:%20%20
        _))
    (else
      (Variables|Default|SetTrack%20Position%20these%20nuts 0)))
  (if (!= (Utilities|Array|FindItem (Variables|Default|GetStopAtStations) (Variables|Default|GetTrack%20Position%20these%20nuts)) -1)
    (Components|Timeline|PlayfromStart (select (Variables|Default|GetSpeedUp) (Variables|Default|GetStopAtStation) (Variables|Default|GetSlowDown)))
    (else
      (Components|Timeline|PlayfromStart (select (Variables|Default|GetSpeedUp) (Variables|Default|GetSpeedingUp) (Variables|Default|GetContinuning%20))))))

(event EventBeginPlay
  ;[0.1166 0.19 1] Get points in the train to make array and use for math later
  (bind _outactors (Actor|GetAllActorsOfClass "/Game/Blueprints/MapItems/BP_Craine.BP_Craine_C"))
  (for _array_element _outactors
    (Utilities|Array|SetArrayElem (Variables|Default|GetSpline%20REF) (Variables|/Game/Blueprints/MapItems/BP_Craine.BP_Craine_C|GetStationNumber _array_element) _array_element true))
  (CallFunction|MoveObject)
  (Variables|Default|SetPoint%20Array (Utilities|Array|MakeArray (Variables|Default|GetPoint%201) (Variables|Default|GetPoint%202) (Variables|Default|GetPoint%203) (Variables|Default|GetPoint%205) (Variables|Default|GetPoint%206) (Variables|Default|GetPoint%207) (Variables|Default|GetPoint%208) (Variables|Default|GetPoint%204))))

(fn ConstructionScript)

(fn MoveTrainCarts
  (params (Point%20on%20lenght :type Float%20%28double-precision%29) (Spline%20deez%20nutz :type Spline%20Component%20Object%20Reference))
  (bind _track_position_these_nuts (Variables|Default|GetTrack%20Position%20these%20nuts))
  (bind _spline_ref (Variables|Default|GetSpline%20REF))
  (bind _returnvalue (Utilities|Array|Length _spline_ref))
  (bind _returnvalue_2 (== _track_position_these_nuts 0))
  (bind _returnvalue_3 (- _track_position_these_nuts 1))
  (bind _returnvalue_4 (- _returnvalue 1))
  (bind _returnvalue_5 (Math|Integer|SelectInt _returnvalue_4 _returnvalue_3 _returnvalue_2))
  (bind _output (Utilities|Array|Get(acopy) _spline_ref _returnvalue_5))
  (bind _traintracks (Variables|/Game/Blueprints/MapItems/BP_Craine.BP_Craine_C|GetTraintracks _output))
  ;[0.2127 0 1] Set the position of each point and rotation
  (for (_array_element _array_index) (Variables|Default|GetPoint%20Array)
    (if (> (- (Utilities|Array|Length (Variables|Default|GetPoint%20Array)) 1) _array_index) ; Prevents Error
      (Transformation|SetWorldTransform _array_element (Math|Transform|MakeTransform (Math|Vector|MakeVector (.x (Spline|GetLocationatDistanceAlongSpline (select (< (- Point%20on%20lenght (* _array_index (Variables|Default|GetDistanceBetweenCarts))) 0.0) _traintracks Spline%20deez%20nutz) (* (- 1.0 (/ (Math|Float|SelectFloat (+ (- Point%20on%20lenght (* _array_index (Variables|Default|GetDistanceBetweenCarts))) (Spline|GetSplineLength _traintracks)) (- Point%20on%20lenght (* _array_index (Variables|Default|GetDistanceBetweenCarts))) (< (- Point%20on%20lenght (* _array_index (Variables|Default|GetDistanceBetweenCarts))) 0.0)) (Spline|GetSplineLength (select (< (- Point%20on%20lenght (* _array_index (Variables|Default|GetDistanceBetweenCarts))) 0.0) _traintracks Spline%20deez%20nutz)))) (Spline|GetSplineLength (select (< (- Point%20on%20lenght (* _array_index (Variables|Default|GetDistanceBetweenCarts))) 0.0) _traintracks Spline%20deez%20nutz))) "World")) (.y (Spline|GetLocationatDistanceAlongSpline (select (< (- Point%20on%20lenght (* _array_index (Variables|Default|GetDistanceBetweenCarts))) 0.0) _traintracks Spline%20deez%20nutz) (* (- 1.0 (/ (Math|Float|SelectFloat (+ (- Point%20on%20lenght (* _array_index (Variables|Default|GetDistanceBetweenCarts))) (Spline|GetSplineLength _traintracks)) (- Point%20on%20lenght (* _array_index (Variables|Default|GetDistanceBetweenCarts))) (< (- Point%20on%20lenght (* _array_index (Variables|Default|GetDistanceBetweenCarts))) 0.0)) (Spline|GetSplineLength (select (< (- Point%20on%20lenght (* _array_index (Variables|Default|GetDistanceBetweenCarts))) 0.0) _traintracks Spline%20deez%20nutz)))) (Spline|GetSplineLength (select (< (- Point%20on%20lenght (* _array_index (Variables|Default|GetDistanceBetweenCarts))) 0.0) _traintracks Spline%20deez%20nutz))) "World")) (+ (.z (Spline|GetLocationatDistanceAlongSpline (select (< (- Point%20on%20lenght (* _array_index (Variables|Default|GetDistanceBetweenCarts))) 0.0) _traintracks Spline%20deez%20nutz) (* (- 1.0 (/ (Math|Float|SelectFloat (+ (- Point%20on%20lenght (* _array_index (Variables|Default|GetDistanceBetweenCarts))) (Spline|GetSplineLength _traintracks)) (- Point%20on%20lenght (* _array_index (Variables|Default|GetDistanceBetweenCarts))) (< (- Point%20on%20lenght (* _array_index (Variables|Default|GetDistanceBetweenCarts))) 0.0)) (Spline|GetSplineLength (select (< (- Point%20on%20lenght (* _array_index (Variables|Default|GetDistanceBetweenCarts))) 0.0) _traintracks Spline%20deez%20nutz)))) (Spline|GetSplineLength (select (< (- Point%20on%20lenght (* _array_index (Variables|Default|GetDistanceBetweenCarts))) 0.0) _traintracks Spline%20deez%20nutz))) "World")) 3e+02)) (Math|Rotator|FindLookatRotation (Transformation|GetWorldLocation (Utilities|Array|Get(acopy) (Variables|Default|GetPoint%20Array) (+ _array_index 1))) (Transformation|GetWorldLocation _array_element)) "1.000000,1.000000,1.000000") false false)
      (else
        (Transformation|SetWorldTransform _array_element (Math|Transform|MakeTransform (Math|Vector|MakeVector (.x (Spline|GetLocationatDistanceAlongSpline (select (< (- Point%20on%20lenght (* _array_index (Variables|Default|GetDistanceBetweenCarts))) 0.0) _traintracks Spline%20deez%20nutz) (* (- 1.0 (/ (Math|Float|SelectFloat (+ (- Point%20on%20lenght (* _array_index (Variables|Default|GetDistanceBetweenCarts))) (Spline|GetSplineLength _traintracks)) (- Point%20on%20lenght (* _array_index (Variables|Default|GetDistanceBetweenCarts))) (< (- Point%20on%20lenght (* _array_index (Variables|Default|GetDistanceBetweenCarts))) 0.0)) (Spline|GetSplineLength (select (< (- Point%20on%20lenght (* _array_index (Variables|Default|GetDistanceBetweenCarts))) 0.0) _traintracks Spline%20deez%20nutz)))) (Spline|GetSplineLength (select (< (- Point%20on%20lenght (* _array_index (Variables|Default|GetDistanceBetweenCarts))) 0.0) _traintracks Spline%20deez%20nutz))) "World")) (.y (Spline|GetLocationatDistanceAlongSpline (select (< (- Point%20on%20lenght (* _array_index (Variables|Default|GetDistanceBetweenCarts))) 0.0) _traintracks Spline%20deez%20nutz) (* (- 1.0 (/ (Math|Float|SelectFloat (+ (- Point%20on%20lenght (* _array_index (Variables|Default|GetDistanceBetweenCarts))) (Spline|GetSplineLength _traintracks)) (- Point%20on%20lenght (* _array_index (Variables|Default|GetDistanceBetweenCarts))) (< (- Point%20on%20lenght (* _array_index (Variables|Default|GetDistanceBetweenCarts))) 0.0)) (Spline|GetSplineLength (select (< (- Point%20on%20lenght (* _array_index (Variables|Default|GetDistanceBetweenCarts))) 0.0) _traintracks Spline%20deez%20nutz)))) (Spline|GetSplineLength (select (< (- Point%20on%20lenght (* _array_index (Variables|Default|GetDistanceBetweenCarts))) 0.0) _traintracks Spline%20deez%20nutz))) "World")) (+ (.z (Spline|GetLocationatDistanceAlongSpline (select (< (- Point%20on%20lenght (* _array_index (Variables|Default|GetDistanceBetweenCarts))) 0.0) _traintracks Spline%20deez%20nutz) (* (- 1.0 (/ (Math|Float|SelectFloat (+ (- Point%20on%20lenght (* _array_index (Variables|Default|GetDistanceBetweenCarts))) (Spline|GetSplineLength _traintracks)) (- Point%20on%20lenght (* _array_index (Variables|Default|GetDistanceBetweenCarts))) (< (- Point%20on%20lenght (* _array_index (Variables|Default|GetDistanceBetweenCarts))) 0.0)) (Spline|GetSplineLength (select (< (- Point%20on%20lenght (* _array_index (Variables|Default|GetDistanceBetweenCarts))) 0.0) _traintracks Spline%20deez%20nutz)))) (Spline|GetSplineLength (select (< (- Point%20on%20lenght (* _array_index (Variables|Default|GetDistanceBetweenCarts))) 0.0) _traintracks Spline%20deez%20nutz))) "World")) 3e+02)) "0, 0, 0" "1.000000,1.000000,1.000000") false false)))))