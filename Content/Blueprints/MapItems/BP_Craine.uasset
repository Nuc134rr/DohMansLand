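; BP_Craine is a map item that lays a deformed mesh along an editable spline named Traintracks, likely crane rails.
; The construction script adds one spline mesh component per spline segment, attached to the root.
; Each segment takes its start and end from the local location and tangent of neighboring spline points.
; The event graph holds no runtime logic.
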(event EventBeginPlay)

(event Collision|EventActorBeginOverlap
  (params (OtherActor :type Actor%20Object%20Reference)))

(event EventTick
  (params (DeltaSeconds :type Float%20%28single-precision%29)))

(fn ConstructionScript
  (bind _traintracks (Variables|Default|GetTraintracks))
  (for _index (range 0 (- (Spline|GetNumberOfSplinePoints (Variables|Default|GetTraintracks)) 2))
    (bind _returnvalue (AddComponent|AddSplineMeshComponent false))
    (SplineMesh|SetStartandEnd _returnvalue (Math|Vector|MakeVector (.x (.Location (Spline|GetLocationandTangentatSplinePoint _traintracks _index "Local"))) (.y (.Location (Spline|GetLocationandTangentatSplinePoint _traintracks _index "Local"))) (.z (.Location (Spline|GetLocationandTangentatSplinePoint _traintracks _index "Local")))) (.Tangent (Spline|GetLocationandTangentatSplinePoint _traintracks _index "Local")) (Math|Vector|MakeVector (.x (.Location (Spline|GetLocationandTangentatSplinePoint _traintracks (+ _index 1) "Local"))) (.y (.Location (Spline|GetLocationandTangentatSplinePoint _traintracks (+ _index 1) "Local"))) (.z (.Location (Spline|GetLocationandTangentatSplinePoint _traintracks (+ _index 1) "Local")))) (.Tangent (Spline|GetLocationandTangentatSplinePoint _traintracks (+ _index 1) "Local")) true :!class /Script/Engine.SplineMeshComponent)
    (Transformation|AttachComponentToComponent _returnvalue (Variables|Default|GetDefaultSceneRoot) "None" "KeepRelative" "KeepRelative" "KeepRelative" true)))