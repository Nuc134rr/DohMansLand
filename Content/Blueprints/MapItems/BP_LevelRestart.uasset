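; BP_LevelRestart is a touch restart button that resets the level when every instance of it is held at the same time.
; Touch begin and end on RestartButton toggle each instance's HasBeenPressed flag.
; On each press, CheckForReset scans all BP_LevelRestart actors, stopping at the first unpressed one.
; If all are pressed, it tells the DohMansLand game mode to reset the level and remove all projectiles.
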(event OnInputTouchEnd(RestartButton)
  (params (FingerIndex :type ETouchIndex%20Enum :default "Touch1") (TouchedComponent :type Primitive%20Component%20Object%20Reference))
  (Variables|Default|SetbHasBeenPressed false))

(event OnInputTouchBegin(RestartButton)
  (params (FingerIndex :type ETouchIndex%20Enum :default "Touch1") (TouchedComponent :type Primitive%20Component%20Object%20Reference))
  (bind _returnvalue (CallFunction|GetDohMansLandGameMode))
  (Variables|Default|SetbHasBeenPressed true)
  (bind _bshouldreset (CallFunction|CheckforReset))
  (if _bshouldreset
    (Default|CallLevelReset _returnvalue)
    (Default|RemoveAllProjectiles _returnvalue)))

(event Collision|EventActorBeginOverlap
  (params (OtherActor :type Actor%20Object%20Reference)))

(event EventTick
  (params (DeltaSeconds :type Float%20%28single-precision%29)))

(fn ConstructionScript)

(fn CheckforReset
  (bind _outactors (Actor|GetAllActorsOfClass "BP_LevelRestart_C"))
  (bind _array_element (Utilities|Array|ForEachLoopwithBreak _outactors :!label _label)
    (:LoopBody
      (if (Variables|BP_LevelRestart_C|GetbHasBeenPressed _array_element)
        (LocalVariables|SetLShouldReset true)
        (else
          (LocalVariables|SetLShouldReset false)
          (goto _label Break))))
    (:Completed
      (return (LocalVariables|GetLShouldReset)))))