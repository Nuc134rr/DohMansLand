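; Blueprint actor that handles screen and audio fade transitions when the level starts and when it resets.
; On BeginPlay it fades the player camera in and binds its fade-out event to the game mode's level-reset event.
; The fade-out runs over a configurable duration, then asks the game mode to reopen the level one second before the fade completes.
; An explosion sound and emitter spawn are left unconnected.
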(event Custom|Begin%20Fade%20out
  ;[1 1 1] Camera Fade in when level starts and fade out when one take remaining and resets level
  (CameraFades|StartCameraFade :self (Game|GetPlayerCameraManager 0) :ToAlpha 2.0 :Duration (Variables|Default|GetFadeDuration) :bShouldFadeAudio true)
  (Utilities|FlowControl|Delay (- (Variables|Default|GetFadeDuration) 1.0))
  (Default|OpenLevel (CallFunction|GetDohMansLandGameMode)))

(event EventBeginPlay
  ;[1 1 1] Camera Fade in when level starts and fade out when one take remaining and resets level
  (CameraFades|StartCameraFade :self (Game|GetPlayerCameraManager 0) :FromAlpha 1.5 :Duration 3.0 :bShouldFadeAudio true)
  (EventDispatchers|BindEventtoLevelReset (CallFunction|GetDohMansLandGameMode) (delegate Custom|Begin%20Fade%20out)))

(fn ConstructionScript)