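; BP_Train is a train actor that travels along the spline of a BP_TrainPathSpline actor found in the level at BeginPlay.
; MoveObject plays a timeline with its rate set from TimeToCompleteInSeconds, mapping its track to distance along the spline.
; Each update sets the train's location and rotation from that distance, sampled in the spline's local space but applied as a world transform.
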(event Custom|Move%20Object
  (bind _spline_ref (Variables|Default|GetSpline%20REF))
  (bind _spline (Variables|/Game/Blueprints/MapItems/BP_TrainPathSpline.BP_TrainPathSpline_C|GetSpline _spline_ref))
  (Components|Timeline|SetPlayRate (Variables|Default|GetTMove%20Object) (/ 1.0 (Variables|Default|GetTime%20to%20complete%20%28in%20Seconds%29)))
  (bind _move_track (Timeline|TMove%20Object Play)
    (:Update
      (Transformation|SetActorTransform (Math|Transform|MakeTransform (Spline|GetLocationatDistanceAlongSpline _spline (Math|Float|Lerp 0.0 (Spline|GetSplineLength (Variables|/Game/Blueprints/MapItems/BP_TrainPathSpline.BP_TrainPathSpline_C|GetSpline (Variables|Default|GetSpline%20REF))) _move_track) "Local") (Spline|GetRotationatDistanceAlongSpline _spline (Math|Float|Lerp 0.0 (Spline|GetSplineLength (Variables|/Game/Blueprints/MapItems/BP_TrainPathSpline.BP_TrainPathSpline_C|GetSpline (Variables|Default|GetSpline%20REF))) _move_track) "Local") "1.000000,1.000000,1.000000")))))

(event EventBeginPlay
  (bind _returnvalue (Actor|GetActorOfClass "/Game/Blueprints/MapItems/BP_TrainPathSpline.BP_TrainPathSpline_C"))
  (Variables|Default|SetSpline%20REF _returnvalue)
  (CallFunction|MoveObject)
  (CallFunction|MoveObject))

(fn ConstructionScript)