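; BP_Helicopter is a touch-interactive helicopter map item whose HeliProps component the player turns by dragging a finger.
; Touching either Box or Box1 stores the finger index, sets RotateBlades and prints a debug message.
; While that finger is pressed, Tick traces under it and sets HeliProps to face the hit point in yaw only.
; RotateBlades is never cleared, so Tick keeps polling that finger index after release.
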(event OnInputTouchBegin(Box1)
  (params (FingerIndex :type ETouchIndex%20Enum :default "Touch1") (TouchedComponent :type Primitive%20Component%20Object%20Reference))
  (Variables|Default|SetbRotateBlades true)
  (Variables|Default|SetHeliIndex FingerIndex)
  (Development|PrintString "Hello"))

(event OnInputTouchBegin(Box)
  (params (FingerIndex :type ETouchIndex%20Enum :default "Touch1") (TouchedComponent :type Primitive%20Component%20Object%20Reference))
  (Variables|Default|SetbRotateBlades true)
  (Variables|Default|SetHeliIndex FingerIndex)
  (Development|PrintString "Hello"))

(event EventTick
  (params (DeltaSeconds :type Float%20%28single-precision%29))
  (bind _heliprops (Variables|Default|GetHeliProps))
  (if (Variables|Default|GetbRotateBlades)
    (if (.bIsCurrentlyPressed (Class|PlayerController|GetInputTouchState (Game|GetPlayerController 0) (Variables|Default|GetHeliIndex)))
      (Transformation|SetWorldRotation _heliprops (Math|Rotator|MakeRotator 0.0 0.0 (.yaw (Math|Rotator|FindLookatRotation (Transformation|GetWorldLocation _heliprops) (.Location (Collision|BreakHitResult (.HitResult (Class|PlayerController|GetHitResultUnderFingerbyChannel (Game|GetPlayerController 0) (Variables|Default|GetHeliIndex) "TraceTypeQuery1" true))))))) false false))))

(fn ConstructionScript)