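; BP_LegoBrick is a map item that shows a Lego brick with a randomized tank color and orientation.
; On BeginPlay it puts a dynamic material on its mesh, sets Color0 to a random tank color from the DohMansLand game mode, and randomizes the mesh's yaw.
; The construction script creates a similarly colored material instance but never assigns it to the mesh.
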(event EventBeginPlay
  (bind _returnvalue (Rendering|Material|CreateDynamicMaterialInstance (Variables|Default|GetStaticMesh) 0 "/Game/Assets/Materials/M_LegobrickRed_Inst.M_LegobrickRed_Inst" "None" :!class /Script/Engine.PrimitiveComponent))
  (Rendering|Material|SetVectorParameterValue _returnvalue "Color0" (.tankcolor (Utilities|Array|Get(acopy) (Variables|/Game/Blueprints/Player/BP_DohMansLand_GameMode.BP_DohMansLand_GameMode_C|GetTank%20Variables (CallFunction|GetDohMansLandGameMode)) (Math|Random|RandomInteger 5))) :!class /Script/Engine.MaterialInstanceDynamic)
  (Transformation|SetWorldRotation (Variables|Default|GetStaticMesh) (Math|Rotator|MakeRotator 0.0 0.0 (Math|Random|RandomFloatinRange 0.0 1.8e+02)) false false))

(fn ConstructionScript
  (bind _returnvalue (Rendering|Material|CreateDynamicMaterialInstance "/Game/Assets/Materials/M_LegobrickRed_Inst.M_LegobrickRed_Inst" "None" "None" :!class /Script/Engine.KismetMaterialLibrary))
  (Rendering|Material|SetVectorParameterValue _returnvalue "Color0" (.tankcolor (Utilities|Array|Get(acopy) (Variables|/Game/Blueprints/Player/BP_DohMansLand_GameMode.BP_DohMansLand_GameMode_C|GetTank%20Variables (CallFunction|GetDohMansLandGameMode)) (Math|Random|RandomInteger 5))) :!class /Script/Engine.MaterialInstanceDynamic))