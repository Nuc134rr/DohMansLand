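; Spectator screen map item: an iPad mesh that switches between player views when touched.
; Each touch clears the previous capture's texture target, then advances through six RenderTargets slots, looping past invalid entries.
; The selected capture alone renders into the shared RT_iPadScreen, fed to the screen's dynamic material.
; The construction script creates that material with AICONGreen as the initial image.
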(event OnInputTouchBegin(iPad)
  (params (FingerIndex :type ETouchIndex%20Enum :default "Touch1") (TouchedComponent :type Primitive%20Component%20Object%20Reference))
  (CallFunction|UpdateDisplay))

(event Custom|UpdateDisplay
  (bind _currentplayer (Variables|Default|GetCurrentPlayer)
    (:then
      (Variables|/Script/Engine.SceneCaptureComponent2D|SetTextureTarget _currentplayer 0))
    (:else
      _))
  (Variables|Default|SetCurrentIndex (select (== (+ (Variables|Default|GetCurrentIndex) 1) 6) 0 (+ (Variables|Default|GetCurrentIndex) 1)) :!label _label)
  (Utilities|IsValid (.Value (Utilities|Map|Find (Variables|Default|GetRenderTargets) (Variables|Default|GetCurrentIndex)))
    (:Is%20Valid
      (bind _output_get (Variables|Default|SetCurrentPlayer (.Value (Utilities|Map|Find (Variables|Default|GetRenderTargets) (Variables|Default|GetCurrentIndex)))))
      (bind _output_get_2 (Variables|/Script/Engine.SceneCaptureComponent2D|SetTextureTarget _output_get "/Game/Assets/Materials/iPad/RT_iPadScreen.RT_iPadScreen"))
      (Rendering|Material|SetTextureParameterValue (Variables|Default|GetIpadScreen) "RenderTarget" _output_get_2))
    (:Is%20Not%20Valid
      (goto _label))))

(fn ConstructionScript
  (bind _ipad (Variables|Default|GetiPad))
  (bind _returnvalue (Rendering|Material|CreateDynamicMaterialInstance _ipad 0 (Rendering|Material|GetMaterial _ipad 0) "None" :!class /Script/Engine.PrimitiveComponent))
  (bind _output_get (Variables|Default|SetIpadScreen _returnvalue))
  (Rendering|Material|SetTextureParameterValue _output_get "RenderTarget" "/Engine/EngineResources/AICON-Green.AICON-Green"))