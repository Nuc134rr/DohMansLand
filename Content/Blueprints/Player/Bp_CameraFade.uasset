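; Level-transition Blueprint that fades the camera and audio in at start and restarts the level when only one tank remains.
; BeginPlay starts the fade-in, while Tick uses a short Delay to repeatedly count BP_BaseTank actors.
; At a count of one, a DoOnce triggers the fade-out, waits, then reopens the current level by name.
; Explosion sound and emitter nodes are present but never run.
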(event EventTick
  (params (DeltaSeconds :type Float%20%28single-precision%29))
  (Utilities|FlowControl|Delay 0.2)
  (bind _outactors (Actor|GetAllActorsOfClass "/Game/Blueprints/Player/BP_BaseTank.BP_BaseTank_C"))
  ;[1 1 1] Camera Fade in when level starts and fade out when one take remaining and resets level
  (if (== (Utilities|Array|Length _outactors) 1)
    (Utilities|FlowControl|DoOnce false
      (:Completed
        (Utilities|FlowControl|DelayUntilNextTick)
        (CameraFades|StartCameraFade :self (Game|GetPlayerCameraManager 0) :ToAlpha 2.0 :Duration 2.0 :bShouldFadeAudio true)
        (Utilities|FlowControl|Delay 3.0)
        (bind _returnvalue (Game|GetCurrentLevelName true))
        (Game|OpenLevel(byName) (Utilities|String|StringToName _returnvalue))))))

(event EventBeginPlay
  ;[1 1 1] Camera Fade in when level starts and fade out when one take remaining and resets level
  (CameraFades|StartCameraFade :self (Game|GetPlayerCameraManager 0) :FromAlpha 1.5 :Duration 3.0 :bShouldFadeAudio true))

(fn ConstructionScript)