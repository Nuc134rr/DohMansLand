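; Game mode for Doh Man's Land, a last-tank-standing match that starts the theme music and sets resolution and screen percentage through console commands on BeginPlay.
; CheckForWin counts players in the Playing state; a lone survivor gets stored as winner, projectiles are cleared, confetti fires in their tank color and GameOver is broadcast.
; OpenLevel fades to white and reloads the current level, delaying first unless triggered by a reset.
; The tank-count music switch is unconnected.
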(event Custom|OpenLevel
  ;[1 1 0.3] Level Reset
  ;;[0.2 0.2 0.2] Checks to see if there's one tank left
  (if (Variables|Default|GetbFromLevelReset)
    _
    (else
      (Utilities|FlowControl|Delay 7.0)))
  (CameraFades|StartCameraFade (Game|GetPlayerCameraManager 0) 0.0 1.0 3.0 "(R=1.000000,G=1.000000,B=1.000000,A=1.000000)" true true)
  (Utilities|FlowControl|Delay 3.0)
  (Game|OpenLevel(byName) (Variables|Default|GetCurrentLevelName)))

(event Custom|RemoveAllProjectiles
  ;[1 1 0.3] Level Reset
  ;;[0.2 0.2 0.2] Removes all projectiles on level reset
  (bind _outactors (Actor|GetAllActorsOfClass "/Game/Projectiles/BP_BaseProjectile.BP_BaseProjectile_C"))
  (for _array_element _outactors
    (Default|RemoveandDestroy _array_element _array_element)))

(event EventBeginPlay
  ;[0.3 1 1] Begin Play
  (Utilities|FlowControl|Sequence
    (:then_0
      (bind _returnvalue (Settings|GetGameUserSettings))
      (Development|ExecuteConsoleCommand (Utilities|String|Append "r.setres " (Utilities|String|ToString(Integer) (.x (Class|GameUserSettings|GetDesktopResolution _returnvalue))) "x" (Utilities|String|ToString(Integer) (.y (Class|GameUserSettings|GetDesktopResolution _returnvalue))) " f") 0)
      (Development|ExecuteConsoleCommand "r.ScreenPercentage 50" 0))
    (:then_2
      (Audio|Components|Audio|FadeIn (Variables|Default|GetMainTheme6TanksRemaining%20) 3.0 5.0 1.0 "Linear" :!class /Script/Engine.AudioComponent))
    (:then_3
      (bind _returnvalue_2 (Game|GetCurrentLevelName true))
      (Variables|Default|SetCurrentLevelName (Utilities|String|StringToName _returnvalue_2)))
    (:then_4
      (EventDispatchers|BindEventtoGameOver (EventDispatchers|CreateEvent :!event Custom|OpenLevel))
      (EventDispatchers|BindEventtoGameOver (EventDispatchers|CreateEvent :!event Custom|RemoveAllProjectiles)))))

(fn ConstructionScript)

(fn CheckforWin
  (bind _alivetanks (LocalVariables|GetAliveTanks))
  (bind _output (Utilities|Array|Get(acopy) _alivetanks))
  (bind _outactors (Actor|GetAllActorsOfClass "/Game/Blueprints/Player/BP_Player.BP_Player_C"))
  (for _array_element _outactors
    (switch Utilities|FlowControl|Switch|SwitchonEPlayerState (Variables|/Game/Blueprints/Player/BP_Player.BP_Player_C|GetEPlayerState _array_element)
      (:NewEnumerator1
        (Utilities|Array|Add (LocalVariables|GetAliveTanks) _array_element))))
  (if (== (Utilities|Array|Length (LocalVariables|GetAliveTanks)) 1)
    (Variables|/Game/Blueprints/Player/BP_Player.BP_Player_C|SetbHasWon (Utilities|Array|Get(acopy) (LocalVariables|GetAliveTanks)) true)
    (bind _outactors_2 (Actor|GetAllActorsOfClass "/Game/Blueprints/Player/BP_Player.BP_Player_C"))
    (for _array_element_2 _outactors_2
      (Default|ClearandRemoveTimer _array_element_2))
    (CallFunction|RemoveAllProjectiles)
    (Variables|/Game/Blueprints/Player/BP_DohMansLand_GameInstance.BP_DohMansLand_GameInstance_C|SetWinnerID (CallFunction|GetDohMansLandGameInstance) (Variables|/Game/Blueprints/Player/BP_Player.BP_Player_C|GetPlayerIndex _output))
    (Audio|SpawnSound2D "/Game/Assets/SFX/misc_outside_noises/Victory_sounds/victory_sound_Cue.victory_sound_Cue" 1.0 1.0 0.0 0)
    (bind _outactors_3 (Actor|GetAllActorsOfClass "/Game/Blueprints/MapItems/BP_Confetti_Spawner.BP_Confetti_Spawner_C"))
    (for _array_element_3 _outactors_3
      (Default|FireConfetti _array_element_3 (.tankcolor (Variables|/Game/Blueprints/Player/BP_Player.BP_Player_C|GetTankVariables _output))))
    (Default|CallGameOver)
    (return)
    (else
      (return))))