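; BP_PlayerTwoTank is the second player's tank, a pawn driven by dedicated P2 input bindings.
; Axis inputs yaw the body mesh and copy its rotation to the actor, yaw the turret separately, and feed forward/backward input to CharacterMovement.
; Fire spawns a projectile at the barrel's location with the turret's rotation, owned by the tank.
; Rotation uses a fixed step per input event, without delta-time scaling.
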(event Input|ActionEvents|InputActionFireP2
  (params (Key :type Key%20Structure :default "None"))
  ;[0.2 0.2 0.2] Shoot (RShift)
  (:Pressed
    (Game|SpawnActorfromClass (Variables|Default|GetProjectileClass) (Math|Transform|MakeTransform (Transformation|GetWorldLocation (Variables|Default|GetBarrel)) (Transformation|GetWorldRotation (Variables|Default|GetTurret)) "1.000000,1.000000,1.000000") "Undefined" self 0)))

(event Input|AxisEvents|InputAxisRightP2
  (params (AxisValue :type Float%20%28single-precision%29))
  (bind _mesh (Variables|Character|GetMesh))
  ;[0.145 0.6838 1] Movement/Rotation
  ;;[0.2 0.2 0.2] Rotate the body of the tank (J and L)
  (Transformation|AddWorldRotation _mesh (Math|Rotator|MakeRotator 0.0 0.0 (* AxisValue 2.0)) false false)
  (Transformation|SetActorRotation (Transformation|GetWorldRotation _mesh)))

(event Input|AxisEvents|InputAxisAimRightP2
  (params (AxisValue :type Float%20%28single-precision%29))
  ;[0.145 0.6838 1] Movement/Rotation
  ;;[0.2 0.2 0.2] Rotate the Turret of the tank (U and O)
  (Transformation|AddWorldRotation (Variables|Default|GetTurret) (Math|Rotator|MakeRotator 0.0 0.0 (* AxisValue 2.0)) false false))

(event Input|AxisEvents|InputAxisUpP2
  (params (AxisValue :type Float%20%28single-precision%29))
  ;[0.145 0.6838 1] Movement/Rotation
  ;;[0.2 0.2 0.2] Move forward and backward (I and K)
  (Class|PawnMovementComponent|AddInputVector (Variables|Character|GetCharacterMovement) (* (Transformation|GetActorForwardVector) AxisValue) false))

(fn ConstructionScript)