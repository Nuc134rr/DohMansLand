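; Visual respawn countdown dial for its owning BP_BaseTank, tinted with that player's tank color from the game mode through dynamic materials.
; It eases its base in on BeginPlay, then a looping timer steps the dial through one full turn over the tank's respawn time.
; When the dial completes its turn or the tank's respawn timer handle is invalid, the base slides away and the actor destroys itself.
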(event Custom|TickTimer
  (bind _timerdial (Variables|Default|GetTimerDial))
  ;[0.2 0.2 0.2] Ticks the timer depending on the cooldown
  (Transformation|AddRelativeRotation _timerdial (Math|Rotator|MakeRotator 0.0 0.0 -6.0) false false)
  (if (Utilities|Time|IsValidTimerHandle (Variables|/Game/Blueprints/Player/BP_BaseTank.BP_BaseTank_C|GetRespawnTimerHandle (.AsBP%20Base%20Tank (Utilities|Casting|CastToBP_BaseTank (Components|GetOwner)))))
    (if (Math|Float|NearlyEqual(Float) (.yaw (Variables|/Script/Engine.SceneComponent|GetRelativeRotation _timerdial)) 0.0 3.0)
      (Components|MoveComponentTo (Variables|Default|GetTimerBase) "0,-4000.000000, 0" (Variables|/Script/Engine.SceneComponent|GetRelativeRotation (Variables|Default|GetTimerBase)) true true 1.0 false :!label _label)
      (Actor|DestroyActor))
    (else
      (Utilities|Time|ClearandInvalidateTimerbyHandle (Variables|Default|GetTimerHandle))
      (goto _label))))

(event Custom|StartTimer
  (bind _returnvalue (Utilities|Time|SetTimerbyEvent (delegate Custom|TickTimer) (/ (Variables|/Game/Blueprints/Player/BP_BaseTank.BP_BaseTank_C|GetRespawnTimer (.AsBP%20Base%20Tank (Utilities|Casting|CastToBP_BaseTank (Components|GetOwner)))) 6e+01) true))
  (Variables|Default|SetTimerHandle _returnvalue))

(event EventBeginPlay
  (bind _timerbase (Variables|Default|GetTimerBase))
  (CallFunction|StartTimer)
  (Components|MoveComponentTo _timerbase "0, 0, 0" (Variables|/Script/Engine.SceneComponent|GetRelativeRotation _timerbase) true true 1.0 false))

(fn ConstructionScript
  (bind _returnvalue (Components|GetOwner))
  (bind _returnvalue_2 (CallFunction|GetDohMansLandGameMode))
  (bind _asbp_base_tank (Utilities|Casting|CastToBP_BaseTank _returnvalue))
  (bind _tank_variables (Variables|/Game/Blueprints/Player/BP_DohMansLand_GameMode.BP_DohMansLand_GameMode_C|GetTank%20Variables _returnvalue_2))
  (bind _playerid (Variables|/Game/Blueprints/Player/BP_BaseTank.BP_BaseTank_C|GetPlayerID _asbp_base_tank))
  (bind _output (Utilities|Array|Get(acopy) _tank_variables _playerid))
  (Utilities|FlowControl|Sequence
    (:then_0
      (bind _returnvalue_3 (Rendering|Material|CreateDynamicMaterialInstance "/Game/Assets/Materials/M_MatteOff-WhitePlastic.M_MatteOff-WhitePlastic" "None" "None" :!class /Script/Engine.KismetMaterialLibrary))
      (Rendering|Material|SetMaterial (Variables|Default|GetTimerDial) 0 _returnvalue_3)
      (Rendering|Material|SetVectorParameterValue _returnvalue_3 "Color" (.tankcolor _output) :!class /Script/Engine.MaterialInstanceDynamic))
    (:then_1
      (bind _returnvalue_4 (Rendering|Material|CreateDynamicMaterialInstance (Variables|Default|GetTimerBase) 1 "/Game/Assets/Materials/M_Count.M_Count" "None" :!class /Script/Engine.PrimitiveComponent))
      (Rendering|Material|SetVectorParameterValue _returnvalue_4 "Color" (.tankcolor _output) :!class /Script/Engine.MaterialInstanceDynamic)
      (Rendering|Material|SetScalarParameterValue _returnvalue_4 "Alpha" 0.7 :!class /Script/Engine.MaterialInstanceDynamic))))