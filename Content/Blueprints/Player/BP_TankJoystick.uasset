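; Touch-driven 3D joystick actor, named for tank control, that tilts its stick toward the player's finger; the file shows only the visual rotation.
; Touching the Cylinder enables tracking, and Tick then repeats a visibility trace under that finger.
; The look-at rotation from the joystick transform cached at BeginPlay drives the stick, with pitch inverted and offset.
; The actor's touch-end event stops tracking and recenters the stick.
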(event OnInputTouchBegin(Cylinder)
  (params (FingerIndex :type ETouchIndex%20Enum :default "Touch1") (TouchedComponent :type Primitive%20Component%20Object%20Reference))
  (bind _returnvalue (Game|GetPlayerController 0))
  (bind _transform (Variables|Default|Gettransform))
  (bind _hitresult (Class|PlayerController|GetHitResultUnderFingerbyChannel _returnvalue FingerIndex "TraceTypeQuery1" true))
  (bind _returnvalue_2 (Math|Rotator|FindRelativeLookatRotation _transform (.location _hitresult)))
  (Variables|Default|Setable true)
  (Transformation|SetRelativeRotation (Variables|Default|Getstick) (Math|Rotator|MakeRotator (.roll _returnvalue_2) (+ (* (.pitch _returnvalue_2) -1.0) -55.0) (.yaw _returnvalue_2)) true false))

(event Custom|OnInputTouchEnd_Event
  (params (FingerIndex :type ETouchIndex%20Enum :default "Touch1") (TouchedActor :type Actor%20Object%20Reference))
  (Variables|Default|Setable false)
  (Transformation|SetRelativeRotation (Variables|Default|Getstick) "0, 0, 0" false false))

(event EventBeginPlay
  (EventDispatchers|BindEventtoOnInputTouchEnd (delegate Custom|OnInputTouchEnd_Event))
  (Variables|Default|Settransform (Transformation|GetWorldTransform (Variables|Default|GetJoystick))))

(event EventTick
  (params (DeltaSeconds :type Float%20%28single-precision%29))
  (if (Variables|Default|Getable)
    (Transformation|SetRelativeRotation (Variables|Default|Getstick) (Math|Rotator|MakeRotator (.roll (Math|Rotator|FindRelativeLookatRotation (Variables|Default|Gettransform) (.location (.HitResult (Class|PlayerController|GetHitResultUnderFingerbyChannel (Game|GetPlayerController 0) (stale OnInputTouchBegin(Cylinder) FingerIndex) "TraceTypeQuery1" true))))) (+ (* (.pitch (Math|Rotator|FindRelativeLookatRotation (Variables|Default|Gettransform) (.location (.HitResult (Class|PlayerController|GetHitResultUnderFingerbyChannel (Game|GetPlayerController 0) (stale OnInputTouchBegin(Cylinder) FingerIndex) "TraceTypeQuery1" true))))) -1.0) -55.0) (.yaw (Math|Rotator|FindRelativeLookatRotation (Variables|Default|Gettransform) (.location (.HitResult (Class|PlayerController|GetHitResultUnderFingerbyChannel (Game|GetPlayerController 0) (stale OnInputTouchBegin(Cylinder) FingerIndex) "TraceTypeQuery1" true)))))) true false)))

(fn ConstructionScript)