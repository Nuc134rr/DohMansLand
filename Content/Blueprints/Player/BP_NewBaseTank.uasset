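; Base tank pawn that drives, aims and fires, with powerups added as components.
; Axis input moves and turns the body while counter-rotating the turret, which eases to target yaw; Tick forwards changed tread speeds.
; Firing is limited by live projectile count and each projectile's fire rate, becoming confetti and a party horn after winning.
; Construction tints body, turret and treads with the tank color, using randomly seeded dynamic materials.
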(event Custom|RotateTurret
  (params (TargetRotation :type Float%20%28double-precision%29) (bResetZ :type Boolean))
  (bind _collision (Variables|Default|GetCollision))
  (bind _turret (Variables|Default|GetTurret))
  (bind _returnvalue (Transformation|GetRelativeTransform _collision))
  (bind _relativerotation (Variables|/Script/Engine.SceneComponent|GetRelativeRotation _turret))
  (bind _returnvalue_2 (Math|Transform|InverseTransformRotation _returnvalue (Math|Rotator|MakeRotator 0.0 0.0 TargetRotation)))
  (bind _returnvalue_3 (select bResetZ 0.0 (.yaw _returnvalue_2)))
  ;[0.3 1 1] MOVEMENT AND ROTATION
  ;;[0.2 0.2 0.2] Rotate the turret based on the spinner input
  (Components|MoveComponentTo _turret (Variables|/Script/Engine.SceneComponent|GetRelativeLocation _turret) (Math|Rotator|MakeRotator (.roll _relativerotation) (.pitch _relativerotation) _returnvalue_3) false false (Utilities|GetDistanceConvertedtoTime _returnvalue_3 (.yaw _relativerotation)) false))

(event Custom|RotateBody
  (params (AxisValue :type Float%20%28double-precision%29))
  (bind _turnspeed (Variables|Movement|GetTurnSpeed))
  (bind _returnvalue (* AxisValue _turnspeed))
  ;[0.3 1 1] MOVEMENT AND ROTATION
  ;;[0.2 0.2 0.2] Rotate the body while counterrotating the turret
  (Variables|Default|SetTreadSpeed (Math|Vector2D|MakeVector2D (.x (Variables|Default|GetTreadSpeed)) (* AxisValue -1.0)))
  (Class|Actor|AddActorWorldRotation (Math|Rotator|MakeRotator 0.0 0.0 _returnvalue))
  (Transformation|AddWorldRotation (Variables|Default|GetTurret) (Math|Rotator|MakeRotator 0.0 0.0 (* _returnvalue -1.0)) false false))

(event Custom|MoveTank
  (params (AxisValue :type Float%20%28double-precision%29))
  ;[0.3 1 1] MOVEMENT AND ROTATION
  ;;[0.2 0.2 0.2] Moves the tank forward
  (Variables|Default|SetTreadSpeed (Math|Vector2D|MakeVector2D AxisValue (.y (Variables|Default|GetTreadSpeed))))
  (Class|PawnMovementComponent|AddInputVector (Variables|Default|GetFloatingPawnMovement) (* AxisValue (Variables|Movement|GetMoveSpeed) -1.0 (Transformation|GetActorForwardVector)) false)
  (if (not (Math|Float|NearlyEqual(Float) 0.0 0.0 1e-06))
    (Utilities|FlowControl|DoOnce false :!label _label
      (:Completed
        (bind _returnvalue (Audio|SpawnSound2D (.movesound (Variables|Gameplay|GetTankVariables)) 1.0 1.0 0.0 0))
        (Variables|Default|SetMoveSound _returnvalue)))
    (else
      (Utilities|IsValid (Variables|Default|GetMoveSound)
        (:Is%20Valid
          (Audio|Components|Audio|Stop (Variables|Default|GetMoveSound))
          (goto _label Reset))))))

(event Custom|FireProjectile
  (bind _barrel (Variables|Default|GetBarrel))
  (bind _returnvalue (Transformation|GetWorldRotation _barrel))
  (bind _returnvalue_2 (Transformation|GetWorldLocation _barrel))
  (bind _returnvalue_3 (Math|Vector|GetForwardVector _returnvalue))
  (bind _returnvalue_4 (* 5e+01 _returnvalue_3))
  (bind _returnvalue_5 (+ _returnvalue_4 _returnvalue_2))
  ;[1 0.3 1] SHOOTING
  ;;[0.2 0.2 0.2] Shoots a projectile
  (if (not (>= (Utilities|Array|Length (Variables|Projectiles|GetActiveProjectiles)) (Variables|Projectiles|GetMaxProjectiles)))
    (Utilities|FlowControl|DoOnce false :!label _label
      (:Completed
        (Utilities|SpawnTurretParticles)
        (if (Variables|Default|GetbHasWon)
          (Audio|PlaySound2D "/Game/Assets/SFX/misc_outside_noises/Victory_sounds/Party_Horn_Cue.Party_Horn_Cue" 1.0 1.0 0.0 0 0)
          (else
            (bind _returnvalue_6 (Game|SpawnActorfromClass (Variables|Projectiles|GetProjectileClass) (Math|Transform|MakeTransform (Math|Vector|MakeVector (.x _returnvalue_5) (.y _returnvalue_5) (.z _returnvalue_5)) _returnvalue "1.000000,1.000000,1.000000") "Undefined" 0 self 0))
            (Utilities|Array|Add (Variables|Projectiles|GetActiveProjectiles) _returnvalue_6)
            (Audio|PlaySound2D (.shootsound (Variables|Gameplay|GetTankVariables)) 1.0 1.0 0.0 0 0)))
        (Utilities|FlowControl|Delay (Variables|/Game/Projectiles/BP_BaseProjectile.BP_BaseProjectile_C|GetFireRate _returnvalue_6))
        (goto _label Reset)))))

(event Custom|AddPowerup
  (params (Powerup :type AC%20Base%20Projectile%20Powerup%20Class%20Reference))
  (Game|AddComponentbyClass Powerup))

(event Custom|RemoveProjectile
  (params (Projectile :type BP%20Base%20Projectile%20Object%20Reference))
  ;[1 0.3 1] SHOOTING
  ;;[0.2 0.2 0.2] Removes projectiles when they fuck off and die
  (Utilities|Array|RemoveItem (Variables|Projectiles|GetActiveProjectiles) Projectile))

(event EventTick
  (params (DeltaSeconds :type Float%20%28single-precision%29))
  (bind _treadspeed (Variables|Default|GetTreadSpeed))
  (if (not (Utilities|Operators|EqualEqual (Variables|Default|GetTreadSpeed) (Variables|Default|GetPreviousTreads) 0.01))
    (Default|UpdateSpeeds (Variables|Default|GetTreads) (.y _treadspeed) (.x _treadspeed))
    (Variables|Default|SetPreviousTreads (Variables|Default|GetTreadSpeed))))

(event EventDestroyed
  (Actor|DestroyActor (Pawn|GetController)))

(fn ConstructionScript
  (for _index (range 0 2)
    (Utilities|SetTankDoh (Variables|Default|GetTankBase) _index false))
  (Utilities|SetTankDoh (Variables|Default|GetTurret) 0 false)
  (Variables|/Game/Blueprints/Generation/BP_TreadsComponent.BP_TreadsComponent_C|SetColor (Variables|Default|GetTreads) (.tankcolor (Variables|Gameplay|GetTankVariables))))