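; Player controller for DohMansLand that applies yaw input scaling at begin play and hosts hotkeys, apparently for testing.
; Releasing F sets fullscreen at desktop resolution through an r.setres console command.
; Number keys add fast-projectile or tank-speed powerup components to player one's pawn and print a message.
; On possess it starts the BT_TankAi behavior tree on an AI controller; an unconnected actor-count check never runs.
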(event EventBeginPlay
  ;[0.2 0.2 0.2] Set Yaw Scaling
  (Class|PlayerController|SetDeprecatedInputYawScale (Variables|Default|GetYawScaling)))

(event EventPossess
  (params (PossessedPawn :type Pawn%20Object%20Reference))
  (AI|RunBehaviorTree (AI|GetAIController (Variables|Default|GetAi_controller)) "/Game/Blueprints/AI/BT_TankAi.BT_TankAi"))

(event Input|KeyboardEvents|F
  (params (Key :type Key%20Structure :default "None"))
  (:Released
    (bind _returnvalue (Settings|GetGameUserSettings))
    (Development|ExecuteConsoleCommand (Utilities|String|Append "r.setres " (Utilities|String|ToString(Integer) (.x (Class|GameUserSettings|GetDesktopResolution _returnvalue))) "x" (Utilities|String|ToString(Integer) (.y (Class|GameUserSettings|GetDesktopResolution _returnvalue))) " f") 0)))

(event Input|KeyboardEvents|2
  (params (Key :type Key%20Structure :default "None"))
  (:Pressed
    (Game|AddComponentbyClass (CallFunction|GetPlayerOnePawn) "/Game/PowerupComponents/Movement/AC_TankSpeedPowerup.AC_TankSpeedPowerup_C")
    (Development|PrintString "Hello")))

(event Input|KeyboardEvents|9
  (params (Key :type Key%20Structure :default "None"))
  (:Pressed
    (Game|AddComponentbyClass (CallFunction|GetPlayerOnePawn) "/Game/PowerupComponents/Movement/AC_TankSpeedPowerup.AC_TankSpeedPowerup_C")
    (Development|PrintString "Speed")))

(event Input|KeyboardEvents|8
  (params (Key :type Key%20Structure :default "None"))
  (:Pressed
    (Game|AddComponentbyClass (CallFunction|GetPlayerOnePawn) "/Game/PowerupComponents/Weapons/ProjectileTypes/AC_FastProjectilesPowerup.AC_FastProjectilesPowerup_C")
    (Development|PrintString "Fast")))

(event Input|KeyboardEvents|3
  (params (Key :type Key%20Structure :default "None"))
  (:Pressed
    (Game|AddComponentbyClass (CallFunction|GetPlayerOnePawn) "/Game/PowerupComponents/Weapons/ProjectileTypes/AC_FastProjectilesPowerup.AC_FastProjectilesPowerup_C")
    (Development|PrintString "Hello")))

(fn ConstructionScript)