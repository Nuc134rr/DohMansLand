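; BP_PlayerOneTank is the tank pawn for player one, driven and fired through P1-specific input bindings.
; Axis inputs yaw the body mesh and copy its rotation to the actor, while forward and backward input feeds CharacterMovement along the actor's forward vector.
; A separate aim axis yaws the turret, and the fire action spawns the projectile class at the barrel's location with the turret's rotation.
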(event Input|ActionEvents|InputActionFireP1
  (params (Key :type Key%20Structure :default "None"))
  ;[0.2 0.2 0.2] Shoot (LShift)
  (:Pressed
    (Game|SpawnActorfromClass (Variables|Default|GetProjectileClass) (Math|Transform|MakeTransform (Transformation|GetWorldLocation (Variables|Default|GetBarrel)) (Transformation|GetWorldRotation (Variables|Default|GetTurret)) "1.000000,1.000000,1.000000") "Undefined" self 0)))

(event Input|AxisEvents|InputAxisAimRightP1
  (params (AxisValue :type Float%20%28single-precision%29))
  ;[0.145 0.6838 1] Movement/Rotation
  ;;[0.2 0.2 0.2] Rotate the Turret of the tank (Q and E)
  (Transformation|AddWorldRotation (Variables|Default|GetTurret) (Math|Rotator|MakeRotator 0.0 0.0 (* AxisValue 2.0)) false false))

(event Input|AxisEvents|InputAxisRightP1
  (params (AxisValue :type Float%20%28single-precision%29))
  (bind _mesh (Variables|Character|GetMesh))
  ;[0.145 0.6838 1] Movement/Rotation
  ;;[0.2 0.2 0.2] Rotate the body of the tank (A and D)
  (Transformation|AddWorldRotation _mesh (Math|Rotator|MakeRotator 0.0 0.0 (* AxisValue 2.0)) false false)
  (Transformation|SetActorRotation (Transformation|GetWorldRotation _mesh)))

(event Input|AxisEvents|InputAxisUpP1
  (params (AxisValue :type Float%20%28single-precision%29))
  ;[0.145 0.6838 1] Movement/Rotation
  ;;[0.2 0.2 0.2] Move forward and backward (W and S)
  (Class|PawnMovementComponent|AddInputVector (Variables|Character|GetCharacterMovement) (* (Transformation|GetActorForwardVector) AxisValue) false))

(fn ConstructionScript)