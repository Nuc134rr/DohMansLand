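; BP_PlayerOneTank1 is a player-controlled tank that drives, turns, aims its turret and fires, bound to the P2 input events despite its PlayerOne name.
; Body input yaws the mesh and copies that rotation to the actor, and forward input feeds the actor's forward vector into CharacterMovement.
; The turret yaws separately, and firing spawns a projectile at the barrel's location with the turret's rotation, owned by the tank.
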(event Custom|P2_RotateBody
  (params (AxisValue :type Float%20%28double-precision%29))
  (bind _mesh (Variables|Character|GetMesh))
  ;[0.145 0.6838 1] Movement/Rotation
  ;;[0.2 0.2 0.2] Rotate the body of the tank (A and D)
  (Transformation|AddWorldRotation _mesh (Math|Rotator|MakeRotator 0.0 0.0 AxisValue) false false)
  (Transformation|SetActorRotation (Transformation|GetWorldRotation _mesh)))

(event Custom|P2_RotateTurret
  (params (AxisValue :type Float%20%28double-precision%29))
  ;[0.145 0.6838 1] Movement/Rotation
  ;;[0.2 0.2 0.2] Rotate the Turret of the tank (Q and E)
  (Transformation|AddWorldRotation (Variables|Default|GetTurret) (Math|Rotator|MakeRotator 0.0 0.0 AxisValue) false false))

(event Custom|P2_Fire
  ;[0.2 0.2 0.2] Shoot (LShift)
  (Game|SpawnActorfromClass (Variables|Default|GetProjectileClass) (Math|Transform|MakeTransform (Transformation|GetWorldLocation (Variables|Default|GetBarrel)) (Transformation|GetWorldRotation (Variables|Default|GetTurret)) "1.000000,1.000000,1.000000") "Undefined" self 0))

(event Custom|P2_MoveForward
  (params (AxisValue :type Float%20%28double-precision%29))
  ;[0.145 0.6838 1] Movement/Rotation
  ;;[0.2 0.2 0.2] Move forward and backward (W and S)
  (Class|PawnMovementComponent|AddInputVector (Variables|Character|GetCharacterMovement) (* (Transformation|GetActorForwardVector) AxisValue) false))

(fn ConstructionScript)