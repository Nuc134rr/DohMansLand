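; Touch joystick actor that turns a stick toward the player's finger and derives a turn direction for the tank's turret.
; A touch on the cylinder starts tracking, which Tick repeats by tracing under the finger and rotating the stick to face the hit point.
; It compares that yaw with the turret's to set NewYaw to -1, 0 or 1, flipping across 180 degrees.
; The touch-end handler is empty.
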(event OnInputTouchBegin(Cylinder)
  (params (FingerIndex :type ETouchIndex%20Enum :default "Touch1") (TouchedComponent :type Primitive%20Component%20Object%20Reference))
  (bind _returnvalue (Game|GetPlayerController 0))
  (bind _transform (Variables|Default|Gettransform))
  (bind (_hitresult _returnvalue_2) (Class|PlayerController|GetHitResultUnderFingerbyChannel _returnvalue FingerIndex "TraceTypeQuery2" false))
  ;[0.4558 0.9502 1] Joystick
  ;;[0.2304 0.3524 1] Code for touch
  (Variables|Default|Setable2 true)
  (Variables|Default|Setable true)
  (if _returnvalue_2
    (if (stale _output_get)
      (Variables|Default|SetFingerLoc (Math|Vector|MakeVector (.x (.location _hitresult)) (.y (.location _hitresult)) 0.0)))
    (else
      (bind _output_get (Variables|Default|Setable false))))
  (Transformation|SetRelativeRotation (Variables|Default|Getstick) (Math|Rotator|MakeRotator 0.0 0.0 (.yaw (Math|Rotator|FindLookatRotation (Math|Vector|MakeVector (.x (.location _transform)) (.y (.location _transform)) (- (.z (.location _transform)) 237.0)) (Variables|Default|GetFingerLoc)))) false true)
  (if (Math|Float|NearlyEqual(Float) (- (.yaw (Math|Rotator|FindLookatRotation (Math|Vector|MakeVector (.x (.location _transform)) (.y (.location _transform)) (- (.z (.location _transform)) 237.0)) (Variables|Default|GetFingerLoc))) (.yaw (Transformation|GetWorldRotation (Variables|/Game/Blueprints/Player/BP_BaseTank.BP_BaseTank_C|GetTurret (Variables|Default|GetTankThatWork))))) 0.0 2.0)
    (Variables|Default|SetNewYaw 0.0)
    (else
      (if (> (- (.yaw (Math|Rotator|FindLookatRotation (Math|Vector|MakeVector (.x (.location _transform)) (.y (.location _transform)) (- (.z (.location _transform)) 237.0)) (Variables|Default|GetFingerLoc))) (.yaw (Transformation|GetWorldRotation (Variables|/Game/Blueprints/Player/BP_BaseTank.BP_BaseTank_C|GetTurret (Variables|Default|GetTankThatWork))))) 0.0)
        (Variables|Default|SetNewYaw 1.0)
        (else
          (Variables|Default|SetNewYaw -1.0)))
      (if (or (< (- (.yaw (Math|Rotator|FindLookatRotation (Math|Vector|MakeVector (.x (.location _transform)) (.y (.location _transform)) (- (.z (.location _transform)) 237.0)) (Variables|Default|GetFingerLoc))) (.yaw (Transformation|GetWorldRotation (Variables|/Game/Blueprints/Player/BP_BaseTank.BP_BaseTank_C|GetTurret (Variables|Default|GetTankThatWork))))) -1.8e+02) (> (- (.yaw (Math|Rotator|FindLookatRotation (Math|Vector|MakeVector (.x (.location _transform)) (.y (.location _transform)) (- (.z (.location _transform)) 237.0)) (Variables|Default|GetFingerLoc))) (.yaw (Transformation|GetWorldRotation (Variables|/Game/Blueprints/Player/BP_BaseTank.BP_BaseTank_C|GetTurret (Variables|Default|GetTankThatWork))))) 1.8e+02))
        (Variables|Default|SetNewYaw (* (Variables|Default|GetNewYaw) -1.0))))))

(event Custom|OnInputTouchEnd_Event
  (params (FingerIndex :type ETouchIndex%20Enum :default "Touch1") (TouchedActor :type Actor%20Object%20Reference))
  ;[0.4558 0.9502 1] Joystick
  ;;[0.2304 0.3524 1] Let Go
)

(event EventBeginPlay
  ;[0.4558 0.9502 1] Joystick
  ;;[0.2304 0.3524 1] Begin Play
  (EventDispatchers|BindEventtoOnInputTouchEnd (delegate Custom|OnInputTouchEnd_Event))
  (Variables|Default|Settransform (Transformation|GetWorldTransform (Variables|Default|GetJoystick))))

(event EventTick
  (params (DeltaSeconds :type Float%20%28single-precision%29))
  (bind _transform (Variables|Default|Gettransform))
  ;[0.4558 0.9502 1] Joystick
  ;;[0.2304 0.3524 1] Code for touch
  (if (Variables|Default|Getable2)
    (if (.ReturnValue (Class|PlayerController|GetHitResultUnderFingerbyChannel (Game|GetPlayerController 0) (stale OnInputTouchBegin(Cylinder) FingerIndex) "TraceTypeQuery2" false))
      (if (stale _output_get)
        (Variables|Default|SetFingerLoc (Math|Vector|MakeVector (.x (.location (.HitResult (Class|PlayerController|GetHitResultUnderFingerbyChannel (Game|GetPlayerController 0) (stale OnInputTouchBegin(Cylinder) FingerIndex) "TraceTypeQuery2" false)))) (.y (.location (.HitResult (Class|PlayerController|GetHitResultUnderFingerbyChannel (Game|GetPlayerController 0) (stale OnInputTouchBegin(Cylinder) FingerIndex) "TraceTypeQuery2" false)))) 0.0)))
      (else
        (bind _output_get (Variables|Default|Setable false))))
    (Transformation|SetRelativeRotation (Variables|Default|Getstick) (Math|Rotator|MakeRotator 0.0 0.0 (.yaw (Math|Rotator|FindLookatRotation (Math|Vector|MakeVector (.x (.location _transform)) (.y (.location _transform)) (- (.z (.location _transform)) 237.0)) (Variables|Default|GetFingerLoc)))) false true)
    (if (Math|Float|NearlyEqual(Float) (- (.yaw (Math|Rotator|FindLookatRotation (Math|Vector|MakeVector (.x (.location _transform)) (.y (.location _transform)) (- (.z (.location _transform)) 237.0)) (Variables|Default|GetFingerLoc))) (.yaw (Transformation|GetWorldRotation (Variables|/Game/Blueprints/Player/BP_BaseTank.BP_BaseTank_C|GetTurret (Variables|Default|GetTankThatWork))))) 0.0 2.0)
      (Variables|Default|SetNewYaw 0.0)
      (else
        (if (> (- (.yaw (Math|Rotator|FindLookatRotation (Math|Vector|MakeVector (.x (.location _transform)) (.y (.location _transform)) (- (.z (.location _transform)) 237.0)) (Variables|Default|GetFingerLoc))) (.yaw (Transformation|GetWorldRotation (Variables|/Game/Blueprints/Player/BP_BaseTank.BP_BaseTank_C|GetTurret (Variables|Default|GetTankThatWork))))) 0.0)
          (Variables|Default|SetNewYaw 1.0)
          (else
            (Variables|Default|SetNewYaw -1.0)))
        (if (or (< (- (.yaw (Math|Rotator|FindLookatRotation (Math|Vector|MakeVector (.x (.location _transform)) (.y (.location _transform)) (- (.z (.location _transform)) 237.0)) (Variables|Default|GetFingerLoc))) (.yaw (Transformation|GetWorldRotation (Variables|/Game/Blueprints/Player/BP_BaseTank.BP_BaseTank_C|GetTurret (Variables|Default|GetTankThatWork))))) -1.8e+02) (> (- (.yaw (Math|Rotator|FindLookatRotation (Math|Vector|MakeVector (.x (.location _transform)) (.y (.location _transform)) (- (.z (.location _transform)) 237.0)) (Variables|Default|GetFingerLoc))) (.yaw (Transformation|GetWorldRotation (Variables|/Game/Blueprints/Player/BP_BaseTank.BP_BaseTank_C|GetTurret (Variables|Default|GetTankThatWork))))) 1.8e+02))
          (Variables|Default|SetNewYaw (* (Variables|Default|GetNewYaw) -1.0)))))))

(fn ConstructionScript)