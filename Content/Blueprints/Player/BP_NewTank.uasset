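; Player tank pawn with body rotation, forward movement and a separately rotating turret.
; MoveBase prints its axis and shares a FloatingPawnMovement input along the forward vector with a W key press, while RotateBody yaws the base by TurnSpeed.
; RotateTurret eases the turret along the shortest path to a root-relative yaw, or zero without ResetZ.
; GetDistanceConvertedToTime should time that turn, but its angle-to-time calculation is left unconnected.
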(event Custom|RotateBody
  (params (Axis :type Float%20%28double-precision%29))
  (Transformation|AddWorldRotation (Variables|Default|GetBase) (Math|Rotator|MakeRotator 0.0 0.0 (* Axis (Variables|Default|GetTurnSpeed))) false false))

(event Custom|MoveBase
  (params (Axis :type Float%20%28double-precision%29))
  (Development|PrintString (Utilities|String|ToString(Float) Axis))
  (Class|PawnMovementComponent|AddInputVector (Variables|Default|GetFloatingPawnMovement) (* (Transformation|GetActorForwardVector) (* Axis (Variables|/Script/Engine.FloatingPawnMovement|GetMaxSpeed (Variables|Default|GetFloatingPawnMovement)))) false))

(event Custom|RotateTurret
  (params (TargetRotation :type Float%20%28double-precision%29) (ResetZ :type Boolean))
  (bind _defaultsceneroot (Variables|Default|GetDefaultSceneRoot))
  (bind _turret (Variables|Default|GetTurret))
  (bind _returnvalue (Transformation|GetRelativeTransform _defaultsceneroot))
  (bind _relativerotation (Variables|/Script/Engine.SceneComponent|GetRelativeRotation _turret))
  (bind _returnvalue_2 (Math|Transform|InverseTransformRotation _returnvalue (Math|Rotator|MakeRotator 0.0 0.0 TargetRotation)))
  (bind _returnvalue_3 (select ResetZ (.yaw _returnvalue_2) 0.0))
  (Components|MoveComponentTo 0 (Variables|/Script/Engine.SceneComponent|GetRelativeLocation _turret) (Math|Rotator|MakeRotator (.roll _relativerotation) (.pitch _relativerotation) _returnvalue_3) false false (|GetDistanceConvertedToTime _returnvalue_3 (.yaw _relativerotation)) true))

(event Input|KeyboardEvents|W
  (params (Key :type Key%20Structure :default "None"))
  (:Pressed
    (Variables|Default|SetAxisValue 1.0)
    (Class|PawnMovementComponent|AddInputVector (Variables|Default|GetFloatingPawnMovement) (* (Transformation|GetActorForwardVector) (* (stale Custom|MoveBase Axis) (Variables|/Script/Engine.FloatingPawnMovement|GetMaxSpeed (Variables|Default|GetFloatingPawnMovement)))) false))
  (:Released
    (Variables|Default|SetAxisValue 0.0)))

(fn ConstructionScript)

(fn GetShortestRotation
  (params (Start :type Float%20%28double-precision%29) (End :type Float%20%28double-precision%29))
  (bind _returnvalue (- Start End))
  (bind _returnvalue_2 (Math|Float|Absolute(Float) _returnvalue))
  (if (>= _returnvalue_2 1.8e+02)
    (return (- 1.8e+02 (- _returnvalue_2 1.8e+02)))
    (else
      (return _returnvalue_2))))