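; On-screen 3D touch joystick for tank rotation that tilts a stick toward the finger and sets a NewYaw turn direction.
; Touching the Cylinder enables a Tick update that traces under the finger and aims the stick via look-at rotation.
; NewYaw becomes ±1 by comparing finger yaw with TankThatWork's mesh yaw, both remapped to 0–360.
; Touch end or a failed trace zeroes NewYaw and eases the stick's pitch back to neutral.
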(event OnInputTouchBegin(Cylinder)
  (params (FingerIndex :type ETouchIndex%20Enum :default "Touch1") (TouchedComponent :type Primitive%20Component%20Object%20Reference))
  (bind _returnvalue (Game|GetPlayerController 0))
  (bind _transform (Variables|Default|Gettransform))
  (bind (_hitresult _returnvalue_2) (Class|PlayerController|GetHitResultUnderFingerbyChannel _returnvalue FingerIndex "TraceTypeQuery2" false))
  (bind _returnvalue_3 (- (.z (.location _transform)) 237.0))
  (bind _returnvalue_4 (Math|Vector|MakeVector (.x (.location _hitresult)) (.y (.location _hitresult)) 0.0))
  (bind _returnvalue_5 (Math|Vector|MakeVector (.x (.location _transform)) (.y (.location _transform)) _returnvalue_3))
  (bind _returnvalue_6 (Math|Rotator|FindLookatRotation _returnvalue_5 _returnvalue_4))
  (bind _returnvalue_7 (Math|Float|MapRangeClamped (.yaw _returnvalue_6) -1.8e+02 1.8e+02 0.0 3.6e+02))
  ;[0.4558 0.9502 1] Joystick
  ;;[0.2304 0.3524 1] Code for touch
  (Variables|Default|Setable true)
  ;;;[0.2768 0.4154 1] Math Stuff
  (if (> _returnvalue_7 (/ (+ (Math|Float|MapRangeClamped (.yaw (Transformation|GetWorldRotation (Variables|/Script/Engine.Character|GetMesh (Variables|Default|GetTankThatWork)))) -1.8e+02 1.8e+02 0.0 3.6e+02) _returnvalue_7) 2.0))
    (Variables|Default|SetNewYaw 1.0)
    (else
      (Variables|Default|SetNewYaw -1.0)))
  (Transformation|SetRelativeRotation (Variables|Default|Getstick) (Math|Rotator|MakeRotator 0.0 (+ (* (.pitch _returnvalue_6) -1.0) -5e+01) (.yaw _returnvalue_6)) false true)
  (Development|PrintString "Hello"))

(event Custom|OnInputTouchEnd_Event
  (params (FingerIndex :type ETouchIndex%20Enum :default "Touch1") (TouchedActor :type Actor%20Object%20Reference))
  (bind _stick (Variables|Default|Getstick))
  (bind _returnvalue (Transformation|GetRelativeTransform _stick))
  ;[0.4558 0.9502 1] Joystick
  ;;[0.2304 0.3524 1] Let Go
  (Variables|Default|Setable false)
  (Variables|Default|SetNewYaw 0.0 :!label _label)
  (Components|MoveComponentTo _stick "0, 0, 0" (Math|Rotator|MakeRotator (.roll (.rotation _returnvalue)) 0.0 (.yaw (.rotation _returnvalue))) false true 0.3 true)
  (goto _label))

(event EventBeginPlay
  ;[0.4558 0.9502 1] Joystick
  ;;[0.2304 0.3524 1] Begin Play
  (EventDispatchers|BindEventtoOnInputTouchEnd (delegate Custom|OnInputTouchEnd_Event))
  (Variables|Default|Settransform (Transformation|GetWorldTransform (Variables|Default|GetJoystick))))

(event EventTick
  (params (DeltaSeconds :type Float%20%28single-precision%29))
  (bind _stick (Variables|Default|Getstick))
  (bind _transform (Variables|Default|Gettransform))
  (bind _returnvalue (Transformation|GetRelativeTransform _stick))
  ;[0.4558 0.9502 1] Joystick
  ;;[0.2304 0.3524 1] Code for touch
  (if (Variables|Default|Getable)
    ;;;[0.2768 0.4154 1] Math Stuff
    (if (.ReturnValue (Class|PlayerController|GetHitResultUnderFingerbyChannel (Game|GetPlayerController 0) (stale OnInputTouchBegin(Cylinder) FingerIndex) "TraceTypeQuery2" false))
      (if (> (Math|Float|MapRangeClamped (.yaw (Math|Rotator|FindLookatRotation (Math|Vector|MakeVector (.x (.location _transform)) (.y (.location _transform)) (- (.z (.location _transform)) 237.0)) (Math|Vector|MakeVector (.x (.location (.HitResult (Class|PlayerController|GetHitResultUnderFingerbyChannel (Game|GetPlayerController 0) (stale OnInputTouchBegin(Cylinder) FingerIndex) "TraceTypeQuery2" false)))) (.y (.location (.HitResult (Class|PlayerController|GetHitResultUnderFingerbyChannel (Game|GetPlayerController 0) (stale OnInputTouchBegin(Cylinder) FingerIndex) "TraceTypeQuery2" false)))) 0.0))) -1.8e+02 1.8e+02 0.0 3.6e+02) (/ (+ (Math|Float|MapRangeClamped (.yaw (Transformation|GetWorldRotation (Variables|/Script/Engine.Character|GetMesh (Variables|Default|GetTankThatWork)))) -1.8e+02 1.8e+02 0.0 3.6e+02) (Math|Float|MapRangeClamped (.yaw (Math|Rotator|FindLookatRotation (Math|Vector|MakeVector (.x (.location _transform)) (.y (.location _transform)) (- (.z (.location _transform)) 237.0)) (Math|Vector|MakeVector (.x (.location (.HitResult (Class|PlayerController|GetHitResultUnderFingerbyChannel (Game|GetPlayerController 0) (stale OnInputTouchBegin(Cylinder) FingerIndex) "TraceTypeQuery2" false)))) (.y (.location (.HitResult (Class|PlayerController|GetHitResultUnderFingerbyChannel (Game|GetPlayerController 0) (stale OnInputTouchBegin(Cylinder) FingerIndex) "TraceTypeQuery2" false)))) 0.0))) -1.8e+02 1.8e+02 0.0 3.6e+02)) 2.0))
        (Variables|Default|SetNewYaw 1.0)
        (else
          (Variables|Default|SetNewYaw -1.0)))
      (Transformation|SetRelativeRotation (Variables|Default|Getstick) (Math|Rotator|MakeRotator 0.0 (+ (* (.pitch (Math|Rotator|FindLookatRotation (Math|Vector|MakeVector (.x (.location _transform)) (.y (.location _transform)) (- (.z (.location _transform)) 237.0)) (Math|Vector|MakeVector (.x (.location (.HitResult (Class|PlayerController|GetHitResultUnderFingerbyChannel (Game|GetPlayerController 0) (stale OnInputTouchBegin(Cylinder) FingerIndex) "TraceTypeQuery2" false)))) (.y (.location (.HitResult (Class|PlayerController|GetHitResultUnderFingerbyChannel (Game|GetPlayerController 0) (stale OnInputTouchBegin(Cylinder) FingerIndex) "TraceTypeQuery2" false)))) 0.0))) -1.0) -5e+01) (.yaw (Math|Rotator|FindLookatRotation (Math|Vector|MakeVector (.x (.location _transform)) (.y (.location _transform)) (- (.z (.location _transform)) 237.0)) (Math|Vector|MakeVector (.x (.location (.HitResult (Class|PlayerController|GetHitResultUnderFingerbyChannel (Game|GetPlayerController 0) (stale OnInputTouchBegin(Cylinder) FingerIndex) "TraceTypeQuery2" false)))) (.y (.location (.HitResult (Class|PlayerController|GetHitResultUnderFingerbyChannel (Game|GetPlayerController 0) (stale OnInputTouchBegin(Cylinder) FingerIndex) "TraceTypeQuery2" false)))) 0.0)))) false true)
      (Development|PrintString "Hello")
      (else
        ;;[0.2304 0.3524 1] Let Go
        (Variables|Default|Setable false)
        (Variables|Default|SetNewYaw 0.0 :!label _label)
        (Components|MoveComponentTo _stick "0, 0, 0" (Math|Rotator|MakeRotator (.roll (.rotation _returnvalue)) 0.0 (.yaw (.rotation _returnvalue))) false true 0.3 true)
        (goto _label)))))

(fn ConstructionScript)