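; General function library for Doh Man's Land, offering shared helpers for typed access, level travel and material randomization.
; Getters return the cast game mode, game instance and the tank pawns of players one to six.
; OpenNewLevel opens a level by name and increments LevelNumber on the game instance.
; SetRandomColors gives a target an M_Doh dynamic material with a random seed and one palette color; the second-color logic is disconnected.
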(fn GetDohMansLandGameMode
  (return (.AsBP%20Doh%20Mans%20Land%20Game%20Mode (Utilities|Casting|CastToBP_DohMansLand_GameMode (Game|GetGameMode)))))

(fn GetDohMansLandGameInstance
  (return (.AsBP%20Doh%20Mans%20Land%20Game%20Instance (Utilities|Casting|CastToBP_DohMansLand_GameInstance (Game|GetGameInstance)))))

(fn SetRandomColors
  (params (Target :type Primitive%20Component%20Object%20Reference))
  (bind _returnvalue (Rendering|Material|CreateDynamicMaterialInstance Target 0 "/Game/Assets/Materials/M_Doh.M_Doh" "None" :!class /Script/Engine.PrimitiveComponent))
  ;[1 1 1] Random Seed
  (Rendering|Material|SetScalarParameterValue _returnvalue "RandomSeed" (Math|Random|RandomFloatinRange 0.0 1e+03) :!class /Script/Engine.MaterialInstanceDynamic)
  ;[1 1 1] Number of Doh Colors
  (switch int 1
    (:0
      _)
    (:1
      (Utilities|FlowControl|Sequence
        (:then_0
          _))))
  ;[1 1 1] Random Color0 Assignment
  (Rendering|Material|SetScalarParameterValue _returnvalue "NumberOfColors" 1.0 :!class /Script/Engine.MaterialInstanceDynamic)
  (switch int (Math|Random|RandomInteger 7)
    (:0
      (Rendering|Material|SetVectorParameterValue _returnvalue "Color0" "(R=0.973445,G=0.042311,B=0.038204,A=1.000000)" :!class /Script/Engine.MaterialInstanceDynamic))
    (:1
      (Rendering|Material|SetVectorParameterValue _returnvalue "Color0" "(R=0.830770,G=0.291771,B=0.000000,A=1.000000)" :!class /Script/Engine.MaterialInstanceDynamic))
    (:2
      (Rendering|Material|SetVectorParameterValue _returnvalue "Color0" "(R=0.701102,G=0.658375,B=0.019382,A=1.000000)" :!class /Script/Engine.MaterialInstanceDynamic))
    (:3
      (Rendering|Material|SetVectorParameterValue _returnvalue "Color0" "(R=0.318547,G=0.665387,B=0.309469,A=1.000000)" :!class /Script/Engine.MaterialInstanceDynamic))
    (:4
      (Rendering|Material|SetVectorParameterValue _returnvalue "Color0" "(R=0.000911,G=0.035601,B=0.514918,A=1.000000)" :!class /Script/Engine.MaterialInstanceDynamic))
    (:5
      (Rendering|Material|SetVectorParameterValue _returnvalue "Color0" "(R=0.346704,G=0.029557,B=0.341914,A=1.000000)" :!class /Script/Engine.MaterialInstanceDynamic))
    (:6
      (Rendering|Material|SetVectorParameterValue _returnvalue "Color0" "(R=0.693872,G=0.693872,B=0.768151,A=1.000000)" :!class /Script/Engine.MaterialInstanceDynamic))))

(fn GetPlayerOnePawn
  (return (.AsBP%20Base%20Tank (Utilities|Casting|CastToBP_BaseTank (Game|Player|GetPlayerPawn 0)))))

(fn GetPlayerTwoPawn
  (return (.AsBP%20Base%20Tank (Utilities|Casting|CastToBP_BaseTank (Game|Player|GetPlayerPawn 0 1)))))

(fn OpenNewLevel
  (params (LevelName :type Name))
  (Game|OpenLevel(byName) 0 LevelName)
  (Math|Integer|IncrementInt (Variables|/Game/Blueprints/Player/BP_DohMansLand_GameInstance.BP_DohMansLand_GameInstance_C|GetLevelNumber (CallFunction|GetDohMansLandGameInstance))))

(fn GetPlayerThreePawn
  (return (.AsBP%20Base%20Tank (Utilities|Casting|CastToBP_BaseTank (Game|Player|GetPlayerPawn 0 2)))))

(fn GetPlayerFourPawn
  (return (.AsBP%20Base%20Tank (Utilities|Casting|CastToBP_BaseTank (Game|Player|GetPlayerPawn 0 3)))))

(fn GetPlayerFivePawn
  (return (.AsBP%20Base%20Tank (Utilities|Casting|CastToBP_BaseTank (Game|Player|GetPlayerPawn 0 4)))))

(fn GetPlayerSixPawn
  (return (.AsBP%20Base%20Tank (Utilities|Casting|CastToBP_BaseTank (Game|Player|GetPlayerPawn 0 5)))))