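; Tank character for DohMansLand, in the AI folder but with no decision logic, exposing events to drive, rotate body and turret, and fire.
; Firing spawns capped, rate-limited projectiles, while movement scales by frame delta.
; Hitting airdrop crates adds their powerup component.
; Game mode per-player data supplies sounds and particle colors; winners get a scaling crown, and the confetti event turns shots into party effects.
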(event Custom|Winnign%20Confetti
  (params (New%20Color :type Linear%20Color%20Structure))
  (bind _particle_values (Variables|Default|GetParticle%20Values))
  (Variables|/Game/Assets/FX/BP_NiagaraValueHolder.BP_NiagaraValueHolder_C|SetSystem _particle_values "/Game/Assets/FX/Confetti.Confetti")
  (Transformation|SetRelativeScale3D _particle_values "4.000000,4.000000,4.000000")
  (Variables|/Game/Assets/FX/BP_NiagaraValueHolder.BP_NiagaraValueHolder_C|SetFloat%20Param _particle_values 5.0)
  (Variables|/Game/Assets/FX/BP_NiagaraValueHolder.BP_NiagaraValueHolder_C|SetColor%20Param _particle_values New%20Color)
  (Utilities|SpawnTurretParticles
    (:%20%20
      (Variables|Default|SetWinnign? true))))

(event Custom|RotateBody
  (params (AxisValue :type Float%20%28double-precision%29))
  (bind _turnspeed (Variables|Movement|GetTurnSpeed))
  (bind _deltaseconds (Variables|Default|GetDeltaSeconds))
  (bind _returnvalue (* AxisValue _turnspeed _deltaseconds))
  ;[0.145 0.6838 1] Movement/Rotation
  ;;[0.2 0.2 0.2] Rotate the body of the tank
  (Pawn|Input|AddControllerYawInput _returnvalue)
  (Transformation|AddWorldRotation (Variables|Default|GetTurret) (Math|Rotator|MakeRotator 0.0 0.0 (* _returnvalue (* (Class|PlayerController|GetDeprecatedInputYawScale (Game|GetPlayerController (Variables|Gameplay|GetPlayerID))) -1.0))) false false))

(event Custom|MoveForward
  (params (AxisValue :type Float%20%28double-precision%29))
  ;[0.145 0.6838 1] Movement/Rotation
  ;;[0.2 0.2 0.2] Move forward
  (Class|PawnMovementComponent|AddInputVector (Variables|Character|GetCharacterMovement) (* (* AxisValue (Variables|Movement|GetMoveSpeed) (Variables|Default|GetDeltaSeconds)) (Transformation|GetActorForwardVector)) false)
  (if (not (Math|Float|NearlyEqual(Float) AxisValue 0.0 1e-06))
    (Utilities|FlowControl|DoOnce false :!label _label
      (:Completed
        (bind _returnvalue (Audio|SpawnSound2D (.movesound (Utilities|Array|Get(acopy) (Variables|/Game/Blueprints/Player/BP_DohMansLand_GameMode.BP_DohMansLand_GameMode_C|GetTank%20Variables (CallFunction|GetDohMansLandGameMode)) (Variables|Gameplay|GetPlayerID))) 1.0 1.0 0.0 0))
        (Variables|Default|SetMove%20Sound _returnvalue)))
    (else
      (Utilities|IsValid (Variables|Default|GetMove%20Sound)
        (:Is%20Valid
          (Audio|Components|Audio|Stop (Variables|Default|GetMove%20Sound))
          (goto _label Reset))))))

(event Custom|Fire
  (bind _self self)
  (bind _projectilescale (Variables|Projectiles|GetProjectileScale))
  (bind _barrel (Variables|Default|GetBarrel))
  (bind _returnvalue (Transformation|GetWorldRotation _barrel))
  (bind _returnvalue_2 (Transformation|GetWorldLocation _barrel))
  (bind _returnvalue_3 (Math|Vector|GetForwardVector _returnvalue))
  (bind _returnvalue_4 (* _projectilescale _returnvalue_3))
  (bind _returnvalue_5 (* "50.000000,50.000000,50.000000" _returnvalue_4))
  (bind _returnvalue_6 (+ _returnvalue_5 _returnvalue_2))
  ;[0.7982 0.2142 1] Projectile Logic
  ;;[0.2 0.2 0.2] Fire Projectile (LShift OR RShift) IF this tank has less than 3 projectiles already spawned
  (if (not (== (Utilities|Array|Length (Variables|Projectiles|GetCurrentProjectiles)) (Variables|Projectiles|GetMaxProjectiles)))
    (Utilities|FlowControl|DoOnce false :!label _label
      (:Completed
        (Utilities|SpawnTurretParticles
          (:%20%20
            (if (Variables|Default|GetWinnign?)
              (Audio|PlaySound2D "/Game/Assets/SFX/misc_outside_noises/Party_Horn_Cue.Party_Horn_Cue" 1.0 1.0 0.0 0 0)
              (else
                (bind _returnvalue_7 (Game|SpawnActorfromClass (Variables|Projectiles|GetProjectileClass) (Math|Transform|MakeTransform (Math|Vector|MakeVector (.x _returnvalue_6) (.y _returnvalue_6) (+ (.z _returnvalue_6) (* (.z (Variables|Projectiles|GetProjectileScale)) 4e+01))) _returnvalue _projectilescale) "Undefined" _self _self 0))
                (Utilities|Array|Add (Variables|Projectiles|GetCurrentProjectiles) _returnvalue_7)
                (Audio|PlaySound2D (.shootsound (Utilities|Array|Get(acopy) (Variables|/Game/Blueprints/Player/BP_DohMansLand_GameMode.BP_DohMansLand_GameMode_C|GetTank%20Variables (CallFunction|GetDohMansLandGameMode)) (Variables|Gameplay|GetPlayerID))) 1.0 1.0 0.0 0 0)))
            (Utilities|FlowControl|Delay (Variables|/Game/Projectiles/BP_BaseProjectile.BP_BaseProjectile_C|GetFireRate _returnvalue_7))
            (goto _label Reset)))))))

(event Custom|RemoveProjectile
  (params (ProjectileToRemove :type BP%20Base%20Projectile%20Object%20Reference))
  ;[0.7982 0.2142 1] Projectile Logic
  ;;[0.2 0.2 0.2] Remove Projectile from array when it dies
  (Utilities|Array|RemoveItem (Variables|Projectiles|GetCurrentProjectiles) ProjectileToRemove))

(event Custom|Rotate%20Turret%20With%20Rotator
  (params (Target%20Rotation :type Float%20%28double-precision%29) (Reset%20Z :type Boolean))
  (bind _turret (Variables|Default|GetTurret))
  (bind _capsulecomponent (Variables|Collision|GetCapsuleComponent))
  (bind _returnvalue (Transformation|GetRelativeTransform _capsulecomponent))
  (bind _relativerotation (Variables|/Script/Engine.SceneComponent|GetRelativeRotation _turret))
  (bind _returnvalue_2 (Math|Transform|InverseTransformRotation _returnvalue (Math|Rotator|MakeRotator 0.0 0.0 Target%20Rotation)))
  (bind _return (CallFunction|AORB 0.0 (.yaw _returnvalue_2) Reset%20Z))
  ;[0.145 0.6838 1] Movement/Rotation
  ;;[0.2 0.2 0.2] Rotate the turret
  (Components|MoveComponentTo _turret (Variables|/Script/Engine.SceneComponent|GetRelativeLocation _turret) (Math|Rotator|MakeRotator (.roll _relativerotation) (.pitch _relativerotation) _return) false false (|GetDistanceConvertedtoTime _return (.yaw _relativerotation)) true))

(event Custom|Winnign%20Crown
  ;[1 1 1] Spawns Crown and scales up gradualy over the Winning tank
  (bind _scaler (Timeline|Tl_Crown%20Scaler Play)
    (:Update
      (Transformation|SetRelativeScale3D (Variables|Default|GetCrown) _scaler))))

(event EventTick
  (params (DeltaSeconds :type Float%20%28single-precision%29))
  ;[0.2 0.2 0.2] makes movement across variable frame rates consistent (substepping) (very important)
  (Variables|Default|SetDeltaSeconds (* DeltaSeconds 1e+02)))

(event Collision|EventHit
  (params (MyComp :type Primitive%20Component%20Object%20Reference) (Other :type Actor%20Object%20Reference) (OtherComp :type Primitive%20Component%20Object%20Reference) (bSelfMoved :type Boolean) (HitLocation :type Vector :default "0, 0, 0") (HitNormal :type Vector :default "0, 0, 0") (NormalImpulse :type Vector :default "0, 0, 0") (Hit :type Hit%20Result%20Structure%20%28by%20ref%29))
  (bind (_asbp_airdrop_crate _bsuccess) (Utilities|Casting|CastToBP_AirdropCrate Other))
  (bind _powerup (Variables|/Game/Blueprints/Airdrop/BP_AirdropCrate.BP_AirdropCrate_C|GetPowerup _asbp_airdrop_crate))
  ;[1 0.5506 0.1137] Comment
  ;;[0.6667 0.6667 0.6667] Powerup Code
  (if _bsuccess
    (CallFunction|MoveCratetoJoysticks _asbp_airdrop_crate)
    (Game|AddComponentbyClass _powerup)
    (Math|Integer|IncrementInt (Variables|Gameplay|GetNumberOfPowerups)
      (:%20%20
        (Default|CallPowerupp _powerup)))))

(event EventDestroyed
  (bind _capsulecomponent (Variables|Collision|GetCapsuleComponent))
  (bind _move_sound (Variables|Default|GetMove%20Sound))
  (bind _returnvalue (Transformation|GetWorldTransform _capsulecomponent))
  (Effects|SpawnEmitteratLocation "/Game/TopDownStarterContent/StarterContent/Particles/P_Explosion.P_Explosion" (.location _returnvalue) (.rotation _returnvalue) "5.000000,5.000000,5.000000")
  (Utilities|IsValid _move_sound
    (:Is%20Valid
      (Audio|Components|Audio|Stop _move_sound))))

(event EventBeginPlay
  (bind _capsulecomponent (Variables|Collision|GetCapsuleComponent))
  (bind _returnvalue (Transformation|GetWorldTransform _capsulecomponent))
  (Utilities|FlowControl|Sequence
    (:then_0
      (if (== (Variables|Gameplay|GetPlayerID) (Variables|/Game/Blueprints/Player/BP_DohMansLand_GameInstance.BP_DohMansLand_GameInstance_C|GetWinnerID (CallFunction|GetDohMansLandGameInstance)))
        (CallFunction|WinnignCrown)))
    (:then_1
      (|SetParticleColors
        (:%20%20
          (bind _returnvalue_2 (Effects|SpawnEmitteratLocation "/Game/TopDownStarterContent/StarterContent/Particles/P_Fire.P_Fire" (.location _returnvalue) (.rotation _returnvalue) "0.500000,0.500000,0.500000"))
          (Utilities|FlowControl|Delay 2.0)
          (Components|DestroyComponent _returnvalue_2)
          ;[1 1 1] Spawns Crown and scales up gradualy over the Winning tank
          (EventDispatchers|BindEventtoDone (CallFunction|GetDohMansLandGameMode) (delegate Custom|Winnign%20Crown)))))))

(fn ConstructionScript)

(fn SetPlayerTankDoh
  (params (InputPin :type Skeletal%20Mesh%20Component%20Object%20Reference) (PlayerID :type Integer) (ElementIndex :type Integer))
  (bind _returnvalue (Rendering|Material|CreateDynamicMaterialInstance InputPin ElementIndex "/Game/Assets/Materials/M_Doh.M_Doh" "None" :!class /Script/Engine.PrimitiveComponent))
  ;[1 1 1] Random Seed
  (bind _output_get (Variables|Default|SetDynamicMaterialInstance _returnvalue))
  (Rendering|Material|SetScalarParameterValue _output_get "RandomSeed" (Math|Random|RandomFloatinRange 0.0 1e+03) :!class /Script/Engine.MaterialInstanceDynamic)
  ;[1 1 1] Random Color0 Assignment
  (Rendering|Material|SetScalarParameterValue (Variables|Default|GetDynamicMaterialInstance) "NumberOfColors" 1.0 :!class /Script/Engine.MaterialInstanceDynamic)
  (Rendering|Material|SetVectorParameterValue (Variables|Default|GetDynamicMaterialInstance) "Color0" (.tankcolor (Utilities|Array|Get(acopy) (Variables|/Game/Blueprints/Player/BP_DohMansLand_GameMode.BP_DohMansLand_GameMode_C|GetTank%20Variables (CallFunction|GetDohMansLandGameMode)) (Variables|Gameplay|GetPlayerID))) :!class /Script/Engine.MaterialInstanceDynamic))

(fn SetPlayerID
  (bind _outactors (Actor|GetAllActorsOfClass "/Game/Blueprints/Player/BP_BaseTank.BP_BaseTank_C"))
  (bind _result (Math|Integer|DecrementInt (Utilities|Array|Length _outactors))
    (:%20%20
      (bind _output_get (Variables|Gameplay|SetPlayerID _result))
      (return _output_get))))

(fn GetShortestRotation
  (params (Start :type Float%20%28double-precision%29) (End :type Float%20%28double-precision%29))
  (bind _returnvalue (- Start End))
  (bind _returnvalue_2 (Math|Float|Absolute(Float) _returnvalue))
  (if (>= _returnvalue_2 1.8e+02)
    (return (- 1.8e+02 (- _returnvalue_2 1.8e+02)))
    (else
      (return _returnvalue_2))))

(fn AORB
  (params (A :type Float%20%28double-precision%29) (B :type Float%20%28double-precision%29) (Condition :type Boolean))
  (if Condition
    (return A)
    (else
      (return B))))

(fn MoveCratetoJoysticks
  (params (CrateRef :type BP%20Airdrop%20Crate%20Object%20Reference))
  (bind _capsulecomponent (Variables|Collision|GetCapsuleComponent))
  (bind _returnvalue (Transformation|GetWorldTransform _capsulecomponent))
  (Effects|SpawnEmitteratLocation "/Game/TopDownStarterContent/StarterContent/Particles/P_Explosion.P_Explosion" (.location _returnvalue) (.rotation _returnvalue) "5.000000,5.000000,5.000000"))