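; On-screen 3D touch control panel for one player's BP_BaseTank, tinted to that tank's color.
; Per-finger touches drive two spring-back levers, a turret spinner and a fire button.
; Tick feeds the tank turret yaw and exponent-curved lever values, summed for throttle and differenced for turning; the idle spinner later follows the turret.
; Movement controls slide in before shooting controls; game mode events gray out or slide the panel away on death or level reset.
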(event OnInputTouchBegin(RightMovestick)
  (params (FingerIndex :type ETouchIndex%20Enum :default "Touch1") (TouchedComponent :type Primitive%20Component%20Object%20Reference))
  ;[0.9376 1 0.4438] Set Variables for Running
  (if (not (Variables|RunConditionBools|GetRotate%20Right%20Movestick))
    (Variables|RunConditionBools|SetRotate%20Right%20Movestick true)
    (Variables|FingerIndexs|SetRight%20Move%20Index FingerIndex)))

(event OnInputTouchBegin(SpinnerBase)
  (params (FingerIndex :type ETouchIndex%20Enum :default "Touch1") (TouchedComponent :type Primitive%20Component%20Object%20Reference))
  ;[0.9376 1 0.4438] Set Variables for Running
  (if (not (Variables|RunConditionBools|GetRotate%20Turret))
    (Variables|RunConditionBools|SetRotate%20Turret true)
    (Variables|FingerIndexs|SetTurret%20Index FingerIndex)))

(event OnInputTouchBegin(Button)
  (params (FingerIndex :type ETouchIndex%20Enum :default "Touch1") (TouchedComponent :type Primitive%20Component%20Object%20Reference))
  ;[1 0 0.01544] Firing
  (if (not (Variables|RunConditionBools|GetButton%20Fire))
    (Variables|RunConditionBools|SetButton%20Fire true)
    (bind _asbp_base_tank (Utilities|Casting|CastToBP_BaseTank (Game|Player|GetPlayerPawn (Variables|Default|GetPlayer%20Index))))
    (Default|Fire _asbp_base_tank)
    (CallFunction|MoveButton 0.05 "0, 0,-80.000000")))

(event OnInputTouchBegin(LeftMovestick)
  (params (FingerIndex :type ETouchIndex%20Enum :default "Touch1") (TouchedComponent :type Primitive%20Component%20Object%20Reference))
  ;[0.9376 1 0.4438] Set Variables for Running
  (if (not (Variables|RunConditionBools|GetRotate%20Left%20Movestick))
    (Variables|RunConditionBools|SetRotate%20Left%20Movestick true)
    (Variables|FingerIndexs|SetLeft%20Move%20Index FingerIndex)))

(event OnInputTouchLeave(Collision)
  (params (FingerIndex :type ETouchIndex%20Enum :default "Touch1") (TouchedComponent :type Primitive%20Component%20Object%20Reference))
  ;[1 0.2846 0.1277] Button released
  (if (Variables|RunConditionBools|GetButton%20Fire)
    (Variables|RunConditionBools|SetButton%20Fire false)
    (CallFunction|MoveButton 0.2 "0, 0, 0")))

(event OnInputTouchBegin(Collision)
  (params (FingerIndex :type ETouchIndex%20Enum :default "Touch1") (TouchedComponent :type Primitive%20Component%20Object%20Reference))
  ;[1 0 0.01544] Firing
  (if (not (Variables|RunConditionBools|GetButton%20Fire))
    (Variables|RunConditionBools|SetButton%20Fire true)
    (bind _asbp_base_tank (Utilities|Casting|CastToBP_BaseTank (Game|Player|GetPlayerPawn (Variables|Default|GetPlayer%20Index))))
    (Default|Fire _asbp_base_tank)
    (CallFunction|MoveButton 0.05 "0, 0,-80.000000")))

(event Custom|Move%20Button
  (params (Over%20Time :type Float%20%28double-precision%29) (Location :type Vector))
  (bind _button (Variables|Default|GetButton))
  ;[1 0.7397 0.1436] Move Button Event To Prevent Moving Twice
  (Components|MoveComponentTo _button Location (Variables|/Script/Engine.SceneComponent|GetRelativeRotation _button) false false Over%20Time false))

(event Custom|RemoveControlls
  (params (PlayerIndex :type Integer))
  (bind _self self)
  ;[0.9319 0.2489 1] subtracting -2000 from the controls once tank is dead and grays out controls
  (if (== PlayerIndex (Variables|Default|GetPlayer%20Index))
    (Rendering|Material|SetVectorParameterValue (Variables|Default|GetMaterialInstance) "Color0" "(R=0.250000,G=0.250000,B=0.250000,A=1.000000)" :!class /Script/Engine.MaterialInstanceDynamic)
    (Utilities|FlowControl|Delay 0.5)
    (Variables|Default|SetMove%20Out%20Location (Math|Transform|TransformLocation (Transformation|GetActorTransform _self) "0,-5000.000000, 0"))
    (Variables|Default|SetStart%20Location (Transformation|GetActorLocation _self))
    (bind _0_1 (Timeline|Move%20Out Play)
      (:Update
        (Transformation|SetActorLocation (Math|Vector|Lerp(Vector) (Variables|Default|GetStart%20Location) (Variables|Default|GetMove%20Out%20Location) _0_1) false false)))))

(event Custom|RemoveOnReset
  (bind _self self)
  (if (Math|Boolean|ANDBoolean (== (Variables|Default|GetPlayer%20Index) (Variables|/Game/Blueprints/Player/BP_DohMansLand_GameInstance.BP_DohMansLand_GameInstance_C|GetWinnerID (CallFunction|GetDohMansLandGameInstance))) (Variables|Default|GetIsTankAlive) true)
    ;[0.9319 0.2489 1] subtracting -2000 from the controls once tank is dead and grays out controls
    (Utilities|FlowControl|Delay 0.5 :!label _label)
    (Variables|Default|SetMove%20Out%20Location (Math|Transform|TransformLocation (Transformation|GetActorTransform _self) "0,-5000.000000, 0"))
    (Variables|Default|SetStart%20Location (Transformation|GetActorLocation _self))
    (bind _0_1 (Timeline|Move%20Out Play)
      (:Update
        (Transformation|SetActorLocation (Math|Vector|Lerp(Vector) (Variables|Default|GetStart%20Location) (Variables|Default|GetMove%20Out%20Location) _0_1) false false)))
    (else
      (bind _outactors (Actor|GetAllActorsOfClass "/Game/Blueprints/Player/BP_BaseTank.BP_BaseTank_C"))
      (if (> (Utilities|Array|Length _outactors) 1)
        (if (Variables|Default|GetIsTankAlive)
          (goto _label))))))

(event EventBeginPlay
  (bind _returnvalue (CallFunction|GetDohMansLandGameMode))
  ;[0 0.95 1] Set Color of Joysticks and Button
  (bind _returnvalue_2 (Rendering|Material|CreateDynamicMaterialInstance "/Game/Assets/Materials/M_JoystickBall_Inst.M_JoystickBall_Inst" "JoysticksColor" "None" :!class /Script/Engine.KismetMaterialLibrary))
  (bind _output_get (Variables|Default|SetMaterialInstance _returnvalue_2))
  (Rendering|Material|SetMaterial (Variables|Default|GetLeft%20Switch) 0 _output_get)
  (Rendering|Material|SetVectorParameterValue _output_get "Color0" (.tankcolor (Utilities|Array|Get(acopy) (Variables|/Game/Blueprints/Player/BP_DohMansLand_GameMode.BP_DohMansLand_GameMode_C|GetTank%20Variables (CallFunction|GetDohMansLandGameMode)) (Variables|Default|GetPlayer%20Index))) :!class /Script/Engine.MaterialInstanceDynamic)
  (EventDispatchers|AssignRemoveControls _returnvalue (delegate Custom|RemoveControlls))
  (EventDispatchers|BindEventtoLevelReset _returnvalue (delegate Custom|RemoveOnReset))
  (Utilities|FlowControl|Delay 2.0)
  ;[0.1437 0.08166 1] Moves in movement controls waits 10 seconds then moves in shooting controls
  (Utilities|FlowControl|Sequence
    (:then_0
      (Utilities|MoveComponentsto0 (Variables|Default|GetRight%20Movestick) 2.0))
    (:then_1
      (Utilities|MoveComponentsto0 (Variables|Default|GetLeft%20Movestick) 2.0
        (:Completed
          (Utilities|FlowControl|Delay 1e+01)
          (Utilities|FlowControl|Sequence
            (:then_0
              (Utilities|MoveComponentsto0 (Variables|Default|GetSpinnerBase) 2.0))
            (:then_1
              (Utilities|MoveComponentsto0 (Variables|Default|GetFire%20Button) 2.0))))))))

(event EventTick
  (params (DeltaSeconds :type Float%20%28single-precision%29))
  (bind _left_switch (Variables|Default|GetLeft%20Switch))
  (bind _left_switch_2 (Variables|Default|GetLeft%20Switch))
  (bind _spinnerbase (Variables|Default|GetSpinnerBase))
  (bind _turret_index (Variables|FingerIndexs|GetTurret%20Index))
  (bind _left_move_index (Variables|FingerIndexs|GetLeft%20Move%20Index))
  (bind _right_move_index (Variables|FingerIndexs|GetRight%20Move%20Index))
  (bind _player_index (Variables|Default|GetPlayer%20Index))
  (bind _joystick_exponent (Variables|Default|GetJoystick%20Exponent))
  (bind _right_switch (Variables|Default|GetRight%20Switch))
  (bind _right_switch_2 (Variables|Default|GetRight%20Switch))
  (bind _right_switch_3 (Variables|Default|GetRight%20Switch))
  (bind _left_switch_3 (Variables|Default|GetLeft%20Switch))
  (bind _returnvalue (Game|Player|GetPlayerPawn _player_index))
  (bind (_returnvalue_roll _returnvalue_pitch _returnvalue_yaw) (Utilities|FindFingerLookatZ _turret_index _spinnerbase))
  (bind _relativerotation (Variables|/Script/Engine.SceneComponent|GetRelativeRotation _right_switch))
  (bind _relativerotation_2 (Variables|/Script/Engine.SceneComponent|GetRelativeRotation _left_switch_3))
  (bind _relativerotation_3 (Variables|/Script/Engine.SceneComponent|GetRelativeRotation _left_switch_2))
  (bind _relativerotation_4 (Variables|/Script/Engine.SceneComponent|GetRelativeRotation _left_switch))
  (bind _relativerotation_5 (Variables|/Script/Engine.SceneComponent|GetRelativeRotation _right_switch_2))
  (bind _relativerotation_6 (Variables|/Script/Engine.SceneComponent|GetRelativeRotation _right_switch_3))
  (bind (_asbp_base_tank _bsuccess) (Utilities|Casting|CastToBP_BaseTank _returnvalue))
  (bind _returnvalue_2 (/ (.pitch _relativerotation_6) 45.0))
  (bind _returnvalue_3 (/ (.pitch _relativerotation_4) 45.0))
  (bind _power_return (CallFunction|FindControlPower _returnvalue_2 _joystick_exponent))
  (bind _power_return_2 (CallFunction|FindControlPower _returnvalue_3 _joystick_exponent))
  (bind _returnvalue_4 (/ _power_return_2 2.0))
  (bind _returnvalue_5 (/ _power_return 2.0))
  ;[0 0.2908 1] Set stick angles
  (Utilities|FlowControl|Sequence
    (:then_0
      ;[0.3749 1 0.9052] Set turret joystick rotation
      (if (and (.bIsCurrentlyPressed (Class|PlayerController|GetInputTouchState (Game|GetPlayerController 0) _turret_index)) (Variables|RunConditionBools|GetRotate%20Turret))
        (bind _output_get (Variables|Default|SetReset%20Turret%20Z false))
        (Transformation|SetRelativeRotation (Variables|Default|GetSpinner) (Math|Rotator|MakeRotator _returnvalue_roll _returnvalue_pitch _returnvalue_yaw) false false)
        (Utilities|FlowControl|RetriggerableDelay 2.0)
        (Variables|Default|SetReset%20Turret%20Z true)
        (else
          (Variables|RunConditionBools|SetRotate%20Turret false)
          (|RotateByTurret _output_get))))
    (:then_1
      (if (and (.bIsCurrentlyPressed (Class|PlayerController|GetInputTouchState (Game|GetPlayerController 0) _left_move_index)) (Variables|RunConditionBools|GetRotate%20Left%20Movestick))
        (Transformation|SetRelativeRotation _left_switch_3 (Math|Rotator|MakeRotator (.roll _relativerotation_2) (Math|Float|Lerp -45.0 45.0 (Utilities|JoystickYDistance _left_move_index (Variables|Default|GetLeft%20Movestick))) (.yaw _relativerotation_2)) false false)
        (goto _label Reset)
        (else
          (Variables|RunConditionBools|SetRotate%20Left%20Movestick false)
          (Utilities|FlowControl|DoOnce true :!label _label
            (:Completed
              (Components|MoveComponentTo _left_switch_2 (Variables|/Script/Engine.SceneComponent|GetRelativeLocation _left_switch_2) (Math|Rotator|MakeRotator (.roll _relativerotation_3) 0.0 (.yaw _relativerotation_3)) true true 0.2 false))))))
    (:then_2
      (if (and (.bIsCurrentlyPressed (Class|PlayerController|GetInputTouchState (Game|GetPlayerController 0) _right_move_index)) (Variables|RunConditionBools|GetRotate%20Right%20Movestick))
        (Transformation|SetRelativeRotation _right_switch_2 (Math|Rotator|MakeRotator (.roll _relativerotation_5) (Math|Float|Lerp -45.0 45.0 (Utilities|JoystickYDistance _right_move_index (Variables|Default|GetRight%20Movestick))) (.yaw _relativerotation_5)) false false)
        (goto _label_2 Reset)
        (else
          (Variables|RunConditionBools|SetRotate%20Right%20Movestick false)
          (Utilities|FlowControl|DoOnce true :!label _label_2
            (:Completed
              (Components|MoveComponentTo _right_switch (Variables|/Script/Engine.SceneComponent|GetRelativeLocation _right_switch) (Math|Rotator|MakeRotator (.roll _relativerotation) 0.0 (.yaw _relativerotation)) true true 0.2 false))))))
    (:then_3
      ;[0.2334 1 0.2359] Feed Inputs To Tank
      (if (and _bsuccess (Utilities|IsValid _returnvalue))
        (Default|RotateTurretwithRotator _asbp_base_tank (.yaw (Transformation|GetWorldRotation (Variables|Default|GetSpinner))) (Variables|Default|GetReset%20Turret%20Z))
        (Default|MoveForward _asbp_base_tank (+ _returnvalue_5 _returnvalue_4))
        (Default|RotateBody _asbp_base_tank (+ (* _returnvalue_5 -1.0) _returnvalue_4))))))

(fn ConstructionScript)

(fn FindControlPower
  (params (Base :type Float%20%28double-precision%29) (Exponent :type Float%20%28double-precision%29))
  (bind _returnvalue (Math|Float|Absolute(Float) Base))
  (bind _returnvalue_2 (Math|Float|Power _returnvalue Exponent))
  (if (< Base 0.0)
    (return (* _returnvalue_2 -1.0))
    (else
      (return _returnvalue_2))))